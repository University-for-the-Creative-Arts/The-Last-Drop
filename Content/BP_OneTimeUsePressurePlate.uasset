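; BP_OneTimeUsePressurePlate is a pressure plate that triggers linked activatable objects when an actor tagged "Heavy" overlaps its Box.
; On begin overlap it plays an activation sound, prints a debug string and calls ActivateDeactivate on every BPActivatable entry.
; Leaving the box does nothing, as the matching release logic is disconnected.
; Despite the name, no guard prevents retriggering on later overlaps.
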(event `self.Box.OnComponentBeginOverlap`
  (params (OverlappedComponent :type "PrimitiveComponent Object Reference") (OtherActor :type "Actor Object Reference") (OtherComp :type "PrimitiveComponent Object Reference") (OtherBodyIndex :type Integer) (bFromSweep :type Boolean) (SweepResult :type "HitResult Structure (by ref)"))
  (if (`self.ActorHasTag` OtherActor "Heavy")
    (`GameplayStatics.PlaySound2D` "/Game/Dynamic/Audio/Events/MS_InteractableActivate.MS_InteractableActivate" 1.0 1.0 0.0 null null)
    (`KismetSystemLibrary.PrintString` "Hello")
    (for _array_element (`self.BP_Activatable`)
      (`/Game/Dynamic/Blueprints/Environment/Activatable/BP_ActivatableParent.Activate/Deactivate` _array_element))))

(event `self.Box.OnComponentEndOverlap`
  (params (OverlappedComponent :type "PrimitiveComponent Object Reference") (OtherActor :type "Actor Object Reference") (OtherComp :type "PrimitiveComponent Object Reference") (OtherBodyIndex :type Integer)))

(fn `UserConstructionScript`)