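; An activatable ice ball thrower that swings its mesh component like a catapult arm when activated.
; Activate/Deactivate runs through a FlipFlop, so only every other call, starting with the first, can trigger a flip.
; Flip uses two eased MoveComponentTo moves to tilt the mesh quickly and return it more slowly to zero rotation, while IsFlipping blocks re-triggering during the motion.
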(event `self.Activate/Deactivate`
  (`/Engine/EditorBlueprintResources/StandardMacros.FlipFlop`
    (:`A`
      (if (not (`self.IsFlipping`))
        (`self.Flip`)))))

(event `Flip`
  (set `self.IsFlipping` true)
  (`KismetSystemLibrary.MoveComponentTo` (`self.SM`) (0.0 0.0 0.0) (struct :`Roll` -70.0) true true 0.25)
  (`KismetSystemLibrary.MoveComponentTo` (`self.SM`) (0.0 0.0 0.0) (struct) true true 0.5)
  (set `self.IsFlipping` false))

(fn `UserConstructionScript`
  (`parent.UserConstructionScript`))