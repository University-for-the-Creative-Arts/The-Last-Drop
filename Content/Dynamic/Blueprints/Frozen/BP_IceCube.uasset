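; Physics-driven ice cube that rides conveyors and can shatter into a Geometry Collection.
; Tick pushes it along its right vector while moving, with tagged overlaps starting, stopping or flip-flopping direction, and physics enabled on leaving a blade.
; A recursive delay loop destroys it when it stays nearly still.
; PhysicsandDestroy swaps physics to the fracture pieces, then Decay animates the dynamic material's opacity before destroying the actor.
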(event `self.ReceiveBeginPlay`
  ;[1 1 1] Start Idle Destroy Loop
  (`self.IdleDestroy`)
  (bind _returnvalue (`PrimitiveComponent.CreateDynamicMaterialInstance` (`self.GeometryCollection`) 0 "/Game/Static/Materials/MI_Ice.MI_Ice" "None"))
  (set `self.IceMaterial` _returnvalue))

(event `IdleDestroy`
  (bind _returnvalue (< (`KismetMathLibrary.VSize` (`SceneComponent.GetComponentVelocity` (`self.StaticMesh`))) 4.0))
  ;[1 1 1] If not moving after 10 secs then destroy
  (if _returnvalue
    (`KismetSystemLibrary.Delay` 10.0)
    (if _returnvalue
      (`self.K2_DestroyActor`)
      (else
        (`self.IdleDestroy` :!label _label)))
    (else
      (`KismetSystemLibrary.Delay` 10.0)
      (goto _label))))

(event `self.ReceiveTick`
  (params (DeltaSeconds :type "Float (single-precision)"))
  (bind _staticmesh (`self.StaticMesh`))
  (bind _staticmesh_2 (`self.StaticMesh`))
  ;[1 1 1] Movement
  ;;[1 1 1] If is moving and is simulating physics
  (if (`self.Moving`)
    (if (`SceneComponent.IsSimulatingPhysics` (`self.StaticMesh`) "None")
      ;;[1 1 1] Flip Direction based on variable
      (if (`self.Moving Right`)
        (`PrimitiveComponent.AddForce` _staticmesh_2 (* (`SceneComponent.GetRightVector` _staticmesh_2) (`self.Speed`)) "None" false)
        (else
          (`PrimitiveComponent.AddForce` _staticmesh (* (`SceneComponent.GetRightVector` _staticmesh) (* (`self.Speed`) -1.0)) "None" false))))))

(event `self.Overlap.OnComponentBeginOverlap`
  (params (OverlappedComponent :type "PrimitiveComponent Object Reference") (OtherActor :type "Actor Object Reference") (OtherComp :type "PrimitiveComponent Object Reference") (OtherBodyIndex :type Integer) (bFromSweep :type Boolean) (SweepResult :type "HitResult Structure (by ref)"))
  ;[1 1 1] Begin Overlap
  ;;[1 1 1] Overlaps where you want it to move
  (if (or (`self.ActorHasTag` OtherActor "Conveyor") (`self.ActorHasTag` OtherActor "IceCube") (`self.ActorHasTag` OtherActor "Crusher"))
    (set `self.Moving` true)
    (else
      ;;[1 1 1] Change Direction
      (if (`self.ActorHasTag` OtherActor "SwapConveyorDirection")
        (set `self.Moving` true)
        (`/Engine/EditorBlueprintResources/StandardMacros.FlipFlop`
          (:`A`
            (set `self.Moving Right` true))
          (:`B`
            (set `self.Moving Right` false)))
        (else
          ;;[1 1 1] Stop Movement
          (if (or (`self.ActorHasTag` OtherActor "EndConveyor") (`self.ActorHasTag` OtherActor "Cart"))
            (set `self.Moving` false)))))))

(event `self.Overlap.OnComponentEndOverlap`
  (params (OverlappedComponent :type "PrimitiveComponent Object Reference") (OtherActor :type "Actor Object Reference") (OtherComp :type "PrimitiveComponent Object Reference") (OtherBodyIndex :type Integer))
  ;[1 1 1] End Overlap and change direction
  (if (`self.ActorHasTag` OtherActor "SwapConveyorDirection")
    (set `self.Moving` false)
    (else
      (set `self.Moving` true))))

(event `self.StaticMesh.OnComponentBeginOverlap`
  (params (OverlappedComponent :type "PrimitiveComponent Object Reference") (OtherActor :type "Actor Object Reference") (OtherComp :type "PrimitiveComponent Object Reference") (OtherBodyIndex :type Integer) (bFromSweep :type Boolean) (SweepResult :type "HitResult Structure (by ref)"))
  ;[1 1 1] Stop on contact with enviroment obsacle
  (if (`self.ActorHasTag` OtherActor "Blade")
    _
    (elif (`self.ActorHasTag` OtherActor "Crusher")
      (bind _asbp_crusher (cast `/Game/Dynamic/Blueprints/Frozen/BP_Crusher` OtherActor)))))

(event `self.StaticMesh.OnComponentEndOverlap`
  (params (OverlappedComponent :type "PrimitiveComponent Object Reference") (OtherActor :type "Actor Object Reference") (OtherComp :type "PrimitiveComponent Object Reference") (OtherBodyIndex :type Integer))
  (if (`self.ActorHasTag` OtherActor "Blade")
    (`PrimitiveComponent.SetSimulatePhysics` (`self.StaticMesh`) true)
    (set `self.Moving` true)))

(event `Physics and Destroy`
  (`PrimitiveComponent.SetSimulatePhysics` (`self.StaticMesh`) false)
  (`PrimitiveComponent.SetSimulatePhysics` (`self.GeometryCollection`) true)
  (`KismetSystemLibrary.Delay` 2.0)
  (`self.Decay`))

(event `Decay`
  (bind (_direction _clear) (`Timeline|Timeline` :!via `PlayFromStart`)
    (:`Update`
      (`MaterialInstanceDynamic.SetScalarParameterValue` (`self.IceMaterial`) "Opacity" (`KismetMathLibrary.Lerp` 0.0 4.0 _clear)))
    (:`Finished`
      (`self.K2_DestroyActor`))))

(fn `UserConstructionScript`)