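; Frozen platform that melts away once when its Activate/Deactivate event fires, losing collision and sinking.
; BeginPlay creates a dynamic ice material on the platform mesh, and the Decay timeline drives its Opacity parameter.
; Activation starts Decay, then after a short delay disables collision and lowers the mesh with MoveComponentTo.
; IsMelted is set only when the timeline finishes, blocking later activations from that point.
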(event `self.ReceiveBeginPlay`
  ;[1 1 1] Opacity
  (bind _returnvalue (`PrimitiveComponent.CreateDynamicMaterialInstance` (`self.SM_Platform`) 0 "/Game/Static/Materials/MI_Ice.MI_Ice" "None"))
  (set `self.IceMaterial` _returnvalue))

(event `self.Activate/Deactivate`
  (bind (_relativelocation_x _relativelocation_y _relativelocation_z) (`KismetMathLibrary.BreakVector` (`SceneComponent.RelativeLocation` (`self.SM_Platform`))))
  ;[1 1 1] If not melted, move down and decay
  (if (not (`self.IsMelted?`))
    (`self.Decay`)
    (`KismetSystemLibrary.Delay` 1.8)
    (`PrimitiveComponent.SetCollisionEnabled` (`self.SM_Platform`) "NoCollision")
    (`KismetSystemLibrary.MoveComponentTo` (`self.SM_Platform`) (`KismetMathLibrary.MakeVector` _relativelocation_x _relativelocation_y (- _relativelocation_z 50.0)) (struct) false false 2.0)))

(event `Decay`
  ;[1 1 1] decay
  (bind (_direction _clear) (`Timeline|Timeline` :!via `PlayFromStart`)
    (:`Update`
      (`MaterialInstanceDynamic.SetScalarParameterValue` (`self.IceMaterial`) "Opacity" (`KismetMathLibrary.Lerp` 0.0 4.0 _clear)))
    (:`Finished`
      (set `self.IsMelted?` true))))

(fn `UserConstructionScript`
  (`parent.UserConstructionScript`))