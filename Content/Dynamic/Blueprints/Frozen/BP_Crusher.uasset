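; BP_Crusher is a hazard that repeatedly slams its Crusher component down and eases it back up.
; The crusher flagged IsFirst starts on BeginPlay, and each crush also triggers NextCrusher after NextDelay to stagger a chain.
; Overlaps break ice cubes via PhysicsAndDestroy, or revert an ice ball to bubble state, return the camera to the body character and pop it.
; The logic that would halt crushing on ice is disconnected.
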(event `self.ReceiveBeginPlay`
  ;[1 1 1] If is first crusher then start loop
  (if (`self.Is First`)
    (`self.Crush`)))

(event `Crush`
  ;[1 1 1] Crush
  (`|ExecutionSequence`
    (:`then_0`
      ;;[1 1 1] Only crush if not overlapping ice
      (if (not (`self.Is OverlappingIce`))
        ;;[1 1 1] Interrupt move
        (set `self.IsCrushing` true)
        ;;[1 1 1] move, wait, then return
        (`KismetSystemLibrary.MoveComponentTo` (`self.Crusher`) (0.0 0.0 -90.0) (struct) false false 0.25 :!label _label)
        (set `self.IsCrushing` false)
        (`KismetSystemLibrary.Delay` 0.5)
        (`self.Return`)
        (else
          (`self.Stop`))))
    (:`then_1`
      ;;[1 1 1] Start next crusher simultaniusly
      (`KismetSystemLibrary.Delay` (`self.Next Delay`))
      (`/Engine/EditorBlueprintResources/StandardMacros.IsValid` (`self.Next Crusher`)
        (:`Is Valid`
          (`self.Crush` (`self.Next Crusher`)))))))

(event `Stop`
  ;[1 1 1] Crush
  ;;[1 1 1] Interrupt move
  (`|ExecutionSequence`
    (:`then_0`
      (goto _label :!via `Stop`))
    (:`then_1`
      (`self.Return`))))

(event `Return`
  ;[1 1 1] Return
  (set `self.IsCrushing` false)
  (`KismetSystemLibrary.MoveComponentTo` (`self.Crusher`) (0.0 0.0 100.0) (struct) false true 0.5)
  (`KismetSystemLibrary.Delay` 0.5)
  (`self.Crush`))

(event `self.CubeTest.OnComponentBeginOverlap`
  (params (OverlappedComponent :type "PrimitiveComponent Object Reference") (OtherActor :type "Actor Object Reference") (OtherComp :type "PrimitiveComponent Object Reference") (OtherBodyIndex :type Integer) (bFromSweep :type Boolean) (SweepResult :type "HitResult Structure (by ref)"))
  ;[1 1 1] Begin overlap icecube, stop and disable
  (if (`self.ActorHasTag` OtherActor "IceCube")
    (bind _asbp_ice_cube (cast `/Game/Dynamic/Blueprints/Frozen/BP_IceCube` OtherActor))
    (`/Game/Dynamic/Blueprints/Frozen/BP_IceCube.Physics and Destroy` _asbp_ice_cube)))

(event `self.Ball Collision.OnComponentBeginOverlap`
  (params (OverlappedComponent :type "PrimitiveComponent Object Reference") (OtherActor :type "Actor Object Reference") (OtherComp :type "PrimitiveComponent Object Reference") (OtherBodyIndex :type Integer) (bFromSweep :type Boolean) (SweepResult :type "HitResult Structure (by ref)"))
  (if true
    (bind _asbp_bubble_char (cast `/Game/Dynamic/Blueprints/Characters/BubbleChar/BP_BubbleChar` OtherActor))
    (`self.Destroy Ice Ball` _asbp_bubble_char)))

(fn `Destroy Ice Ball`
  (params (Target :type "/Game/Dynamic/Blueprints/Characters/BubbleChar/BP_BubbleChar Object Reference"))
  (set `SurfaceStateComponent.BubbleStates` "Default" (`/Game/Dynamic/Blueprints/Characters/BubbleChar/BP_BubbleChar.AC_BubbleStates` Target))
  (set `/Game/Dynamic/Blueprints/Actor_Components/AC_BubbleStats.Lifespan` 10.0 (`/Game/Dynamic/Blueprints/Characters/BubbleChar/BP_BubbleChar.AC_BubbleStats` Target))
  (bind _returnvalue (`PrimitiveComponent.CreateDynamicMaterialInstance` (`/Game/Dynamic/Blueprints/Characters/BubbleChar/BP_BubbleChar.Sphere` Target) 0 "/Game/Dynamic/Blueprints/Characters/BubbleChar/MI_Bubble.MI_Bubble" "None"))
  (set `/Game/Dynamic/Blueprints/Characters/BubbleChar/BP_BubbleChar.BubbleMaterial` _returnvalue Target)
  (bind _asbp_body_char (cast `/Game/Dynamic/Blueprints/Characters/BodyChar/BP_BodyChar` (`GameplayStatics.GetPlayerCharacter` 0)))
  (`PlayerController.SetViewTargetWithBlend` (`PlayerState.GetPlayerController` (`Pawn.PlayerState` _asbp_body_char)) _asbp_body_char 0.0 "VTBlend_Linear" 0.0 false)
  (`/Game/Dynamic/Blueprints/Actor_Components/AC_BubbleControls.Pop` (`/Game/Dynamic/Blueprints/Characters/BubbleChar/BP_BubbleChar.AC_BubbleControls` Target) Target))

(fn `UserConstructionScript`)