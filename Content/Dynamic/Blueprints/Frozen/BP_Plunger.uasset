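; BP_Plunger is an actor whose SMPlunger component endlessly cycles between a low and a raised position along its local vertical.
; BeginPlay caches the starting rotation and starts a loop of two custom events, Move and Return, which call each other after delays.
; Move drives the component down quickly with MoveComponentTo, while Return raises it slowly with ease-in and waits longer before the next plunge.
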(event `self.ReceiveBeginPlay`
  (set `self.Start Rotation` (`SceneComponent.RelativeRotation` (`self.SM_Plunger`)))
  (`self.Move`))

(event `Move`
  (`KismetSystemLibrary.MoveComponentTo` (`self.SM_Plunger`) (0.0 0.0 -300.0) (`self.Start Rotation`) false false 0.3)
  (`KismetSystemLibrary.Delay` 1.0)
  (`self.Return`))

(event `Return`
  (`KismetSystemLibrary.MoveComponentTo` (`self.SM_Plunger`) (0.0 0.0 60.0) (`self.Start Rotation`) false true 2.0)
  (`KismetSystemLibrary.Delay` 5.0)
  (`self.Move`))

(fn `UserConstructionScript`)