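; Animated mechanical arm that appears to carry a pipe between conveyor A and conveyor B.
; On BeginPlay it caches both conveyor actor types and plays a timeline that rotates the arm segments.
; The timeline's Attach event flip-flops between resetting, attaching and showing the arm's own Pipe, and detaching and hiding it.
; Each phase calls SpawnPipe on the matching conveyors (A on pickup, B on release), faking the handoff with one reused component.
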(event `self.ReceiveBeginPlay`
  (`self.Mechanical Arm Start`)
  (bind _outactors (`GameplayStatics.GetAllActorsOfClass` "/Game/Dynamic/Blueprints/Frozen/BP_ConveyorPipeA.BP_ConveyorPipeA_C"))
  (set `self.BP_conveyorpipeA` _outactors)
  (bind _outactors_2 (`GameplayStatics.GetAllActorsOfClass` "/Game/Dynamic/Blueprints/Frozen/BP_ConveyorPipeB.BP_ConveyorPipeB_C"))
  (set `self.BP_conveyorpipeB` _outactors_2))

(event `Mechanical Arm Start`
  (bind _pipe (`self.Pipe`))
  (bind _pipe_2 (`self.Pipe`))
  (bind _pipe_3 (`self.Pipe`))
  (set `self.PipeOriginalLocation` (`SceneComponent.K2_GetComponentLocation` _pipe_3))
  (set `self.PipeOriginalRotation` (`SceneComponent.K2_GetComponentRotation` _pipe_3))
  (bind (_direction _armrotationdown _armupperrotate _armlowerrotate _largecylinderrotate) (`Timeline|Arm Rotate For Pickup` :!via `PlayFromStart`)
    (:`Update`
      (`SceneComponent.K2_SetRelativeRotation` (`self.MechanicalArmLargeCylinder_A88B8D65`) (`KismetMathLibrary.MakeRotator` _armrotationdown 0.0 _largecylinderrotate) false false)
      (`SceneComponent.K2_SetRelativeRotation` (`self.MechanicalArmUpper_27AF2947`) (`KismetMathLibrary.MakeRotator` _armupperrotate) false false)
      (`SceneComponent.K2_SetRelativeRotation` (`self.MechanicalArmLower_41EF3FDB`) (`KismetMathLibrary.MakeRotator` _armlowerrotate) false false))
    (:`Attach`
      (`/Engine/EditorBlueprintResources/StandardMacros.FlipFlop`
        (:`A`
          (`SceneComponent.K2_SetWorldLocationAndRotation` _pipe_2 (`self.PipeOriginalLocation`) (`self.PipeOriginalRotation`) false true)
          (`SceneComponent.K2_AttachToComponent` _pipe_2 (`self.MechanicalArmHead_B00DA569`) "None" "KeepWorld" "KeepWorld" "KeepWorld" true)
          (for _array_element (`self.BP_conveyorpipeA`)
            (`/Game/Dynamic/Blueprints/Frozen/BP_ConveyorPipeA.SpawnPipe` _array_element)
            (`SceneComponent.SetHiddenInGame` _pipe false false)))
        (:`B`
          (`SceneComponent.K2_DetachFromComponent` _pipe_2 "KeepWorld" "KeepWorld" "KeepWorld" true)
          (for _array_element_2 (`self.BP_conveyorpipeB`)
            (`/Game/Dynamic/Blueprints/Frozen/BP_ConveyorPipeB.SpawnPipe` _array_element_2)
            (`SceneComponent.SetHiddenInGame` _pipe true false)))))))

(fn `UserConstructionScript`)