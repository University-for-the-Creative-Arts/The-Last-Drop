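; Falling platform that wobbles as a warning, then drops after the player steps onto it.
; An overlap on the Box by player character 0 runs a chain of latent eased MoveComponentTo rotations, rocking the Platform back and forth before a final tilt.
; After a short delay it enables physics simulation on the Platform, with TimeToFall scaling every step's duration.
; The Blueprint contains no reset or respawn logic.
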(event `self.Box.OnComponentBeginOverlap`
  (params (OverlappedComponent :type "PrimitiveComponent Object Reference") (OtherActor :type "Actor Object Reference") (OtherComp :type "PrimitiveComponent Object Reference") (OtherBodyIndex :type Integer) (bFromSweep :type Boolean) (SweepResult :type "HitResult Structure (by ref)"))
  (if (== OtherActor (`GameplayStatics.GetPlayerCharacter` 0))
    ;[1 1 1] Wiggle platform
    (`KismetSystemLibrary.MoveComponentTo` (`self.Platform`) (0.0 0.0 0.0) (struct :`Pitch` 5.0) true true (/ (`self.TimeToFall`) 8.0))
    (`KismetSystemLibrary.MoveComponentTo` (`self.Platform`) (0.0 0.0 0.0) (struct :`Pitch` -5.0) true true (/ (`self.TimeToFall`) 8.0))
    (`KismetSystemLibrary.MoveComponentTo` (`self.Platform`) (0.0 0.0 0.0) (struct :`Pitch` 5.0) true true (/ (`self.TimeToFall`) 8.0))
    (`KismetSystemLibrary.MoveComponentTo` (`self.Platform`) (0.0 0.0 0.0) (struct :`Pitch` -5.0) true true (/ (`self.TimeToFall`) 8.0))
    (`KismetSystemLibrary.MoveComponentTo` (`self.Platform`) (0.0 0.0 0.0) (struct :`Pitch` 5.0) true true (/ (`self.TimeToFall`) 8.0))
    (`KismetSystemLibrary.MoveComponentTo` (`self.Platform`) (0.0 0.0 0.0) (struct :`Pitch` 5.0 :`Roll` 10.0) true true (/ (`self.TimeToFall`) 4.0))
    (`KismetSystemLibrary.Delay` (/ (`self.TimeToFall`) 4.0))
    (`PrimitiveComponent.SetSimulatePhysics` (`self.Platform`) true)))

(fn `UserConstructionScript`)