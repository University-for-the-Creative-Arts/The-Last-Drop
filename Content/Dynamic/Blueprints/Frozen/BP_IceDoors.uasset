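; Ice door actor that slides two doors apart and runs a cart out to tip, destroy collected ice cubes, then return.
; A chain of timed MoveComponentTo events drives doors and cart, starting at BeginPlay and looping after each close and delay.
; The trigger box collects unique IceCube-tagged actors and also starts the sequence at three or more.
; DestroyIceCubes removes array entries while iterating, so it can skip cubes.
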(event `self.ReceiveBeginPlay`
  ;[1 1 1] Set Start locations
  (set `self.Door1StartLocation` (`SceneComponent.GetRelativeTransform` (`self.Door1`)))
  (set `self.Door2StartLocation` (`SceneComponent.GetRelativeTransform` (`self.Door2`)))
  (set `self.CartStartLocation` (`SceneComponent.GetRelativeTransform` (`self.Cart`)))
  (`self.OpenDoors`))

(event `self.Box.OnComponentBeginOverlap`
  (params (OverlappedComponent :type "PrimitiveComponent Object Reference") (OtherActor :type "Actor Object Reference") (OtherComp :type "PrimitiveComponent Object Reference") (OtherBodyIndex :type Integer) (bFromSweep :type Boolean) (SweepResult :type "HitResult Structure (by ref)"))
  ;[1 1 1] Cart Filled?
  ;;[1 1 1] If has tag and isnt in array then add it to array
  (if (`self.ActorHasTag` OtherActor "IceCube")
    (if (== (`KismetArrayLibrary.Array_Find` (`self.IceCubes`) OtherActor) -1)
      (`KismetArrayLibrary.Array_Add` (`self.IceCubes`) OtherActor)
      ;;[1 1 1] If there are 3 or more then open doors
      (if (>= (`KismetArrayLibrary.Array_Length` (`self.IceCubes`)) 3)
        (`self.OpenDoors`)))))

(event `OpenDoors`
  (bind _door1startlocation (`self.Door1StartLocation`))
  (bind _door2startlocation (`self.Door2StartLocation`))
  ;[1 1 1] Open Doors then move cart
  (`|ExecutionSequence`
    (:`then_0`
      (`KismetSystemLibrary.MoveComponentTo` (`self.Door1`) (`KismetMathLibrary.MakeVector` (+ (.x (.location _door1startlocation)) 175.0) (.y (.location _door1startlocation)) (.z (.location _door1startlocation))) (.rotation _door1startlocation) true false 1.0))
    (:`then_1`
      (`KismetSystemLibrary.MoveComponentTo` (`self.Door2`) (`KismetMathLibrary.MakeVector` (+ (.x (.location _door2startlocation)) -175.0) (.y (.location _door2startlocation)) (.z (.location _door2startlocation))) (.rotation _door2startlocation) true false 1.0)
      (`self.MoveCart`))))

(event `MoveCart`
  (bind _cartstartlocation (`self.CartStartLocation`))
  (bind (_cartstartlocation_location _cartstartlocation_rotation) (`KismetMathLibrary.BreakTransform` (`self.CartStartLocation`)))
  (bind _cartstartlocation_2 (`self.CartStartLocation`))
  (bind _cartstartlocation_3 (`self.CartStartLocation`))
  ;[1 1 1] Move Cart
  ;;[1 1 1] Move cart and rotate
  (`KismetSystemLibrary.MoveComponentTo` (`self.Cart`) (`KismetMathLibrary.MakeVector` (.x (.location _cartstartlocation_3)) (+ (.y (.location _cartstartlocation_3)) -610.0) (.z (.location _cartstartlocation_3))) (.rotation _cartstartlocation_3) false true 3.0)
  (`KismetSystemLibrary.MoveComponentTo` (`self.Cart`) (`KismetMathLibrary.MakeVector` (.x (.location _cartstartlocation)) (+ (.y (.location _cartstartlocation)) -610.0) (.z (.location _cartstartlocation))) (`KismetMathLibrary.MakeRotator` (+ (.roll (.rotation _cartstartlocation)) -60.0) (.pitch (.rotation _cartstartlocation)) (.yaw (.rotation _cartstartlocation))) true false 3.0)
  ;;[1 1 1] Move cart back and destroy ice cubes
  (`KismetSystemLibrary.Delay` 0.2)
  (`self.DestroyIceCubes`)
  (`KismetSystemLibrary.MoveComponentTo` (`self.Cart`) (`KismetMathLibrary.MakeVector` (.x (.location _cartstartlocation_2)) (+ (.y (.location _cartstartlocation_2)) -610.0) (.z (.location _cartstartlocation_2))) (.rotation _cartstartlocation_2) false true 2.0)
  (`KismetSystemLibrary.MoveComponentTo` (`self.Cart`) _cartstartlocation_location _cartstartlocation_rotation true true 2.0)
  (`self.CloseDoors`))

(event `CloseDoors`
  (bind (_door1startlocation_location _door1startlocation_rotation) (`KismetMathLibrary.BreakTransform` (`self.Door1StartLocation`)))
  (bind (_door2startlocation_location _door2startlocation_rotation) (`KismetMathLibrary.BreakTransform` (`self.Door2StartLocation`)))
  ;[1 1 1] Close Doors
  (`|ExecutionSequence`
    (:`then_0`
      (`KismetSystemLibrary.MoveComponentTo` (`self.Door1`) _door1startlocation_location _door1startlocation_rotation true false 1.0))
    (:`then_1`
      (`KismetSystemLibrary.MoveComponentTo` (`self.Door2`) _door2startlocation_location _door2startlocation_rotation true false 1.0)
      (if true
        (`KismetSystemLibrary.Delay` 4.0)
        (`self.OpenDoors`)))))

(fn `DestroyIceCubes`
  ;[1 1 1] Destroy ice cubes
  (for _array_element (`self.IceCubes`)
    ;;[1 1 1] If actor is valid, destory and remove it from array, if not just remove it
    (`/Engine/EditorBlueprintResources/StandardMacros.IsValid` _array_element
      (:`Is Valid`
        (`self.K2_DestroyActor` _array_element)
        (`KismetArrayLibrary.Array_RemoveItem` (`self.IceCubes`) _array_element))
      (:`Is Not Valid`
        (`KismetArrayLibrary.Array_RemoveItem` (`self.IceCubes`) _array_element))))
  (return))

(fn `UserConstructionScript`)