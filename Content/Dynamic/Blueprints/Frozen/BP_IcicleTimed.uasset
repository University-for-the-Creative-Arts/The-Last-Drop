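; BP_IcicleTimed is an icicle that drops in a repeating, ordered sequence with other instances.
; Order 0 starts on BeginPlay; each icicle waits TimeToNext, spawns BP_Fractured_Icicle, hides its mesh and triggers that copy's Decay.
; It finds the next Order through GetAllActorsOfClass, or restarts at 0 if IsFinal.
; It then resets with a random yaw and a timeline that grows the GeometryCollection back from zero scale.
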(event `self.ReceiveBeginPlay`
  ;[1 1 1] Start cones
  (`self.Start Cones`))

(event `Start Cones`
  ;[1 1 1] If is starting cone, fall
  (if (== (`self.Order`) 0)
    (`self.Fall Cone`)))

(event `Fall Cone`
  ;[1 1 1] Delay, spawn cone actor, disable visibility of SM, start next item, 3 second delay then destroy cone actor
  (`KismetSystemLibrary.Delay` (`self.TimeToNext`))
  (bind _returnvalue (`|SpawnActorFromClass` "/Game/Dynamic/Blueprints/Frozen/BP_Fractured_Icicle.BP_Fractured_Icicle_C" (`self.GetTransform`) "Undefined" "MultiplyWithRoot" null null))
  (`|ExecutionSequence`
    (:`then_0`
      (`SceneComponent.SetVisibility` (`self.GeometryCollection`) false false)
      (`self.Next Item`))
    (:`then_1`
      (`/Game/Dynamic/Blueprints/Frozen/BP_Fractured_Icicle.Decay` _returnvalue))))

(event `Next Item`
  ;[1 1 1] Next cone
  (if (`self.IsFinal`)
    ;;[1 1 1] Restarts conr sequence
    (bind _outactors (`GameplayStatics.GetAllActorsOfClass` "BP_IcicleTimed_C"))
    (for _array_element _outactors
      (bind _asbp_icicle_timed (cast `/Game/Dynamic/Blueprints/Frozen/BP_IcicleTimed` _array_element))
      (if (== (`/Game/Dynamic/Blueprints/Frozen/BP_IcicleTimed.Order` _asbp_icicle_timed) 0)
        (`self.Start Cones` _asbp_icicle_timed)))
    (`self.Reset Main Cone`)
    (else
      ;;[1 1 1] Gets next item in order, then fall
      (bind _outactors_2 (`GameplayStatics.GetAllActorsOfClass` "BP_IcicleTimed_C"))
      (for _array_element_2 _outactors_2
        (bind _asbp_icicle_timed_2 (cast `/Game/Dynamic/Blueprints/Frozen/BP_IcicleTimed` _array_element_2))
        (if (== (`/Game/Dynamic/Blueprints/Frozen/BP_IcicleTimed.Order` _asbp_icicle_timed_2) (+ (`self.Order`) 1))
          (`self.Fall Cone` _asbp_icicle_timed_2)))
      (`self.Reset Main Cone`))))

(event `Reset Main Cone`
  ;[1 1 1] Resart SM cone visual
  (`self.K2_SetActorRotation` (`KismetMathLibrary.MakeRotator` 0.0 0.0 (`KismetMathLibrary.RandomFloatInRange` -360.0 360.0)))
  (`SceneComponent.SetVisibility` (`self.GeometryCollection`) true false)
  (bind (_direction _grow) (`Timeline|Timeline` :!via `PlayFromStart`)
    (:`Update`
      (bind _returnvalue (`KismetMathLibrary.Lerp` 0.0 1.0 _grow))
      (`SceneComponent.SetWorldScale3D` (`self.GeometryCollection`) (`KismetMathLibrary.MakeVector` _returnvalue _returnvalue _returnvalue)))))

(fn `UserConstructionScript`)