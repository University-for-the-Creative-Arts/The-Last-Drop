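; BP_IceSpawner is an actor that keeps spawning BP_IceCube actors at its own transform, starting on BeginPlay.
; A self-calling Spawn event loops on delays, spawning only while fewer than five cubes wait and otherwise printing a message and retrying later.
; The Waiting component's overlap events add and remove actors tagged IceCube from the WaitingCubes array, which limits the spawning.
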(event `self.ReceiveBeginPlay`
  (`self.Spawn`))

(event `Spawn`
  (if (< (`KismetArrayLibrary.Array_Length` (`self.WaitingCubes`)) 5)
    (`|SpawnActorFromClass` "/Game/Dynamic/Blueprints/Frozen/BP_IceCube.BP_IceCube_C" (`self.GetTransform`) "Undefined" "MultiplyWithRoot" null null)
    (`KismetSystemLibrary.Delay` 3.0)
    (`self.Spawn`)
    (else
      (`KismetSystemLibrary.PrintString` "noroom" false)
      (`KismetSystemLibrary.Delay` 4.0)
      (`self.Spawn`))))

(event `self.Waiting.OnComponentBeginOverlap`
  (params (OverlappedComponent :type "PrimitiveComponent Object Reference") (OtherActor :type "Actor Object Reference") (OtherComp :type "PrimitiveComponent Object Reference") (OtherBodyIndex :type Integer) (bFromSweep :type Boolean) (SweepResult :type "HitResult Structure (by ref)"))
  (bind _waitingcubes (`self.WaitingCubes`))
  (if (`self.ActorHasTag` OtherActor "IceCube")
    (if (== (`KismetArrayLibrary.Array_Find` (`self.WaitingCubes`) OtherActor) -1)
      (`KismetArrayLibrary.Array_Add` _waitingcubes OtherActor)
      (`KismetSystemLibrary.PrintString` (`KismetStringLibrary.Conv_IntToString` (`KismetArrayLibrary.Array_Length` _waitingcubes))))))

(event `self.Waiting.OnComponentEndOverlap`
  (params (OverlappedComponent :type "PrimitiveComponent Object Reference") (OtherActor :type "Actor Object Reference") (OtherComp :type "PrimitiveComponent Object Reference") (OtherBodyIndex :type Integer))
  (if (`self.ActorHasTag` OtherActor "IceCube")
    (`KismetArrayLibrary.Array_RemoveItem` (`self.WaitingCubes`) OtherActor)))

(fn `UserConstructionScript`)