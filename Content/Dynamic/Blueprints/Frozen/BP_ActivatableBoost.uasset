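; Activatable boost pad that pushes the ice ball along the direction of the pad's arrow.
; Activate/Deactivate toggles whether boosting is allowed on each call, or keeps it enabled when AlwaysActive is set.
; On overlap, an enabled pad applies a mass-independent force to the ball's sphere, scaled by BoostMultiplier.
; An IsBoosting flag blocks repeat pushes until the ball leaves the box.
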(event `self.Activate/Deactivate`
  (if (`self.Always Active`)
    (set `self.CanBoost` true)
    (else
      (`/Engine/EditorBlueprintResources/StandardMacros.FlipFlop`
        (:`A`
          (set `self.CanBoost` true))
        (:`B`
          (set `self.CanBoost` false))))))

(event `self.BoostBox.OnComponentBeginOverlap`
  (params (OverlappedComponent :type "PrimitiveComponent Object Reference") (OtherActor :type "Actor Object Reference") (OtherComp :type "PrimitiveComponent Object Reference") (OtherBodyIndex :type Integer) (bFromSweep :type Boolean) (SweepResult :type "HitResult Structure (by ref)"))
  ;[1 1 1] If not already boosting, then boost based on forward vector of arrow
  (if (`self.CanBoost`)
    (if (not (`self.IsBoosting`))
      (bind _asbp_ice_ball (cast `/Game/Dynamic/Blueprints/Characters/IceBallBP/BP_IceBall` OtherActor))
      (`PrimitiveComponent.AddForce` (`/Game/Dynamic/Blueprints/Characters/IceBallBP/BP_IceBall.Sphere` _asbp_ice_ball) (* (`SceneComponent.GetForwardVector` (`self.Arrow`)) (* (`self.BoostMultiplier`) 10000.0)) "None" true)
      (set `self.IsBoosting` true))))

(event `self.BoostBox.OnComponentEndOverlap`
  (params (OverlappedComponent :type "PrimitiveComponent Object Reference") (OtherActor :type "Actor Object Reference") (OtherComp :type "PrimitiveComponent Object Reference") (OtherBodyIndex :type Integer))
  ;[1 1 1] Stop boosting
  (cast `/Game/Dynamic/Blueprints/Characters/IceBallBP/BP_IceBall` OtherActor)
  (set `self.IsBoosting` false))

(fn `UserConstructionScript`
  (`parent.UserConstructionScript`))