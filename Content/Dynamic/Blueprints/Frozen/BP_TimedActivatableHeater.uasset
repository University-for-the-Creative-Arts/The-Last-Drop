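; Timed heater hazard that melts BP_IceBall actors on contact, likely for a frozen-themed level.
; From BeginPlay, HeaterOn and HeaterOff call each other through a shared delay, pulsing the Niagara effect.
; Overlapping the Heater component destroys Meltable-tagged ice balls with a spark effect, gated only by IsOn, so melting continues during the visual off phase.
; Activate/Deactivate only switches the heater off, clearing IsOn to end the cycle.
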(event `self.ReceiveBeginPlay`
  (`self.Heater On`))

(event `Heater On`
  ;[1 1 1] Heater loop cycle
  (if (`self.IsOn`)
    (`ActorComponent.Activate` (`self.Niagara`) false)
    (`KismetSystemLibrary.Delay` (`self.Delay`))
    (if (`self.IsOn`)
      (`self.Heater Off`))
    (else
      (`self.Heater Off`))))

(event `Heater Off`
  (bind _niagara (`self.Niagara`))
  ;[1 1 1] Heater loop cycle
  (`/Engine/EditorBlueprintResources/StandardMacros.IsValid` _niagara
    (:`Is Valid`
      (`ActorComponent.Deactivate` _niagara)
      (`KismetSystemLibrary.Delay` (`self.Delay`))
      (if (`self.IsOn`)
        (`self.Heater On`)))))

(event `self.Activate/Deactivate`
  ;[1 1 1] Activate disables heater
  (set `self.IsOn` false)
  (`self.Heater Off`))

(event `self.Heater.OnComponentBeginOverlap`
  (params (OverlappedComponent :type "PrimitiveComponent Object Reference") (OtherActor :type "Actor Object Reference") (OtherComp :type "PrimitiveComponent Object Reference") (OtherBodyIndex :type Integer) (bFromSweep :type Boolean) (SweepResult :type "HitResult Structure (by ref)"))
  (if (`self.IsOn`)
    (if (`self.ActorHasTag` OtherActor "Meltable")
      (bind _asbp_ice_ball (cast `/Game/Dynamic/Blueprints/Characters/IceBallBP/BP_IceBall` OtherActor))
      (bind (_returnvalue_location _returnvalue_rotation) (`KismetMathLibrary.BreakTransform` (`self.GetTransform` _asbp_ice_ball)))
      (`NiagaraFunctionLibrary.SpawnSystemAtLocation` "/Game/Dynamic/Niagara/NS_IceSpark.NS_IceSpark" _returnvalue_location _returnvalue_rotation (0.5 0.5 0.5))
      (`self.K2_DestroyActor` _asbp_ice_ball))))

(fn `UserConstructionScript`
  (`parent.UserConstructionScript`))