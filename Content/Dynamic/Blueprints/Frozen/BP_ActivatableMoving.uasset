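; BP_ActivatableMoving is an activatable bridge that slides into place, apparently as a puzzle reward.
; Activate/Deactivate sets Solved and triggers MOVE, which plays a timeline that moves the Bridge's relative X toward the End component and unhides the bridge and railings.
; The lerp starts from the bridge's current X on every update, so motion compounds rather than following the curve linearly.
; Unwired leftovers include a puzzle-side cast note and a MoveComponentTo alternative.
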(event `self.Activate/Deactivate`
  (set `self.Solved` true)
  (`self.MOVE`))

(event `MOVE`
  (bind _relativelocation_x (`KismetMathLibrary.BreakVector` (`SceneComponent.RelativeLocation` (`self.End`))))
  (bind _relativelocation_x_2 (`KismetMathLibrary.BreakVector` (`SceneComponent.RelativeLocation` (`self.Bridge`))))
  (if (`self.Solved`)
    (bind (_direction _curve) (`Timeline|Timeline` :`NewTime` (`self.MoveTime`) :!via `PlayFromStart`)
      (:`Update`
        (`SceneComponent.K2_SetRelativeLocation` (`self.Bridge`) (`KismetMathLibrary.MakeVector` (`KismetMathLibrary.Lerp` _relativelocation_x_2 _relativelocation_x _curve)) false false)
        (`SceneComponent.SetHiddenInGame` (`self.Bridge`) false false)
        (`SceneComponent.SetHiddenInGame` (`self.Railing1`) false false)
        (`SceneComponent.SetHiddenInGame` (`self.Railing`) false false)))))

(fn `UserConstructionScript`
  (`parent.UserConstructionScript`))