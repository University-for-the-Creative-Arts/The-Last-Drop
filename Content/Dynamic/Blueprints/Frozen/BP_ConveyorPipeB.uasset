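; BP_ConveyorPipeB is a conveyor pipe that appears and slides along its local Y axis when SpawnPipe is triggered.
; BeginPlay caches the Pipe component's starting relative location.
; SpawnPipe unhides the pipe and restarts the PipeMovement timeline, whose track value is subtracted from the starting Y while roll stays fixed at a right angle.
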(event `self.ReceiveBeginPlay`
  (set `self.Pipe Starting Position` (`SceneComponent.RelativeLocation` (`self.Pipe`))))

(event `SpawnPipe`
  (bind (_pipe_starting_position_x _pipe_starting_position_y _pipe_starting_position_z) (`KismetMathLibrary.BreakVector` (`self.Pipe Starting Position`)))
  (`SceneComponent.SetHiddenInGame` (`self.Pipe`) false false)
  (bind (_direction _newtrack_1) (`Timeline|PipeMovement` :!via `PlayFromStart`)
    (:`Update`
      (`SceneComponent.K2_SetRelativeLocationAndRotation` (`self.Pipe`) (`KismetMathLibrary.MakeVector` _pipe_starting_position_x (- _pipe_starting_position_y _newtrack_1) _pipe_starting_position_z) (`KismetMathLibrary.MakeRotator` 90.0) false false))))

(fn `UserConstructionScript`)