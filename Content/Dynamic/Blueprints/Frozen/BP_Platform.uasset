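; BP_Platform is a moving platform that eases its SM component between relative location and rotation targets PointA and PointB.
; It can start toward PointA on BeginPlay; when looping, each move waits a stay duration, then re-triggers ToPoint toward the other point.
; The next target is chosen by comparing the last location to PointA within a tolerance.
; The construction script adds arrow components at an array of positions.
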(event `self.ReceiveBeginPlay`
  ;[1 1 1] If Starts on play, go to point A
  (if (`self.StartOnPlay`)
    (`self.To Point` (`self.Point A`) (`self.Point A Rotation`))))

(event `To Point`
  (params (`Relative Location` :type "Vector Structure") (`Relative Rotation` :type "Rotator Structure"))
  ;[1 1 1] Move
  ;;[1 1 1] Move to point
  (`KismetSystemLibrary.MoveComponentTo` (`self.SM`) `Relative Location` `Relative Rotation` true true (`self.Move Time`))
  (`KismetSystemLibrary.Delay` (`self.StayDuration`))
  ;;[1 1 1] If looping, then loop
  (if (`self.IsLooping`)
    ;;[1 1 1] Go to next point
    (if (== (`self.Point A`) `Relative Location` :`ErrorTolerance` 10.0)
      (`self.To Point` (`self.Point B`) (`self.Point B Rotation`))
      (else
        (`self.To Point` (`self.Point A`) (`self.Point A Rotation`))))))

(fn `UserConstructionScript`
  (for _array_element _
    (`AddComponent|NODE_AddArrowComponent-0` :`RelativeTransform` (`KismetMathLibrary.MakeTransform` _array_element))))