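; BP_Blade is a swinging blade trap that breaks the player's ice ball.
; From BeginPlay it loops by calling itself, using MoveComponentTo to pitch the blade quickly, pause, then ease back to its start rotation.
; A BP_BubbleChar entering the box during the fast stroke has its bubble state, lifespan and material reset.
; The view target then returns to the player's BP_BodyChar and the bubble pops.
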(event `self.ReceiveBeginPlay`
  (set `self.Start Rotation` (`SceneComponent.RelativeRotation` (`self.SM_Blade`)))
  (`KismetSystemLibrary.Delay` 1.0)
  (set `self.IsLooping` true)
  (`self.Loop`))

(event `Loop`
  (bind _sm_blade (`self.SM_Blade`))
  (bind _sm_blade_2 (`self.SM_Blade`))
  (bind (_relativerotation_roll _relativerotation_pitch _relativerotation_yaw) (`KismetMathLibrary.BreakRotator` (`SceneComponent.RelativeRotation` _sm_blade_2)))
  (set `self.IsSwinging` true)
  (`KismetSystemLibrary.MoveComponentTo` _sm_blade_2 (`SceneComponent.RelativeLocation` _sm_blade_2) (`KismetMathLibrary.MakeRotator` _relativerotation_roll (+ _relativerotation_pitch 70.0) _relativerotation_yaw) false true 0.1)
  (set `self.IsSwinging` false)
  (`KismetSystemLibrary.Delay` 0.5)
  (`KismetSystemLibrary.MoveComponentTo` _sm_blade (`SceneComponent.RelativeLocation` _sm_blade) (`self.Start Rotation`) true true 0.4)
  (`KismetSystemLibrary.Delay` 1.0)
  (if (`self.IsLooping`)
    (`self.Loop`)))

(event `self.Box.OnComponentBeginOverlap`
  (params (OverlappedComponent :type "PrimitiveComponent Object Reference") (OtherActor :type "Actor Object Reference") (OtherComp :type "PrimitiveComponent Object Reference") (OtherBodyIndex :type Integer) (bFromSweep :type Boolean) (SweepResult :type "HitResult Structure (by ref)"))
  (if (`self.IsSwinging`)
    (bind _asbp_bubble_char (cast `/Game/Dynamic/Blueprints/Characters/BubbleChar/BP_BubbleChar` OtherActor))
    (`self.Destroy Ice Ball` _asbp_bubble_char)))

(fn `Destroy Ice Ball`
  (params (Target :type "/Game/Dynamic/Blueprints/Characters/BubbleChar/BP_BubbleChar Object Reference"))
  (set `SurfaceStateComponent.BubbleStates` "Default" (`/Game/Dynamic/Blueprints/Characters/BubbleChar/BP_BubbleChar.AC_BubbleStates` Target))
  (set `/Game/Dynamic/Blueprints/Actor_Components/AC_BubbleStats.Lifespan` 10.0 (`/Game/Dynamic/Blueprints/Characters/BubbleChar/BP_BubbleChar.AC_BubbleStats` Target))
  (bind _returnvalue (`PrimitiveComponent.CreateDynamicMaterialInstance` (`/Game/Dynamic/Blueprints/Characters/BubbleChar/BP_BubbleChar.Sphere` Target) 0 "/Game/Dynamic/Blueprints/Characters/BubbleChar/MI_Bubble.MI_Bubble" "None"))
  (set `/Game/Dynamic/Blueprints/Characters/BubbleChar/BP_BubbleChar.BubbleMaterial` _returnvalue Target)
  (bind _asbp_body_char (cast `/Game/Dynamic/Blueprints/Characters/BodyChar/BP_BodyChar` (`GameplayStatics.GetPlayerCharacter` 0)))
  (`PlayerController.SetViewTargetWithBlend` (`PlayerState.GetPlayerController` (`Pawn.PlayerState` _asbp_body_char)) _asbp_body_char 0.0 "VTBlend_Linear" 0.0 false)
  (`/Game/Dynamic/Blueprints/Actor_Components/AC_BubbleControls.Pop` (`/Game/Dynamic/Blueprints/Characters/BubbleChar/BP_BubbleChar.AC_BubbleControls` Target) Target))

(fn `UserConstructionScript`)