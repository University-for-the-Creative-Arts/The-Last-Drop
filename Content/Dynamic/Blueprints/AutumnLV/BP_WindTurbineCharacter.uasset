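; Wind turbine that can be switched on and off, lifting BP_BodyChar characters that enter its box while it runs.
; SwitchOn/Off plays or reverses the Spin timeline, whose value scales the fan's per-update yaw rotation.
; Timeline updates also set or pause a FanOn timer, which adds zero rotation.
; Box overlap inverts gravity and sets upward velocity with a small downward force; leaving sets gravity scale to a fixed positive value.
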(event `Switch On/Off`
  (if (`self.IsFanOn?`)
    (set `self.IsFanOn?` false)
    (bind (_direction _newtrack_0) (`Timeline|Spin` :!via `Reverse` :!label _label)
      (:`Update`
        (`SceneComponent.K2_AddRelativeRotation` (`self.FanPart`) (`KismetMathLibrary.MakeRotator` 0.0 0.0 (`KismetMathLibrary.Lerp` 0.0 22.5 _newtrack_0)) false false)
        (if (not (`self.IsFanOn?`))
          (`KismetSystemLibrary.K2_PauseTimerHandle` (stale _returnvalue))
          (else
            (bind _returnvalue (`KismetSystemLibrary.K2_SetTimerDelegate` (delegate `FanOn`) (`GameplayStatics.GetWorldDeltaSeconds`)))))))
    (else
      (set `self.IsFanOn?` true)
      (goto _label))))

(event `FanOn`
  (`SceneComponent.K2_AddRelativeRotation` :`self` (`self.FanPart`)))

(event `self.Box.OnComponentBeginOverlap`
  (params (OverlappedComponent :type "PrimitiveComponent Object Reference") (OtherActor :type "Actor Object Reference") (OtherComp :type "PrimitiveComponent Object Reference") (OtherBodyIndex :type Integer) (bFromSweep :type Boolean) (SweepResult :type "HitResult Structure (by ref)"))
  (if (`self.IsFanOn?`)
    (bind _asbp_body_char (cast `/Game/Dynamic/Blueprints/Characters/BodyChar/BP_BodyChar` OtherActor))
    (bind _charactermovement (`Character.CharacterMovement` _asbp_body_char))
    (set `CharacterMovementComponent.GravityScale` -1.0 _charactermovement)
    (set `MovementComponent.Velocity` (0.0 0.0 100.0) _charactermovement)
    (`CharacterMovementComponent.AddForce` _charactermovement (0.0 0.0 -100.0))))

(event `self.Box.OnComponentEndOverlap`
  (params (OverlappedComponent :type "PrimitiveComponent Object Reference") (OtherActor :type "Actor Object Reference") (OtherComp :type "PrimitiveComponent Object Reference") (OtherBodyIndex :type Integer))
  (bind _asbp_body_char (cast `/Game/Dynamic/Blueprints/Characters/BodyChar/BP_BodyChar` OtherActor))
  (set `CharacterMovementComponent.GravityScale` 1.75 (`Character.CharacterMovement` _asbp_body_char)))

(fn `UserConstructionScript`)