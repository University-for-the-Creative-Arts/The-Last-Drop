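; BP_ElectricDoor is an Autumn level obstacle that is destroyed through its Flammable event, meant to fire when a burning bubble touches it.
; On BeginPlay it calls UpdateDataStatic and caches the player as BP_BodyChar.
; Flammable removes the Box component and disables actor collision at once, then prints a debug string and destroys the actor after a short delay.
; Despite the name, the graph contains no electrical or opening logic.
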(event `self.ReceiveBeginPlay`
  (`self.UpdateDataStatic`)
  (bind _asbp_body_char (cast `/Game/Dynamic/Blueprints/Characters/BodyChar/BP_BodyChar` (`GameplayStatics.GetPlayerCharacter` 0)))
  (set `self.Player` _asbp_body_char))

(event `self.Flammable`
  ;[1 1 1] Once the burning bubble touches the object, burns it and destroys it.
  (`ActorComponent.K2_DestroyComponent` (`self.Box`))
  (`self.SetActorEnableCollision` false)
  (`KismetSystemLibrary.Delay` 2.0)
  (`KismetSystemLibrary.PrintString` "DestroyedWall" true true (struct :`R` 1.0 :`G` 0.298067 :`B` 0.288119 :`A` 1.0))
  (`self.K2_DestroyActor`))

(fn `UserConstructionScript`
  (`parent.UserConstructionScript`))