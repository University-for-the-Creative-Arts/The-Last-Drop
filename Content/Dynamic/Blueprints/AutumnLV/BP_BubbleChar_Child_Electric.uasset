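; Electric variant of the bubble character that triggers flammable objects on contact and resets unfinished torch puzzles when popped.
; On BeginPlay it registers itself with the body character's bubble controller and bandit player controller, and binds the pop input to DisableTorches on every incomplete BP_TorchManager.
; Its Sphere1 overlap sends FlammableMessage to actors implementing BPI_Flammable.
; A player self-kill spawn branch is present but never runs.
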(event `self.ReceiveBeginPlay`
  (bind _ac_bubblecontroller (`/Game/Dynamic/Blueprints/Characters/BodyChar/BP_BodyChar.AC_BubbleController` (`self.BP_BodyChar`)))
  (`parent.ReceiveBeginPlay`)
  (set `/Game/Dynamic/Blueprints/Characters/BodyChar/AC_BubbleController.BP_BubbleChar` self _ac_bubblecontroller)
  (set `/Game/Dynamic/Blueprints/Interfaces/PC_BubbleBandit.BP Bubble Char` self (`/Game/Dynamic/Blueprints/Characters/BodyChar/AC_BubbleController.PC Bubble Bandit` _ac_bubblecontroller))
  (add `/Game/Dynamic/Blueprints/Actor_Components/AC_BubbleControls.IA_Pop` (`self.AC_BubbleControls`) (delegate `DisableTorches`)))

(event `DisableTorches`
  (bind _outactors (`GameplayStatics.GetAllActorsOfClass` "/Game/Dynamic/Blueprints/SummerLV/BP_TorchManager.BP_TorchManager_C"))
  (for _array_element _outactors
    (if (not (`/Game/Dynamic/Blueprints/SummerLV/BP_TorchManager.Complete?` _array_element))
      (`/Game/Dynamic/Blueprints/SummerLV/BP_TorchManager.DisableTorches` _array_element))))

(event `self.Sphere1.OnComponentBeginOverlap`
  (params (OverlappedComponent :type "PrimitiveComponent Object Reference") (OtherActor :type "Actor Object Reference") (OtherComp :type "PrimitiveComponent Object Reference") (OtherBodyIndex :type Integer) (bFromSweep :type Boolean) (SweepResult :type "HitResult Structure (by ref)"))
  (if (`KismetSystemLibrary.DoesImplementInterface` OtherActor "/Game/Dynamic/Blueprints/SummerLV/BPI_Flammable.BPI_Flammable_C")
    (message `/Game/Dynamic/Blueprints/SummerLV/BPI_Flammable.Flammable` OtherActor)))

(fn `UserConstructionScript`
  (`parent.UserConstructionScript`))