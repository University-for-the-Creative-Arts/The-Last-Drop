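; BP_Door is a door that slides a Cube between two marker components, StartLocation and TargetLocation.
; A custom event waits through a short delay, then a FlipFlop plays a timeline that lerps the Cube's world location without sweeping.
; Play and Stop calls, likely for audio, bracket the movement.
; Only the FlipFlop's A branch is wired, so alternate triggers do nothing and no closing motion exists.
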(event `CustomEvent`
  (`KismetSystemLibrary.Delay` 1.0)
  (`/Engine/EditorBlueprintResources/StandardMacros.FlipFlop`
    (:`A`
      (`AudioComponent.Play` 0.0)
      (bind (_direction _newtrack_0 _z) (`Timeline|Timeline`)
        (:`Update`
          (`SceneComponent.K2_SetWorldLocation` (`self.Cube`) (`KismetMathLibrary.VLerp` (`SceneComponent.K2_GetComponentLocation` (`self.StartLocation`)) (`SceneComponent.K2_GetComponentLocation` (`self.TargetLocation`)) _z) false false))
        (:`Finished`
          (`AudioComponent.Stop`))))))

(fn `UserConstructionScript`)