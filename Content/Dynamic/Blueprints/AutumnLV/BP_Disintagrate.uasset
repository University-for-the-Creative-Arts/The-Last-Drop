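; Disintegration effect actor that dissolves a skeletal mesh and a static mesh, each paired with a Niagara system.
; Construction script and update events run setup macros that create dynamic materials and push Alpha, boosted edge colour and textures to meshes, with matching dissolve parameters to Niagara.
; Separate events play a timeline per mesh, starting at a time scaled from Alpha, driving material and particle Alpha together.
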(event `SKTimeline`
  (`|ExecutionSequence`
    (:`then_0`
      (bind (_direction _newtrack_0) (`Timeline|Timeline_1` :`NewTime` (* (`self.Alpha`) 5.0) :!via `SetNewTime` :!label _label)
        (:`Update`
          (`MeshComponent.SetScalarParameterValueOnMaterials` (`self.SkeletalMesh`) "Alpha" _newtrack_0)
          (`NiagaraComponent.SetVariableFloat` (`self.SK_Niagara`) "Alpha" _newtrack_0))))
    (:`then_1`
      (goto _label))))

(event `StaticDisTime`
  (`|ExecutionSequence`
    (:`then_0`
      (bind (_direction _newtrack_0) (`Timeline|Timeline_2` :`NewTime` (* (`self.Alpha`) 2.5) :!via `SetNewTime` :!label _label_2)
        (:`Update`
          (`MeshComponent.SetScalarParameterValueOnMaterials` (`self.StaticMesh`) "Alpha" _newtrack_0)
          (`NiagaraComponent.SetVariableFloat` (`self.Niagara`) "Alpha" _newtrack_0))))
    (:`then_1`
      (goto _label_2))))

(event `UpdateDataSK`
  (`self.SKMesh_Setup` (`self.SK_Niagara`) (`self.SkeletalMesh`)))

(event `UpdateDataStatic`
  (`self.StaticMesh_Setup` (`self.Niagara`) (`self.StaticMesh`)))

(fn `UserConstructionScript`
  (`self.SKMesh_Setup` (`self.SK_Niagara`) (`self.SkeletalMesh`))
  (`self.StaticMesh_Setup` (`self.Niagara`) (`self.StaticMesh`)))