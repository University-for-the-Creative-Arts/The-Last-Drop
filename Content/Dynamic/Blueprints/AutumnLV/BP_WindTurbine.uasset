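; Wind turbine actor that spins its fan mesh and pushes the bubble character with a burst of force.
; A looping timer started on BeginPlay yaws the fan constantly.
; SwitchOnOff adds a timeline-eased spin, then starts or pauses a second spin timer based on IsFanOn on each update.
; Entering the box applies acceleration-based force along E's forward vector, only when the bubble has nothing attached.
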(event `self.ReceiveBeginPlay`
  ;[1 1 1] Starts and spins the static mesh of the turbine and the intensity of the spinning
  (`KismetSystemLibrary.K2_SetTimerDelegate` (delegate `Rotate Fan`) 0.01 true))

(event `Rotate Fan`
  (bind _fanpart (`self.FanPart`))
  (bind (_relativerotation_roll _relativerotation_pitch _relativerotation_yaw) (`KismetMathLibrary.BreakRotator` (`SceneComponent.RelativeRotation` _fanpart)))
  ;[1 1 1] Starts and spins the static mesh of the turbine and the intensity of the spinning
  (`SceneComponent.K2_SetRelativeRotation` _fanpart (`KismetMathLibrary.MakeRotator` _relativerotation_roll _relativerotation_pitch (+ _relativerotation_yaw 8.0)) false false))

(event `self.Box.OnComponentBeginOverlap`
  (params (OverlappedComponent :type "PrimitiveComponent Object Reference") (OtherActor :type "Actor Object Reference") (OtherComp :type "PrimitiveComponent Object Reference") (OtherBodyIndex :type Integer) (bFromSweep :type Boolean) (SweepResult :type "HitResult Structure (by ref)"))
  ;[1 1 1] Force added onto the bubble (with and without attachments)
  (bind _asbp_bubble_char (cast `/Game/Dynamic/Blueprints/Characters/BubbleChar/BP_BubbleChar` OtherActor))
  (if (not (`/Game/Dynamic/Blueprints/Characters/BubbleChar/BP_BubbleChar.HasAttached?` _asbp_bubble_char))
    (`PrimitiveComponent.AddForce` (`Character.CapsuleComponent` _asbp_bubble_char) (* (`SceneComponent.GetForwardVector` (`self.e`)) 60000.0) "None" true)))

(event `SwitchOnOff`
  ;[1 1 1] Fan being turned on
  (bind (_direction _newtrack_0) (`Timeline|Timeline`)
    (:`Update`
      (`SceneComponent.K2_AddRelativeRotation` (`self.FanPart`) (`KismetMathLibrary.MakeRotator` 0.0 0.0 (`KismetMathLibrary.Lerp` 0.0 15.0 _newtrack_0)) false false)
      (if (not (`self.IsFanOn?`))
        (`KismetSystemLibrary.K2_PauseTimerHandle` (stale _returnvalue))
        (else
          (bind _returnvalue (`KismetSystemLibrary.K2_SetTimerDelegate` (delegate `FanOn`) (`GameplayStatics.GetWorldDeltaSeconds`) true)))))))

(event `FanOn`
  ;[1 1 1] Fan being turned on
  (`SceneComponent.K2_AddRelativeRotation` (`self.FanPart`) (struct :`Yaw` 15.0) false false))

(fn `UserConstructionScript`)