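; BP_DownLiftEnd is an ending lift that takes control from the player and fades the screen when they enter its trigger box.
; On overlap it disables input, stops character movement and starts a timeline that offsets the lift's relative Z by a configurable amount.
; The timeline's play rate is scaled by TimeToComplete, and a configurable camera fade begins after half that time.
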(event `Upward`
  (`TimelineComponent.SetPlayRate` (`self.Up`) (/ 1.0 (`self.TimeToComplete`)))
  (bind (_direction _movement) (`Timeline|Up` :!via `PlayFromStart`)
    (:`Update`
      (`SceneComponent.K2_SetRelativeLocation` (`self.Lift`) (`KismetMathLibrary.MakeVector` 0.0 0.0 (* _movement (`self.MovementAmount`))) false false))))

(event `self.Box.OnComponentBeginOverlap`
  (params (OverlappedComponent :type "PrimitiveComponent Object Reference") (OtherActor :type "Actor Object Reference") (OtherComp :type "PrimitiveComponent Object Reference") (OtherBodyIndex :type Integer) (bFromSweep :type Boolean) (SweepResult :type "HitResult Structure (by ref)"))
  (bind _returnvalue (`GameplayStatics.GetPlayerCharacter` 0))
  (if (== OtherActor _returnvalue)
    (`self.StartSequence`)
    (`self.DisableInput` _returnvalue (`GameplayStatics.GetPlayerController` 0))
    (`self.DisableInput` (`GameplayStatics.GetPlayerController` 0) (`GameplayStatics.GetPlayerController` 0))
    (`MovementComponent.StopMovementImmediately` (`Character.CharacterMovement` _returnvalue))))

(event `StartSequence`
  (`self.Upward`)
  (`KismetSystemLibrary.Delay` (/ (`self.TimeToComplete`) 2.0))
  (`PlayerCameraManager.StartCameraFade` (`GameplayStatics.GetPlayerCameraManager` 0) 0.0 (`self.EndAlpha`) (`self.FadeOutDuration`) (`self.FadeColour`) (`self.Should Fade Audio`) (`self.Hold when Finished`)))

(fn `UserConstructionScript`)