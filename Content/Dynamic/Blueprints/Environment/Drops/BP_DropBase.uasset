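; BP_DropBase is a base actor for environment drops that are reused from a pool instead of being destroyed.
; SetInUse switches collision, visibility and tick together, and BeginPlay starts the drop in the inactive state.
; Activation restarts a TimeToLive timer that calls ReturnToPool, which deactivates the drop by calling SetInUse again with false.
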(event `self.ReceiveBeginPlay`
  (`self.Set In Use` false))

(event `Set In Use`
  (params (InUse :type Boolean))
  (set `self.InUse` InUse)
  (`self.SetActorEnableCollision` InUse)
  (`self.SetActorHiddenInGame` (not InUse))
  (`self.SetActorTickEnabled` InUse)
  (`KismetSystemLibrary.K2_ClearAndInvalidateTimerHandle` (`self.TimeTo`))
  (if InUse
    (bind _returnvalue (`KismetSystemLibrary.K2_SetTimerDelegate` (delegate `Return To Pool`) (`self.Time ToLive`)))
    (set `self.TimeTo` _returnvalue)))

(event `Return To Pool`
  (`self.Set In Use` false))

(fn `UserConstructionScript`)