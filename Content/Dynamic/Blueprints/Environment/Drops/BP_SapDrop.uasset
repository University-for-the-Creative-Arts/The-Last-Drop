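; BP_SapDrop is an environment prop that shows a sap drop falling over and over.
; From BeginPlay, a latent MoveComponentTo loop moves the static mesh to EndPos over DropSpeed, which acts as a duration.
; It then spawns a Niagara effect attached to EndPos with a Z offset, waits briefly and moves the mesh back to StartPos with zero duration before repeating.
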(event `self.ReceiveBeginPlay`
  (bind _endpos (`self.EndPos`))
  (`KismetSystemLibrary.MoveComponentTo` (`self.StaticMesh`) (`SceneComponent.RelativeLocation` _endpos) (struct) false false (`self.DropSpeed`) :!label _label)
  (`NiagaraFunctionLibrary.SpawnSystemAttached` "/Game/Dynamic/Niagara/NS_SapTest2.NS_SapTest2" _endpos "None" (0.0 0.0 100.0) (struct) "KeepRelativeOffset")
  (`KismetSystemLibrary.Delay` 0.5)
  (`KismetSystemLibrary.MoveComponentTo` (`self.StaticMesh`) (`SceneComponent.RelativeLocation` (`self.StartPos`)) (struct) false false 0.0)
  (goto _label))

(fn `UserConstructionScript`)