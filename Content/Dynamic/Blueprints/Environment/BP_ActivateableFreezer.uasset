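; Activatable freezer hazard that turns the player's bubble into a heavy ice ball while its trigger box exists.
; An overlapping body character has its sphere hidden and spawns a bubble through AC_BubbleController, which gets the Ice state, ice material and Heavy tag.
; An overlapping bubble only gets the Heavy tag; both paths share the camera blend and half-scale step targeting the overlap's bubble cast.
; Activate/Deactivate destroys the box, permanently disabling the effect.
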(event `self.Activate/Deactivate`
  (`ActorComponent.K2_DestroyComponent` (`self.Box`)))

(event `self.Box.OnComponentBeginOverlap`
  (params (OverlappedComponent :type "PrimitiveComponent Object Reference") (OtherActor :type "Actor Object Reference") (OtherComp :type "PrimitiveComponent Object Reference") (OtherBodyIndex :type Integer) (bFromSweep :type Boolean) (SweepResult :type "HitResult Structure (by ref)"))
  (bind _aspc_bubble_bandit (cast `/Game/Dynamic/Blueprints/Interfaces/PC_BubbleBandit` (`GameplayStatics.GetPlayerController` 0) :!pure true))
  ;[1 1 1] Overlap with bubble
  (bind _asbp_bubble_char (cast `/Game/Dynamic/Blueprints/Characters/BubbleChar/BP_BubbleChar` OtherActor)
    (:`then`
      ;;[1 1 1] Give ice ball heavy tag
      (set `Actor.Tags` (`|MakeArray` "Heavy" :!type "Name") _asbp_bubble_char))
    (:`CastFailed`
      ;[1 1 1] Overlap with player
      (bind _asbp_body_char (cast `/Game/Dynamic/Blueprints/Characters/BodyChar/BP_BodyChar` OtherActor))
      (`SceneComponent.SetVisibility` (`/Game/Dynamic/Blueprints/Characters/BodyChar/BP_BodyChar.Sphere` _asbp_body_char) false false)
      (bind _ac_bubblecontroller (`/Game/Dynamic/Blueprints/Characters/BodyChar/BP_BodyChar.AC_BubbleController` _asbp_body_char))
      (bind _asac_bubble_controller (cast `/Game/Dynamic/Blueprints/Characters/BodyChar/AC_BubbleController` _ac_bubblecontroller))
      (`/Game/Dynamic/Blueprints/Characters/BodyChar/AC_BubbleController.SpawnBubble` _asac_bubble_controller (`/Game/Dynamic/Blueprints/Interfaces/PC_BubbleBandit.Sphere` _aspc_bubble_bandit) _aspc_bubble_bandit)
      (bind _bp_bubblechar (`/Game/Dynamic/Blueprints/Characters/BodyChar/AC_BubbleController.BP_BubbleChar` _ac_bubblecontroller))
      (set `SurfaceStateComponent.BubbleStates` "Ice" (`/Game/Dynamic/Blueprints/Characters/BubbleChar/BP_BubbleChar.AC_BubbleStates` _bp_bubblechar))
      (`PrimitiveComponent.SetMaterial` (`/Game/Dynamic/Blueprints/Characters/BubbleChar/BP_BubbleChar.Sphere` _bp_bubblechar) 0 "/Game/Static/Materials/MAT_Ice.MAT_Ice")
      (set `Actor.Tags` (`|MakeArray` "Heavy" :!type "Name") _bp_bubblechar)))
  ;;[1 1 1] Change cam
  (bind _asbp_body_char_2 (cast `/Game/Dynamic/Blueprints/Characters/BodyChar/BP_BodyChar` (`GameplayStatics.GetPlayerCharacter` 0)))
  (`PlayerController.SetViewTargetWithBlend` (`PlayerState.GetPlayerController` (`Pawn.PlayerState` _asbp_body_char_2)) _asbp_bubble_char 0.0 "VTBlend_Linear" 0.0 false)
  (`SceneComponent.SetRelativeScale3D` (`/Game/Dynamic/Blueprints/Characters/BubbleChar/BP_BubbleChar.Sphere` _asbp_bubble_char) (0.5 0.5 0.5)))

(fn `UserConstructionScript`
  (`parent.UserConstructionScript`))