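; BP_SpinningActor is an environment actor that rotates its static mesh in repeated quarter-turn steps around the roll axis.
; After a configurable delay on BeginPlay, it starts the first spin and sets a looping timer to repeat it every few seconds.
; Each spin caches the mesh's current relative rotation, then a timeline lerps it toward that rotation plus 90 degrees of roll.
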(event `self.ReceiveBeginPlay`
  (`KismetSystemLibrary.Delay` (`self.Delay`))
  (`self.StartSpin`)
  (`KismetSystemLibrary.K2_SetTimerDelegate` (delegate `StartSpin`) 6.0 true))

(event `StartSpin`
  (bind (_relative_rotation_roll _relative_rotation_pitch _relative_rotation_yaw) (`KismetMathLibrary.BreakRotator` (`self.Relative Rotation`)))
  (set `self.Relative Rotation` (`SceneComponent.RelativeRotation` (`self.StaticMesh`)))
  (bind (_direction _newtrack_0) (`Timeline|spin` :!via `PlayFromStart`)
    (:`Update`
      (`SceneComponent.K2_SetRelativeRotation` (`self.StaticMesh`) (`KismetMathLibrary.RLerp` (`self.Relative Rotation`) (`KismetMathLibrary.MakeRotator` (+ _relative_rotation_roll 90.0) _relative_rotation_pitch _relative_rotation_yaw) _newtrack_0) false false))))

(fn `UserConstructionScript`)