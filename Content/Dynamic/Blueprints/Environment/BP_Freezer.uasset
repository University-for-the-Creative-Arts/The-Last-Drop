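; BP_Freezer is an environment actor whose box trigger currently switches the camera rather than freezing anything.
; When a BP_BubbleChar enters the box, the controller of player 0's BP_BodyChar blends its view target to that bubble character.
; Unconnected leftover logic would check a Freezable tag and spawn BP_IceBall with a spark effect; a note marks it unneeded in favor of PM_ICE.
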(event `self.Box.OnComponentBeginOverlap`
  (params (OverlappedComponent :type "PrimitiveComponent Object Reference") (OtherActor :type "Actor Object Reference") (OtherComp :type "PrimitiveComponent Object Reference") (OtherBodyIndex :type Integer) (bFromSweep :type Boolean) (SweepResult :type "HitResult Structure (by ref)"))
  (bind _asbp_bubble_char (cast `/Game/Dynamic/Blueprints/Characters/BubbleChar/BP_BubbleChar` OtherActor))
  (bind _asbp_body_char (cast `/Game/Dynamic/Blueprints/Characters/BodyChar/BP_BodyChar` (`GameplayStatics.GetPlayerCharacter` 0)))
  (`PlayerController.SetViewTargetWithBlend` (`PlayerState.GetPlayerController` (`Pawn.PlayerState` _asbp_body_char)) _asbp_bubble_char 0.0 "VTBlend_Linear" 0.0 false))

(fn `UserConstructionScript`)