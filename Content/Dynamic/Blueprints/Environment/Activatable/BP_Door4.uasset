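; BP_Door4 is an activatable environment actor that removes itself when triggered and doubles as a test death zone.
; Activate/Deactivate waits a second, then a FlipFlop's first output moves the mesh to world origin and destroys the actor; the second output is unused.
; Overlapping PlatformCollision teleports a BP_BodyChar to the temporary RespawnTemp location, a placeholder for a future checkpoint.
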(event `self.Activate/Deactivate`
  (`KismetSystemLibrary.Delay` 1.0)
  (`/Engine/EditorBlueprintResources/StandardMacros.FlipFlop`
    (:`A`
      (`SceneComponent.K2_SetWorldLocation` (`self.StaticMesh`) (0.0 0.0 0.0) false false)
      (`self.K2_DestroyActor`))))

(event `self.PlatformCollision.OnComponentBeginOverlap`
  (params (OverlappedComponent :type "PrimitiveComponent Object Reference") (OtherActor :type "Actor Object Reference") (OtherComp :type "PrimitiveComponent Object Reference") (OtherBodyIndex :type Integer) (bFromSweep :type Boolean) (SweepResult :type "HitResult Structure (by ref)"))
  ;[1 1 1] This is a test death mechanic. Respawn_Temp will be replaced with a checkpoint
  (bind _asbp_body_char (cast `/Game/Dynamic/Blueprints/Characters/BodyChar/BP_BodyChar` OtherActor))
  (`self.K2_SetActorLocation` _asbp_body_char (`SceneComponent.K2_GetComponentLocation` (`self.Respawn_Temp`)) false false))

(fn `UserConstructionScript`
  (`parent.UserConstructionScript`))