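; BP_TipTimerBox is an activatable trigger box that runs a countdown intended to precede a gameplay hint.
; The first overlap while DisplayAHint is set clears that flag, then starts a looping one-second timer if the actor is a BP_BodyChar.
; Each tick decrements TimeBeforeHint and prints the time left as debug text.
; At zero the timer only clears itself; no hint display is implemented here.
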(event `self.Box.OnComponentBeginOverlap`
  (params (OverlappedComponent :type "PrimitiveComponent Object Reference") (OtherActor :type "Actor Object Reference") (OtherComp :type "PrimitiveComponent Object Reference") (OtherBodyIndex :type Integer) (bFromSweep :type Boolean) (SweepResult :type "HitResult Structure (by ref)"))
  (if (`self.displayAHint?`)
    (set `self.displayAHint?` false)
    (cast `/Game/Dynamic/Blueprints/Characters/BodyChar/BP_BodyChar` OtherActor)
    (`KismetSystemLibrary.K2_SetTimer` null "TimerTrackerbeforeHint" 1.0 true)))

(fn `TimerTrackerbeforeHint`
  ;[0.5532 1 0.4835 1 13] Timer function. Taking "Time Before Hint" - 1 sets the new "Time Before Hint" and checks if the "Time Before Hint" <= 0
  (bind _output_get (set `self.timeBeforeHint` (- (`self.timeBeforeHint`) 1.0)))
  (if (<= _output_get 0.0)
    ;[1 0.9017 0.3671] Resets the timer.
    (`KismetSystemLibrary.K2_ClearTimer` null "TimerTrackerbeforeHint")
    (else
      ;[1 1 1] Debug of a timer. countdown
      (`KismetSystemLibrary.PrintString` (`KismetStringLibrary.Concat_StrStr` "Time left before displaying a hint:  " (`KismetStringLibrary.Conv_DoubleToString` _output_get)) true true (struct :`R` 1.0 :`G` 0.949418 :`A` 1.0) 1.0))))

(fn `UserConstructionScript`)