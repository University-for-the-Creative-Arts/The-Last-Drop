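; Activatable sliding door that moves a cube between a start and a target marker when its Activate/Deactivate event fires.
; After a short delay, a FlipFlop alternately plays and reverses a timeline that lerps the cube's world location.
; Audio plays during the movement and stops when the timeline finishes.
; A test death mechanic for respawning BP_BodyChar on platform overlap is left disconnected.
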(event `self.Activate/Deactivate`
  (bind _audio (`self.Audio`))
  (`KismetSystemLibrary.Delay` 1.0)
  (`/Engine/EditorBlueprintResources/StandardMacros.FlipFlop`
    (:`A`
      (`AudioComponent.Play` _audio 0.0)
      (bind (_direction _z) (`Timeline|UPDown` :!label _label)
        (:`Update`
          (`SceneComponent.K2_SetWorldLocation` (`self.Cube`) (`KismetMathLibrary.VLerp` (`SceneComponent.K2_GetComponentLocation` (`self.StartLocation`)) (`SceneComponent.K2_GetComponentLocation` (`self.TargetLocation`)) _z) false false))
        (:`Finished`
          (`AudioComponent.Stop` (`self.Audio`)))))
    (:`B`
      (`AudioComponent.Play` _audio 0.0)
      (goto _label :!via `Reverse`))))

(event `self.PlatformCollision.OnComponentBeginOverlap`
  (params (OverlappedComponent :type "PrimitiveComponent Object Reference") (OtherActor :type "Actor Object Reference") (OtherComp :type "PrimitiveComponent Object Reference") (OtherBodyIndex :type Integer) (bFromSweep :type Boolean) (SweepResult :type "HitResult Structure (by ref)"))
  ;[1 1 1] This is a test death mechanic. Respawn_Temp will be replaced with a checkpoint
)

(fn `UserConstructionScript`
  (`parent.UserConstructionScript`))