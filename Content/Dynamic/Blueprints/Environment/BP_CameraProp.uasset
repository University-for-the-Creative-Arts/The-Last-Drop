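; BP_CameraProp is an environment camera prop that turns to face the player while they are inside its box trigger.
; BP_BodyChar entering the box sets PlayerIN, and any overlap ending clears it without a class check.
; While the flag is set, Tick smoothly interpolates actor rotation toward the player pawn using RInterpTo.
; The starting rotation is stored but never restored, and the SpotLight color change is unconnected.
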(event `self.ReceiveBeginPlay`
  (set `self.startPos` (`self.K2_GetActorRotation`)))

(event `self.ReceiveTick`
  (params (DeltaSeconds :type "Float (single-precision)"))
  (if (`self.PlayerIN?`)
    (`self.K2_SetActorRotation` (`KismetMathLibrary.RInterpTo` (`self.K2_GetActorRotation`) (`KismetMathLibrary.FindLookAtRotation` (`self.K2_GetActorLocation`) (`self.K2_GetActorLocation` (`GameplayStatics.GetPlayerPawn` 0))) (`GameplayStatics.GetWorldDeltaSeconds`) 2.0) true)))

(event `self.Box.OnComponentBeginOverlap`
  (params (OverlappedComponent :type "PrimitiveComponent Object Reference") (OtherActor :type "Actor Object Reference") (OtherComp :type "PrimitiveComponent Object Reference") (OtherBodyIndex :type Integer) (bFromSweep :type Boolean) (SweepResult :type "HitResult Structure (by ref)"))
  (cast `/Game/Dynamic/Blueprints/Characters/BodyChar/BP_BodyChar` OtherActor)
  (set `self.PlayerIN?` true))

(event `self.Box.OnComponentEndOverlap`
  (params (OverlappedComponent :type "PrimitiveComponent Object Reference") (OtherActor :type "Actor Object Reference") (OtherComp :type "PrimitiveComponent Object Reference") (OtherBodyIndex :type Integer))
  (set `self.PlayerIN?` false))

(fn `UserConstructionScript`)