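; BP_BubbleElectric is a bubble character Blueprint, named as the electric variant, that relies on its parent class for its behavior.
; On BeginPlay it runs the parent logic, then registers itself as the active BPBubbleChar on the body character's ACBubbleController and on that controller's PCBubbleBandit.
; It adds no electric-specific logic: overlap and Tick are disabled stubs, and construction only calls the parent.
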(event `self.ReceiveBeginPlay`
  (bind _ac_bubblecontroller (`/Game/Dynamic/Blueprints/Characters/BodyChar/BP_BodyChar.AC_BubbleController` (`self.BP_BodyChar`)))
  (`parent.ReceiveBeginPlay`)
  (set `/Game/Dynamic/Blueprints/Characters/BodyChar/AC_BubbleController.BP_BubbleChar` self _ac_bubblecontroller)
  (set `/Game/Dynamic/Blueprints/Interfaces/PC_BubbleBandit.BP Bubble Char` self (`/Game/Dynamic/Blueprints/Characters/BodyChar/AC_BubbleController.PC Bubble Bandit` _ac_bubblecontroller)))

(fn `UserConstructionScript`
  (`parent.UserConstructionScript`))