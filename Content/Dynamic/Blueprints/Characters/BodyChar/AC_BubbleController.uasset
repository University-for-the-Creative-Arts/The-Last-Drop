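; Actor component on BP_BodyChar that spawns and launches the player's bubble character, allowing one at a time.
; SpawnBubble creates BP_BubbleChar at the body, shares it with the Bubble Bandit player controller, and impulses it toward the cursor's hit point.
; It then registers the bubble with the body's camera behaviour for tracking and signals the spawn.
; PopReset clears the bubble reference and makes the given sphere visible again.
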(fn `Pop Reset`
  (params (Sphere :type "StaticMeshComponent Object Reference"))
  (set `self.BP_BubbleChar` null)
  (`SceneComponent.SetVisibility` Sphere true false))

(fn `SpawnBubble`
  (params (SMAC_Sphere :type "StaticMeshComponent Object Reference") (PC_BubbleBandit :type "/Game/Dynamic/Blueprints/Interfaces/PC_BubbleBandit Object Reference"))
  (locals (BP_BubbleChar :type "/Game/Dynamic/Blueprints/Characters/BubbleChar/BP_BubbleChar Object Reference") (BP_BodyChar :type "/Game/Dynamic/Blueprints/Characters/BodyChar/BP_BodyChar Object Reference"))
  (bind _pc_bubble_bandit (`self.PC Bubble Bandit`))
  (bind _bp_bodychar (`local.BP_BodyChar`))
  (`self.BP_BubbleChar`
    (:`then`)
    (:`else`
      (bind _asbp_body_char (cast `/Game/Dynamic/Blueprints/Characters/BodyChar/BP_BodyChar` (`self.GetOwner`)))
      (set `local.BP_BodyChar` _asbp_body_char)
      (set `self.PC Bubble Bandit` PC_BubbleBandit)
      (if (not (`KismetSystemLibrary.IsValid` (`local.BP_BubbleChar`)))
        (bind _returnvalue (`|SpawnActorFromClass` "/Game/Dynamic/Blueprints/Characters/BubbleChar/BP_BubbleChar.BP_BubbleChar_C" (`KismetMathLibrary.MakeTransform` (`SceneComponent.K2_GetComponentLocation` (`Actor.RootComponent` _bp_bodychar))) "Undefined" "MultiplyWithRoot" null _bp_bodychar null))
        (bind _output_get (set `self.BP_BubbleChar` _returnvalue))
        (set `/Game/Dynamic/Blueprints/Interfaces/PC_BubbleBandit.BP Bubble Char` _output_get _pc_bubble_bandit)
        (if (`KismetSystemLibrary.IsValid` _pc_bubble_bandit)
          (`PrimitiveComponent.AddImpulse` (`Character.CapsuleComponent` _output_get) (* (`KismetMathLibrary.GetDirectionUnitVector` (`SceneComponent.K2_GetComponentLocation` (`Actor.RootComponent` (`local.BP_BodyChar`))) (`.Location` (`GameplayStatics.BreakHitResult` (`PlayerController.GetHitResultUnderCursorByChannel` (`GameplayStatics.GetPlayerController` 0) "TraceTypeQuery1" true)))) (`self.LaunchForce`)) "None" true)
          (bind _asactor (cast `Actor` (`self.BP_BubbleChar`)))
          (`/Game/Dynamic/Blueprints/Actor_Components/AC_CamBehaviour.AddTrackingActor` (`/Game/Dynamic/Blueprints/Characters/BodyChar/BP_BodyChar.AC_CamBehaviour` (`local.BP_BodyChar`)) _asactor)
          (`self.IA_BubbleSpawn`)
          (return))))))