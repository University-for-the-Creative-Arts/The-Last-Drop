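; BP_IceBall is a physics ball that constantly rolls toward the point under the mouse cursor.
; Each Tick, Move traces under the cursor and applies horizontal acceleration to the sphere in that direction.
; During play it registers as a tracking actor with the player character's camera behaviour component.
; Player overlap only prints a pickup placeholder, and LaunchBall, uncalled here, applies an impulse scaled from the sphere's world location.
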(event `self.ReceiveTick`
  (params (DeltaSeconds :type "Float (single-precision)"))
  ;[1 1 1] Move ball constantally
  (`self.Move`))

(event `self.ReceiveBeginPlay`
  ;[1 1 1] Tack the ball on play, stop on end
  (bind _asbp_body_char (cast `/Game/Dynamic/Blueprints/Characters/BodyChar/BP_BodyChar` (`GameplayStatics.GetPlayerCharacter` 0)))
  (`/Game/Dynamic/Blueprints/Characters/Components/AC_CamBehaviour.AddTrackingActor` (`/Game/Dynamic/Blueprints/Characters/BodyChar/BP_BodyChar.AC_CamBehaviour` _asbp_body_char) self))

(event `self.ReceiveEndPlay`
  (params (EndPlayReason :type "EEndPlayReason Enum" :default "Destroyed"))
  ;[1 1 1] Tack the ball on play, stop on end
  (`/Game/Dynamic/Blueprints/Characters/Components/AC_CamBehaviour.RemoveTrackingActor` (`/Game/Dynamic/Blueprints/Characters/BodyChar/BP_BodyChar.AC_CamBehaviour` (stale `self.ReceiveBeginPlay` _asbp_body_char)) self))

(event `self.Collision.OnComponentBeginOverlap`
  (params (OverlappedComponent :type "PrimitiveComponent Object Reference") (OtherActor :type "Actor Object Reference") (OtherComp :type "PrimitiveComponent Object Reference") (OtherBodyIndex :type Integer) (bFromSweep :type Boolean) (SweepResult :type "HitResult Structure (by ref)"))
  ;[1 1 1] Pick up (Add later)
  (if (== OtherActor (`GameplayStatics.GetPlayerCharacter` 0))
    (`KismetSystemLibrary.PrintString` "pick me up")))

(fn `LaunchBall`
  (bind _sphere (`self.Sphere`))
  ;[1 1 1] Launch ball when player throws
  (`PrimitiveComponent.AddImpulse` _sphere (* (`SceneComponent.K2_GetComponentLocation` _sphere) 25.0) "None" false))

(fn `Move`
  (bind (_returnvalue_x _returnvalue_y) (`KismetMathLibrary.BreakVector` (* (`KismetMathLibrary.GetDirectionUnitVector` (`self.K2_GetActorLocation`) (`.Location` (`GameplayStatics.BreakHitResult` (`PlayerController.GetHitResultUnderCursorByChannel` (`GameplayStatics.GetPlayerController` 0) "TraceTypeQuery1" true)))) 700.0)))
  ;[1 1 1] add force on direction of cursor
  (`PrimitiveComponent.AddForce` (`self.Sphere`) (`KismetMathLibrary.MakeVector` _returnvalue_x _returnvalue_y) "None" true))

(fn `UserConstructionScript`)