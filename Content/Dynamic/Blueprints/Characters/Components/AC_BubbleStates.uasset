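; Actor component that applies the effects of a bubble state to a bubble character.
; StateUpdate finds the DT_BubbleStates row whose name matches the state enum, then applies its multipliers to speed, gravity, lifespan and max distance.
; Lifespan scales from a hardcoded base, while the others multiply current values, so repeated calls compound.
; BeginPlay is empty, and a duplicate lookup in the EventGraph is unwired.
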(event `self.ReceiveBeginPlay`)

(fn `StateUpdate`
  (params (BubbleCharRef :type "/Game/Dynamic/Blueprints/Characters/BubbleChar/BP_BubbleChar Object Reference") (BubbleStateIn :type "/Game/Dynamic/DataTables/Enum_BubbleStates Enum" :default "NewEnumerator0"))
  (bind _ac_bubblecontrols (`/Game/Dynamic/Blueprints/Characters/BubbleChar/BP_BubbleChar.AC_BubbleControls` (`self.BubbleCharRef`)))
  (bind _ac_bubblecontrols_2 (`/Game/Dynamic/Blueprints/Characters/BubbleChar/BP_BubbleChar.AC_BubbleControls` (`self.BubbleCharRef`)))
  (set `self.BubbleCharRef` BubbleCharRef)
  (bind _output_get (set `self.DataTable` "/Game/Dynamic/DataTables/DT_BubbleStates.DT_BubbleStates"))
  (bind _outrownames (`DataTableFunctionLibrary.GetDataTableRowNames` _output_get))
  (for _array_element _outrownames
    (if (== _array_element (`|GetEnumeratorNameAsString` BubbleStateIn))
      (bind _returnvalue (`|GetDataTableRow` "/Game/Dynamic/DataTables/DT_BubbleStates.DT_BubbleStates" _array_element)
        (:`then`
          (bind _output_get_2 (set `self.StateRow` _returnvalue))
          (break)))))
  (bind (_bubblestate _speedmultiplier _gravitymultiplier _lifespanmultiplier _maxdistancemultiplier) (break `/Game/Dynamic/DataTables/S_BubbleStates` _output_get_2))
  (set `/Game/Dynamic/Blueprints/Actor_Components/AC_BubbleControls.Bubble Speed` (* (`/Game/Dynamic/Blueprints/Actor_Components/AC_BubbleControls.Bubble Speed` _ac_bubblecontrols_2) _speedmultiplier) _ac_bubblecontrols_2)
  (set `/Game/Dynamic/Blueprints/Characters/BubbleChar/BP_BubbleChar.GravityForce` (* (`/Game/Dynamic/Blueprints/Characters/BubbleChar/BP_BubbleChar.GravityForce` (`self.BubbleCharRef`)) _gravitymultiplier) (`self.BubbleCharRef`))
  (set `/Game/Dynamic/Blueprints/Actor_Components/AC_BubbleStats.Lifespan` (* 10.0 _lifespanmultiplier) (`/Game/Dynamic/Blueprints/Characters/BubbleChar/BP_BubbleChar.AC_BubbleStats` (`self.BubbleCharRef`)))
  (set `/Game/Dynamic/Blueprints/Actor_Components/AC_BubbleControls.Max Distance` (* (`/Game/Dynamic/Blueprints/Actor_Components/AC_BubbleControls.Max Distance` _ac_bubblecontrols) _maxdistancemultiplier) _ac_bubblecontrols))