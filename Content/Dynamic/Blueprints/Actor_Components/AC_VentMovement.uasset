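; Actor component that moves its owner along an assigned spline, apparently for travel through vents.
; Starting movement picks forward or reverse by comparing the owner's distance to both spline ends, entering from the nearer one.
; Once a delay timer has elapsed, Tick advances a clamped spline distance at Speed and sets the owner's location without sweeping.
; Reaching either end stops movement and restarts the timer, gating the next trip.
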(event `self.ReceiveTick`
  (params (DeltaSeconds :type "Float (single-precision)"))
  (bind _distancealongspline (`self.DistanceAlongSpline`))
  (if (>= (`self.CurrentVentTimer`) (`self.InitVentTimer`))
    (if (and (`KismetSystemLibrary.IsValid` (`self.SplineComponent`)) (`self.bIsMovingAlongSpline`))
      (if (`self.bIsReverseDirection`)
        (set `self.DistanceAlongSpline` (- (`self.DistanceAlongSpline`) (* (`self.Speed`) DeltaSeconds)))
        (else
          (set `self.DistanceAlongSpline` (+ (`self.DistanceAlongSpline`) (* (`self.Speed`) DeltaSeconds)))))
      (set `self.DistanceAlongSpline` (`KismetMathLibrary.FClamp` (`self.DistanceAlongSpline`) 0.0 (`SplineComponent.GetSplineLength` (`self.SplineComponent`))))
      (`Actor.K2_SetActorLocation` (`self.GetOwner`) (`SplineComponent.GetLocationAtDistanceAlongSpline` (`self.SplineComponent`) (`self.DistanceAlongSpline`) "World") false false)
      (if (or (<= _distancealongspline 0.0) (>= _distancealongspline (`SplineComponent.GetSplineLength` (`self.SplineComponent`))))
        (`self.StopSplineMovement`)))
    (else
      (set `self.CurrentVentTimer` (+ (`self.CurrentVentTimer`) DeltaSeconds)))))

(fn `SetDirection`
  (bind _splinecomponent (`self.SplineComponent`))
  (if (`KismetSystemLibrary.IsValid` (`self.SplineComponent`))
    (bind _output_get (set `self.bIsReverseDirection` (> (`KismetMathLibrary.Vector_Distance` (`Actor.K2_GetActorLocation` (`self.GetOwner`)) (`SplineComponent.GetLocationAtSplinePoint` (`self.SplineComponent`) 0 "World")) (`KismetMathLibrary.Vector_Distance` (`Actor.K2_GetActorLocation` (`self.GetOwner`)) (`SplineComponent.GetLocationAtSplinePoint` _splinecomponent (`SplineComponent.GetNumberOfSplinePoints` _splinecomponent) "World")))))
    (if _output_get
      (set `self.DistanceAlongSpline` (`SplineComponent.GetSplineLength` (`self.SplineComponent`))))
    (return)))

(fn `StartSplineMovement`
  (set `self.DistanceAlongSpline` 0.0)
  (`self.SetDirection`)
  (set `self.bIsMovingAlongSpline` true))

(fn `StopSplineMovement`
  (set `self.bIsMovingAlongSpline` false)
  (set `self.DistanceAlongSpline` 0.0)
  (set `self.CurrentVentTimer` 0.0))