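; Actor component that switches the player bubble's elemental state, such as Sap, Fire, Water or Ice, and applies that state's modifiers.
; Tick compares the state enum to the cached DT_BubbleStates row, loading the matching row on a mismatch.
; StateUpdate multiplies current speed, gravity and max distance, so changes compound across switches, while lifespan scales from a fixed base.
; An unused row-name lookup remains, marked as a failed test.
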(event `self.ReceiveBeginPlay`
  (set `self.DataTable` "/Game/Dynamic/DataTables/DT_BubbleStates.DT_BubbleStates")
  (bind _asbp_bubble_char (cast `/Game/Dynamic/Blueprints/Characters/BubbleChar/BP_BubbleChar` (`self.GetOwner`)))
  (set `self.BubbleCharRef` _asbp_bubble_char)
  (`self.RowSelect` "Default"))

(event `self.ReceiveTick`
  (params (DeltaSeconds :type "Float (single-precision)"))
  (bind _staterow_bubblestate (break `/Game/Dynamic/DataTables/S_BubbleStates` (`self.StateRow`)))
  (if (not (== _staterow_bubblestate (`KismetMathLibrary.Conv_ByteToInt` (`self.BubbleStates`))))
    (switch `EBubbleStates` (`self.BubbleStates`)
      (:`Default`
        (`self.RowSelect` "Default"))
      (:`Sap`
        (`self.RowSelect` "Sap"))
      (:`Fire`
        (`self.RowSelect` "Fire"))
      (:`Oil`
        (`self.RowSelect` "Oil"))
      (:`Flammable`
        (`self.RowSelect` "Flammable"))
      (:`Water`
        (`self.RowSelect` "Water"))
      (:`Ice`
        (`self.RowSelect` "Ice")))
    (`self.StateUpdate`)))

(fn `RowSelect`
  (params (RowName :type Name))
  (bind _returnvalue (`|GetDataTableRow` (`self.DataTable`) RowName)
    (:`then`
      (set `self.StateRow` _returnvalue)
      (return))))

(fn `StateUpdate`
  (bind (_bubblestate _speedmultiplier _gravitymultiplier _lifespanmultiplier _maxdistancemultiplier) (break `/Game/Dynamic/DataTables/S_BubbleStates` (`self.StateRow`)))
  (bind _ac_bubblecontrols (`/Game/Dynamic/Blueprints/Characters/BubbleChar/BP_BubbleChar.AC_BubbleControls` (`self.BubbleCharRef`)))
  (bind _ac_bubblecontrols_2 (`/Game/Dynamic/Blueprints/Characters/BubbleChar/BP_BubbleChar.AC_BubbleControls` (`self.BubbleCharRef`)))
  (set `/Game/Dynamic/Blueprints/Actor_Components/AC_BubbleControls.Bubble Speed` (* (`/Game/Dynamic/Blueprints/Actor_Components/AC_BubbleControls.Bubble Speed` _ac_bubblecontrols_2) _speedmultiplier) _ac_bubblecontrols_2)
  (set `/Game/Dynamic/Blueprints/Characters/BubbleChar/BP_BubbleChar.GravityForce` (* (`/Game/Dynamic/Blueprints/Characters/BubbleChar/BP_BubbleChar.GravityForce` (`self.BubbleCharRef`)) _gravitymultiplier) (`self.BubbleCharRef`))
  (set `/Game/Dynamic/Blueprints/Actor_Components/AC_BubbleStats.Lifespan` (* 10.0 _lifespanmultiplier) (`/Game/Dynamic/Blueprints/Characters/BubbleChar/BP_BubbleChar.AC_BubbleStats` (`self.BubbleCharRef`)))
  (set `/Game/Dynamic/Blueprints/Actor_Components/AC_BubbleControls.Max Distance` (* (`/Game/Dynamic/Blueprints/Actor_Components/AC_BubbleControls.Max Distance` _ac_bubblecontrols) _maxdistancemultiplier) _ac_bubblecontrols))