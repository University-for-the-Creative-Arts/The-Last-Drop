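; AC_BubbleStats is an actor component that tracks a bubble's lifespan and computes a skin value meant to drive its material effect.
; LifeTimerCount subtracts delta seconds from Lifespan and returns the remaining time.
; BubbleSkin adds elapsed lifetime scaled by LifeTimeBuffer, counted twice, to the gap between MaxDistance and CurrentDistance weighted by a negative constant.
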(fn `Bubble Skin`
  (returns (Value :type "Float (double-precision)"))
  (bind _returnvalue (* (* (- (`self.Lifespan`) (`self.Life time Init Value`)) -1.0) (`self.LifeTime Buffer`)))
  (return (+ _returnvalue (+ _returnvalue (* (- (`self.Max Distance`) (`self.Current Distance`)) -1.5)))))

(fn `LifeTimerCount`
  (params (`Delta Seconds` :type "Float (double-precision)"))
  (returns (LifeTimer :type "Float (double-precision)"))
  (bind _output_get (set `self.Lifespan` (- (`self.Lifespan`) `Delta Seconds`)))
  (return _output_get))