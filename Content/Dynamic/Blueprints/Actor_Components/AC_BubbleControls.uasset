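; Actor component for the player-steered bubble character, handling movement, jumping, water-driven size changes and popping.
; BubbleMovement pushes the capsule toward the cursor hit point, with Ice limited to the Y axis under heavier gravity.
; Sphere overlaps with BPI_BubbleInteract actors flag water, so Tick grows or shrinks the bubble, and exiting sets lifespan by size.
; Pop skips Ice, otherwise notifies nearby BPI_PopInteract actors, spawns Sap or Water drops and destroys the bubble.
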(event `self.ReceiveBeginPlay`
  (bind _asbp_bubble_char (cast `/Game/Dynamic/Blueprints/Characters/BubbleChar/BP_BubbleChar` (`self.GetOwner`)))
  (bind _output_get (set `self.As BP Bubble Char` _asbp_bubble_char))
  (set `self.Sphere2` (`/Game/Dynamic/Blueprints/Characters/BubbleChar/BP_BubbleChar.Sphere2` _output_get))
  (`SceneComponent.SetRelativeScale3D` (`self.Sphere2`) (1.0 1.0 1.0))
  (`SceneComponent.SetRelativeScale3D` (`/Game/Dynamic/Blueprints/Characters/BubbleChar/BP_BubbleChar.Sphere1` (`self.As BP Bubble Char`)) (1.0 1.0 1.0)))

(event `self.Sphere2.OnComponentBeginOverlap`
  (params (OverlappedComponent :type "PrimitiveComponent Object Reference") (OtherActor :type "Actor Object Reference") (OtherComp :type "PrimitiveComponent Object Reference") (OtherBodyIndex :type Integer) (bFromSweep :type Boolean) (SweepResult :type "HitResult Structure (by ref)"))
  (if (`KismetSystemLibrary.DoesImplementInterface` OtherActor "/Game/Dynamic/Blueprints/Interfaces/BPI_BubbleInteract.BPI_BubbleInteract_C")
    (set `self.IsInWater` true)))

(event `self.Sphere2.OnComponentEndOverlap`
  (params (OverlappedComponent :type "PrimitiveComponent Object Reference") (OtherActor :type "Actor Object Reference") (OtherComp :type "PrimitiveComponent Object Reference") (OtherBodyIndex :type Integer))
  (if (`KismetSystemLibrary.DoesImplementInterface` OtherActor "/Game/Dynamic/Blueprints/Interfaces/BPI_BubbleInteract.BPI_BubbleInteract_C")
    (set `self.IsInWater` false)
    (if (> (`self.CurrentSize`) (`self.MinSize`))
      (set `/Game/Dynamic/Blueprints/Actor_Components/AC_BubbleStats.Lifespan` (`self.WaterBubbleLifespan`) (`/Game/Dynamic/Blueprints/Characters/BubbleChar/BP_BubbleChar.AC_BubbleStats` (`self.As BP Bubble Char`)))
      (else
        (set `/Game/Dynamic/Blueprints/Actor_Components/AC_BubbleStats.Lifespan` (`self.BubbleLifespan`) (`/Game/Dynamic/Blueprints/Characters/BubbleChar/BP_BubbleChar.AC_BubbleStats` (`self.As BP Bubble Char`)))))))

(event `self.ReceiveTick`
  (params (DeltaSeconds :type "Float (single-precision)"))
  (`self.Growth Shrink` DeltaSeconds))

(fn `Bubble Movement`
  (params (`Capsule Component` :type "CapsuleComponent Object Reference") (`Bubble Char` :type "/Game/Dynamic/Blueprints/Characters/BubbleChar/BP_BubbleChar Object Reference"))
  (locals (NewLocalVar :type "BodyInstanceAsyncPhysicsTickHandle Structure"))
  (bind _ac_bubblestats (`/Game/Dynamic/Blueprints/Characters/BubbleChar/BP_BubbleChar.AC_BubbleStats` `Bubble Char`))
  (bind _returnvalue (* (`KismetMathLibrary.GetDirectionUnitVector` (`Actor.K2_GetActorLocation` (`self.GetOwner`)) (`.Location` (`GameplayStatics.BreakHitResult` (`PlayerController.GetHitResultUnderCursorByChannel` (`GameplayStatics.GetPlayerController` 0) "TraceTypeQuery1" true)))) (`self.Bubble Speed`)))
  (bind (_returnvalue_x _returnvalue_y) (`KismetMathLibrary.BreakVector` (* _returnvalue 1.5)))
  (`/Engine/EditorBlueprintResources/StandardMacros.IsValid` `Bubble Char`
    (:`Is Valid`
      (if (`|EnumEquality` (`SurfaceStateComponent.BubbleStates` (`/Game/Dynamic/Blueprints/Characters/BubbleChar/BP_BubbleChar.AC_BubbleStates` `Bubble Char`)) "Ice")
        (set `/Game/Dynamic/Blueprints/Characters/BubbleChar/BP_BubbleChar.GravityForce` -750.0 `Bubble Char`)
        (`PrimitiveComponent.AddForce` `Capsule Component` (`KismetMathLibrary.MakeVector` 0.0 _returnvalue_y) "None" true)
        (set `/Game/Dynamic/Blueprints/Actor_Components/AC_BubbleStats.Lifespan` 1.0 _ac_bubblestats)
        (set `/Game/Dynamic/Blueprints/Actor_Components/AC_BubbleStats.Max Distance` 99999999.0 _ac_bubblestats)
        (else
          (`PrimitiveComponent.AddForce` `Capsule Component` _returnvalue "None" true)
          (set `/Game/Dynamic/Blueprints/Characters/BubbleChar/BP_BubbleChar.GravityForce` -100.0 `Bubble Char`)
          (set `/Game/Dynamic/Blueprints/Actor_Components/AC_BubbleStats.Max Distance` 1000.0 (`/Game/Dynamic/Blueprints/Characters/BubbleChar/BP_BubbleChar.AC_BubbleStats` `Bubble Char`)))))))

(fn `BubbleJump`
  (params (CapsuleComponent :type "CapsuleComponent Object Reference"))
  (`PrimitiveComponent.AddImpulse` CapsuleComponent (`KismetMathLibrary.MakeVector` 0.0 0.0 (`self.JumpForce`)) "None" true))

(fn `Calculate distance`
  (params (`Actor ` :type "Actor Object Reference") (BodyChar :type "/Game/Dynamic/Blueprints/Characters/BodyChar/BP_BodyChar Object Reference"))
  (returns (`Auto Pop Distance` :type Boolean))
  (bind _returnvalue (`Actor.GetComponentByClass` `Actor ` "/Game/Dynamic/Blueprints/Actor_Components/AC_BubbleStats.AC_BubbleStats_C"))
  (bind _output_get (set `/Game/Dynamic/Blueprints/Actor_Components/AC_BubbleStats.Current Distance` (`KismetMathLibrary.Vector_Distance` (`Actor.K2_GetActorLocation` BodyChar) (`Actor.K2_GetActorLocation` `Actor `)) _returnvalue))
  (return (< (`/Game/Dynamic/Blueprints/Actor_Components/AC_BubbleStats.Max Distance` _returnvalue) _output_get)))

(fn `Growth`
  (params (WaterGainAmount :type "Float (double-precision)"))
  (set `self.CurrentSize` (+ WaterGainAmount (`self.CurrentSize`)))
  (if (>= (`self.CurrentSize`) (`self.MaxSize`))
    (set `self.CurrentSize` (`self.MaxSize`))))

(fn `Growth Shrink`
  (params (DeltaSeconds :type "Float (double-precision)"))
  (bind _delta_seconds (`self.Delta Seconds`))
  (bind _water_gain_amount (`self.Water Gain Amount`))
  (bind _currentsize (`self.CurrentSize`))
  (bind _water_loss_amount (`self.Water Loss Amount`))
  (bind _currentsize_2 (`self.CurrentSize`))
  (bind _delta_seconds_2 (`self.Delta Seconds`))
  (bind _returnvalue (`SceneComponent.GetRelativeTransform` (`/Game/Dynamic/Blueprints/Characters/BubbleChar/BP_BubbleChar.Sphere2` (`self.As BP Bubble Char`))))
  (bind _returnvalue_2 (`SceneComponent.GetRelativeTransform` (`/Game/Dynamic/Blueprints/Characters/BubbleChar/BP_BubbleChar.Sphere2` (`self.As BP Bubble Char`))))
  (bind _returnvalue_3 (`KismetMathLibrary.FInterpTo` (.z (.scale _returnvalue)) _currentsize _delta_seconds _water_gain_amount))
  (bind _returnvalue_4 (`KismetMathLibrary.FInterpTo` (.x (.scale _returnvalue)) _currentsize _delta_seconds _water_gain_amount))
  (bind _returnvalue_5 (`KismetMathLibrary.FInterpTo` (.y (.scale _returnvalue)) _currentsize _delta_seconds _water_gain_amount))
  (bind _returnvalue_6 (`KismetMathLibrary.FInterpTo` (.z (.scale _returnvalue_2)) _currentsize_2 _delta_seconds_2 _water_loss_amount))
  (bind _returnvalue_7 (`KismetMathLibrary.FInterpTo` (.x (.scale _returnvalue_2)) _currentsize_2 _delta_seconds_2 _water_loss_amount))
  (bind _returnvalue_8 (`KismetMathLibrary.FInterpTo` (.y (.scale _returnvalue_2)) _currentsize_2 _delta_seconds_2 _water_loss_amount))
  (set `self.Delta Seconds` DeltaSeconds)
  (if (`self.IsInWater`)
    (`self.Growth` (`self.Water Gain Amount`))
    (`SceneComponent.SetRelativeScale3D` (`/Game/Dynamic/Blueprints/Characters/BubbleChar/BP_BubbleChar.Sphere2` (`self.As BP Bubble Char`)) (`KismetMathLibrary.MakeVector` _returnvalue_4 _returnvalue_5 _returnvalue_3))
    (`SceneComponent.SetRelativeScale3D` (`/Game/Dynamic/Blueprints/Characters/BubbleChar/BP_BubbleChar.Sphere` (`self.As BP Bubble Char`)) (`KismetMathLibrary.MakeVector` _returnvalue_4 _returnvalue_5 _returnvalue_3))
    (else
      (`self.Shrink` (`self.Water Loss Amount`))
      (`SceneComponent.SetRelativeScale3D` (`/Game/Dynamic/Blueprints/Characters/BubbleChar/BP_BubbleChar.Sphere2` (`self.As BP Bubble Char`)) (`KismetMathLibrary.MakeVector` _returnvalue_7 _returnvalue_8 _returnvalue_6))
      (`SceneComponent.SetRelativeScale3D` (`/Game/Dynamic/Blueprints/Characters/BubbleChar/BP_BubbleChar.Sphere` (`self.As BP Bubble Char`)) (`KismetMathLibrary.MakeVector` _returnvalue_7 _returnvalue_8 _returnvalue_6)))))

(fn `Pop`
  (params (BubbleChar :type "/Game/Dynamic/Blueprints/Characters/BubbleChar/BP_BubbleChar Object Reference"))
  (locals (BubbleCharRef :type "/Game/Dynamic/Blueprints/Characters/BubbleChar/BP_BubbleChar Object Reference"))
  (bind _bp_bodychar (`/Game/Dynamic/Blueprints/Characters/BubbleChar/BP_BubbleChar.BP_BodyChar` (`local.BubbleCharRef`)))
  (bind _sphere1 (`/Game/Dynamic/Blueprints/Characters/BubbleChar/BP_BubbleChar.Sphere1` (`local.BubbleCharRef`)))
  (set `local.BubbleCharRef` BubbleChar)
  (if (`|EnumEquality` (`SurfaceStateComponent.BubbleStates` (`/Game/Dynamic/Blueprints/Characters/BubbleChar/BP_BubbleChar.AC_BubbleStates` (`local.BubbleCharRef`))) "Ice")
    (`KismetSystemLibrary.PrintString` "ice ball doesnt pop")
    (else
      (`self.IA_Pop`)
      (`/Game/Dynamic/Blueprints/Characters/BodyChar/AC_BubbleController.Pop Reset` (`/Game/Dynamic/Blueprints/Characters/BodyChar/BP_BodyChar.AC_BubbleController` _bp_bodychar) (`/Game/Dynamic/Blueprints/Characters/BodyChar/BP_BodyChar.Sphere` _bp_bodychar))
      (`NiagaraFunctionLibrary.SpawnSystemAtLocation` "/Game/Dynamic/Niagara/NS_Pop.NS_Pop" (`Actor.K2_GetActorLocation` (`local.BubbleCharRef`)))
      (`/Game/Dynamic/Blueprints/Actor_Components/AC_CamBehaviour.RemoveTrackingActor` (`/Game/Dynamic/Blueprints/Characters/BodyChar/BP_BodyChar.AC_CamBehaviour` (`/Game/Dynamic/Blueprints/Characters/BubbleChar/BP_BubbleChar.BP_BodyChar` (`local.BubbleCharRef`))) (`local.BubbleCharRef`))
      (`self.PopTrace`)
      (switch `EBubbleStates` (`SurfaceStateComponent.BubbleStates` (`/Game/Dynamic/Blueprints/Characters/BubbleChar/BP_BubbleChar.AC_BubbleStates` (`local.BubbleCharRef`)))
        (:`Default`
          (`GameplayStatics.PlaySound2D` "/Game/Dynamic/Audio/Events/MS_Pop.MS_Pop" 1.0 1.0 0.0 null null)
          (`Actor.K2_DestroyActor` (`local.BubbleCharRef`))
          (set `PlayerController.bShowMouseCursor` false (`GameplayStatics.GetPlayerController` 0)))
        (:`Sap`
          (bind _returnvalue (`|SpawnActorFromClass` "/Game/Dynamic/Blueprints/BP_SapLiquidSphere.BP_SapLiquidSphere_C" (`Actor.GetTransform` (`local.BubbleCharRef`)) "AdjustIfPossibleButAlwaysSpawn" "MultiplyWithRoot" null null))
          (`GameplayStatics.PlaySound2D` "/Game/Dynamic/Audio/Events/MS_Pop.MS_Pop" 1.0 1.0 0.0 null _returnvalue)
          (`Actor.K2_DestroyActor` (`local.BubbleCharRef`))
          (set `PlayerController.bShowMouseCursor` false (`GameplayStatics.GetPlayerController` 0)))
        (:`Water`
          (bind _returnvalue_2 (`|SpawnActorFromClass` "/Game/Dynamic/Blueprints/Environment/Drops/BP_WaterDrop.BP_WaterDrop_C" (`Actor.GetTransform` (`local.BubbleCharRef`)) "AdjustIfPossibleButAlwaysSpawn" "MultiplyWithRoot" null 1.0 null))
          (`GameplayStatics.PlaySound2D` "/Game/Dynamic/Audio/Events/MS_Pop.MS_Pop" 1.0 1.0 0.0 null _returnvalue_2)
          (`Actor.K2_DestroyActor` (`local.BubbleCharRef`))
          (set `PlayerController.bShowMouseCursor` false (`GameplayStatics.GetPlayerController` 0)))
        (:`Ice`
          (`self.Bubble Movement` (`Character.CapsuleComponent` (`local.BubbleCharRef`)))
          (`PrimitiveComponent.SetSimulatePhysics` _sphere1 true)
          (`PrimitiveComponent.SetConstraintMode` _sphere1 "XZPlane")
          (`GameplayStatics.PlaySound2D` "/Game/Dynamic/Audio/Events/MS_Pop.MS_Pop" 1.0 1.0 0.0 null null)
          (`Actor.K2_DestroyActor` (`local.BubbleCharRef`))
          (set `PlayerController.bShowMouseCursor` false (`GameplayStatics.GetPlayerController` 0)))))))

(fn `PopTrace`
  (bind _returnvalue (`Actor.K2_GetActorLocation` (`self.GetOwner`)))
  (bind _outhits (`KismetSystemLibrary.SphereTraceMulti` _returnvalue _returnvalue 150.0 "TraceTypeQuery1"))
  (for _array_element _outhits
    (if (`KismetSystemLibrary.DoesImplementInterface` (`.HitActor` (`GameplayStatics.BreakHitResult` _array_element)) "/Game/Dynamic/Blueprints/Interfaces/BPI_PopInteract.BPI_PopInteract_C")
      (message `/Game/Dynamic/Blueprints/Interfaces/BPI_PopInteract.BPI_PopInteract` (`.HitActor` (`GameplayStatics.BreakHitResult` _array_element))))))

(fn `Shrink`
  (params (WaterLossAmount :type "Float (double-precision)"))
  (if (<= (`self.CurrentSize`) (`self.MaxSize`))
    (set `self.CurrentSize` (- (`self.CurrentSize`) WaterLossAmount))
    (if (<= (`self.CurrentSize`) (`self.MinSize`))
      (set `self.CurrentSize` (`self.MinSize`)))))