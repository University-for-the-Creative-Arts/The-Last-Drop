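; Actor component that lets a bubble pick up and carry its owner's mesh, with support for resetting that object.
; Pickup claims an unattached bubble, scales its sphere to the object, snaps the mesh onto its capsule and plays a sound.
; A bound pop event triggers Drop, which restores physics and collision if flagged.
; ResetLocation drops the object, pops the bubble and restores the location and rotation cached by GetSelfTransform.
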(event `ResetLocation`
  (bind _sm_ref (`self.SM Ref`))
  (bind _bubble_ref (`self.Bubble Ref`))
  (`KismetSystemLibrary.PrintString` "AC_BubblePickup:: RESETTING!")
  (`self.Drop`)
  (`/Engine/EditorBlueprintResources/StandardMacros.IsValid` _bubble_ref
    (:`Is Valid`
      (`/Game/Dynamic/Blueprints/Actor_Components/AC_BubbleControls.Pop` (`/Game/Dynamic/Blueprints/Characters/BubbleChar/BP_BubbleChar.AC_BubbleControls` _bubble_ref) _bubble_ref))
    (:`Is Not Valid`
      _))
  (`SceneComponent.K2_SetWorldTransform` _sm_ref (`KismetMathLibrary.MakeTransform` (`self.InitLocation`) (`self.InitRotation`) (`SceneComponent.K2_GetComponentScale` _sm_ref)) false false))

(event `self.ReceiveBeginPlay`)

(event `GetSelfTransform`
  (bind _selfactor (`self.SelfActor`))
  (set `self.InitLocation` (`Actor.K2_GetActorLocation` _selfactor))
  (set `self.InitRotation` (`Actor.K2_GetActorRotation` _selfactor)))

(event `Pickup`
  (params (BubbleRef :type "/Game/Dynamic/Blueprints/Characters/BubbleChar/BP_BubbleChar Object Reference") (`SM ref` :type "StaticMeshComponent Object Reference") (ShouldSimulatePhysics :type Boolean) (BubbleFalloff :type "Float (double-precision)"))
  (if (not (`/Game/Dynamic/Blueprints/Characters/BubbleChar/BP_BubbleChar.HasAttached?` BubbleRef))
    (set `/Game/Dynamic/Blueprints/Characters/BubbleChar/BP_BubbleChar.HasAttached?` true BubbleRef)
    (`SceneComponent.SetRelativeScale3D` (`/Game/Dynamic/Blueprints/Characters/BubbleChar/BP_BubbleChar.Sphere` BubbleRef) (* (`Actor.GetActorScale3D` (`self.GetOwner` `SM ref`)) 1.4))
    (set `self.Should Simulate Physics` ShouldSimulatePhysics)
    (set `self.Bubble Ref` BubbleRef)
    (set `self.SM Ref` `SM ref`)
    (add `/Game/Dynamic/Blueprints/Characters/BubbleChar/BP_BubbleChar.IA_Pop` (`self.Bubble Ref`) (delegate `Drop`))
    (`SceneComponent.K2_AttachToComponent` (`self.SM Ref`) (`Character.CapsuleComponent` (`self.Bubble Ref`)) "None" "SnapToTarget" "SnapToTarget" "KeepRelative" true)
    (`GameplayStatics.PlaySound2D` "/Game/Dynamic/Audio/Events/MS_Pickup.MS_Pickup" 1.0 1.0 0.0 null null)))

(event `Drop`
  (bind _sm_ref (`self.SM Ref`))
  (if (`self.Should Simulate Physics`)
    (`PrimitiveComponent.SetSimulatePhysics` _sm_ref true)
    (`PrimitiveComponent.SetCollisionEnabled` _sm_ref "QueryAndPhysics")))