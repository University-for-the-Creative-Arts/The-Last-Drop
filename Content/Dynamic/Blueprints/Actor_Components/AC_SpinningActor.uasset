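; Actor component for spinning its owning actor by offsetting the actor's rotation whenever the StartSpinning event is called.
; StartSpinning passes its Time input and the Axis rotator to Calculation, then combines the result with the owner's current rotation.
; Calculation holds per-axis multiplications by time and TimeToRotate, but they are shown unconnected to its outputs.
; StartSpin is an empty stub, and BeginPlay only reassigns RelativeRotation to itself.
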(event `self.ReceiveBeginPlay`
  (set `self.RelativeRotation` (`self.RelativeRotation`)))

(event `StartSpinning`
  (params (Time :type "Float (double-precision)") (Axis :type "Rotator Structure"))
  (bind _returnvalue (`self.GetOwner`))
  (`Actor.K2_SetActorRotation` _returnvalue (`KismetMathLibrary.ComposeRotators` (`Actor.K2_GetActorRotation` _returnvalue) (`KismetMathLibrary.MakeRotator` (* (* Time Axis_Roll) (`self.TimeToRotate`)) (* (* Time Axis_Pitch) (`self.TimeToRotate`)) (* (* Axis_Yaw Time) (`self.TimeToRotate`)))) false))

(fn `StartSpin`)