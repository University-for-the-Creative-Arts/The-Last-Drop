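; Wind turbine that, once switched on, lifts BP_BodyChar characters entering its box with negative gravity and upward velocity.
; SwitchOnOff only turns it on, running a timeline that ramps blade yaw and starts a looping per-frame timer to keep spinning.
; "Heavy"-tagged characters toggle linked BPActivatable actors with a sound on entry while on, and on every exit.
; Exit also restores gravity, regardless of fan state.
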(event `SwitchOnOff`
  (if (not (`self.IsFanOn?`))
    (set `self.IsFanOn?` true)
    (bind (_direction _newtrack_0) (`Timeline|Fan`)
      (:`Update`
        (`SceneComponent.K2_AddRelativeRotation` (`self.StaticMesh`) (`KismetMathLibrary.MakeRotator` 0.0 0.0 (`KismetMathLibrary.Lerp` 0.0 15.0 _newtrack_0)) false false)
        (if (not (`self.IsFanOn?`))
          (`KismetSystemLibrary.K2_PauseTimerHandle` (stale _returnvalue))
          (else
            (bind _returnvalue (`KismetSystemLibrary.K2_SetTimerDelegate` (delegate `FanOn`) (`GameplayStatics.GetWorldDeltaSeconds`) true))))))))

(event `FanOn`
  (`SceneComponent.K2_AddRelativeRotation` (`self.StaticMesh`) (struct :`Yaw` 15.0) false false))

(event `self.Box.OnComponentBeginOverlap`
  (params (OverlappedComponent :type "PrimitiveComponent Object Reference") (OtherActor :type "Actor Object Reference") (OtherComp :type "PrimitiveComponent Object Reference") (OtherBodyIndex :type Integer) (bFromSweep :type Boolean) (SweepResult :type "HitResult Structure (by ref)"))
  (if (`self.IsFanOn?`)
    (bind _asbp_body_char (cast `/Game/Dynamic/Blueprints/Characters/BodyChar/BP_BodyChar` OtherActor))
    (bind _charactermovement (`Character.CharacterMovement` _asbp_body_char))
    (set `CharacterMovementComponent.GravityScale` -1.0 _charactermovement)
    (set `MovementComponent.Velocity` (0.0 0.0 100.0) _charactermovement)
    (`CharacterMovementComponent.AddForce` _charactermovement (0.0 0.0 -100.0))
    (if (`self.ActorHasTag` OtherActor "Heavy")
      (`GameplayStatics.PlaySound2D` "/Game/Dynamic/Audio/Events/MS_InteractableActivate.MS_InteractableActivate" 1.0 1.0 0.0 null null)
      (`KismetSystemLibrary.PrintString` "Hello")
      (for _array_element (`self.BP Activatable`)
        (`/Game/Dynamic/Blueprints/Environment/Activatable/BP_ActivatableParent.Activate/Deactivate` _array_element)))))

(event `self.Box.OnComponentEndOverlap`
  (params (OverlappedComponent :type "PrimitiveComponent Object Reference") (OtherActor :type "Actor Object Reference") (OtherComp :type "PrimitiveComponent Object Reference") (OtherBodyIndex :type Integer))
  (bind _asbp_body_char (cast `/Game/Dynamic/Blueprints/Characters/BodyChar/BP_BodyChar` OtherActor))
  (set `CharacterMovementComponent.GravityScale` 1.75 (`Character.CharacterMovement` _asbp_body_char))
  (if (`self.ActorHasTag` OtherActor "Heavy")
    (`GameplayStatics.PlaySound2D` "/Game/Dynamic/Audio/Events/MS_InteractableActivate.MS_InteractableActivate" 1.0 1.0 0.0 null null)
    (for _array_element (`self.BP Activatable`)
      (`/Game/Dynamic/Blueprints/Environment/Activatable/BP_ActivatableParent.Activate/Deactivate` _array_element))))

(fn `UserConstructionScript`)