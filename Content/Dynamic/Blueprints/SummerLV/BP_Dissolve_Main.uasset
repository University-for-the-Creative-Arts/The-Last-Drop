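; Dissolve effect actor that fades a skeletal mesh and a static mesh, each paired with a Niagara system.
; Setup functions share Alpha, edge colour and dissolve texture between materials and particles, boosting colour for materials and creating dynamic instances for the texture.
; The construction script applies both setups.
; UpdateDataSK and UpdateDataStatic rerun their setup, then play a timeline from an Alpha-scaled time to animate Alpha on both mesh and particles.
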(event `UpdateDataSK`
  (bind _skeletalmesh (`self.SkeletalMesh`))
  (bind _sk_niagara (`self.SK_Niagara`))
  (`self.SKMesh_Setup` _sk_niagara _skeletalmesh)
  (`|ExecutionSequence`
    (:`then_0`
      (bind (_direction _newtrack_0) (`Timeline|Timeline` :`NewTime` (* (`self.Alpha`) 5.0) :!via `SetNewTime` :!label _label)
        (:`Update`
          (`MeshComponent.SetScalarParameterValueOnMaterials` _skeletalmesh "Alpha" _newtrack_0)
          (`NiagaraComponent.SetVariableFloat` _sk_niagara "Alpha" _newtrack_0))))
    (:`then_1`
      (goto _label))))

(event `UpdateDataStatic`
  (bind _staticmesh (`self.StaticMesh`))
  (bind _niagara (`self.Niagara`))
  (`self.StaticMesh_Setup` _niagara _staticmesh)
  (`|ExecutionSequence`
    (:`then_0`
      (bind (_direction _newtrack_0) (`Timeline|Timeline_0` :`NewTime` (* (`self.Alpha`) 5.0) :!via `SetNewTime` :!label _label_2)
        (:`Update`
          (`MeshComponent.SetScalarParameterValueOnMaterials` _staticmesh "Alpha" _newtrack_0)
          (`NiagaraComponent.SetVariableFloat` _niagara "Alpha" _newtrack_0))))
    (:`then_1`
      (goto _label_2))))

(fn `UserConstructionScript`
  (`self.SKMesh_Setup` (`self.SK_Niagara`) (`self.SkeletalMesh`))
  (`self.StaticMesh_Setup` (`self.Niagara`) (`self.StaticMesh`)))