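; Heat room hazard that the player disables by standing on pressure plates until a Tick-driven progress counter reaches 100%.
; Entering the volume activates the first plate and starts a recursive one-second heat countdown, skipped while in water, that reloads the test level at zero.
; Reactivate picks a random plate other than the last pressed, then rebuilds the plate list by room tag.
; Completion stops Tick, plates and volume collision.
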(event `Complete`
  ;[0.5873 1 0.6459] Player completes the room
  (`self.SetActorTickEnabled` false)
  (for _array_element (`self.Plates`)
    (`/Game/Dynamic/Blueprints/SummerLV/BP_HeatPlate.Deactivate` _array_element))
  (set `self.PlayerInRoom?` false)
  (`PrimitiveComponent.SetCollisionEnabled` (`self.HeatRoomVolume`) "NoCollision"))

(event `self.ReceiveTick`
  (params (DeltaSeconds :type "Float (single-precision)"))
  ;[1 1 1] Tick that activates when stood on a pressure plate, increasing the progress to disabling the heat room
  (bind _output_get (set `self.RoomPercentage` (+ (`self.RoomPercentage`) 1)))
  (`KismetSystemLibrary.PrintText` (`|FormatText` "{Percent}%" _output_get) true true (struct :`R` 0.983729 :`G` 0.171702 :`B` 1.0 :`A` 1.0) 3.0 "2009")
  (if (== _output_get 100)
    (`self.Complete`)))

(event `self.HeatRoomVolume.OnComponentBeginOverlap`
  (params (OverlappedComponent :type "PrimitiveComponent Object Reference") (OtherActor :type "Actor Object Reference") (OtherComp :type "PrimitiveComponent Object Reference") (OtherBodyIndex :type Integer) (bFromSweep :type Boolean) (SweepResult :type "HitResult Structure (by ref)"))
  ;[1 0.6872 0.6507] Player enters the volume of the heat room
  (if (== OtherActor (`GameplayStatics.GetPlayerCharacter` 0))
    (`KismetSystemLibrary.PrintString` "EnteredHeat" true true (struct :`R` 1.0 :`B` 0.016844 :`A` 1.0) 2.0 "1991")
    (`/Game/Dynamic/Blueprints/SummerLV/BP_HeatPlate.Activate` (`|GetArrayItem` (`self.Plates`)))
    (set `self.RoomPercentage` 0)
    (set `self.PlayerInRoom?` true)
    (set `self.PlayerHeat` 15)
    (`KismetSystemLibrary.Delay` 1.0)
    (`self.HeatActive`)))

(event `self.HeatRoomVolume.OnComponentEndOverlap`
  (params (OverlappedComponent :type "PrimitiveComponent Object Reference") (OtherActor :type "Actor Object Reference") (OtherComp :type "PrimitiveComponent Object Reference") (OtherBodyIndex :type Integer))
  ;[0.529 0.8122 1] Player exits the volume of the heat room
  (if (== OtherActor (`GameplayStatics.GetPlayerCharacter` 0))
    (`KismetSystemLibrary.PrintString` "ExitedHeat" true true (struct :`G` 0.330809 :`B` 1.0 :`A` 1.0) 2.0 "1991")))

(event `self.ReceiveBeginPlay`
  ;[1 1 1] Begin by assigning all plates within the area a number, and give them all a tag unique to this area.
  (for (_array_element _array_index) (`self.Plates`)
    (set `/Game/Dynamic/Blueprints/SummerLV/BP_HeatPlate.PlateNum` _array_index _array_element)
    (set `Actor.Tags` (`|MakeArray` (`self.RoomTag`)) _array_element))
  (bind _returnvalue (`GameplayStatics.GetActorOfClass` "/Game/Dynamic/Blueprints/Characters/BodyChar/BP_BodyChar.BP_BodyChar_C"))
  (set `self.PlayerCharacter` _returnvalue)
  (`KismetSystemLibrary.PrintString` "FoundPlayer" true true (struct :`R` 0.325488 :`B` 1.0 :`A` 1.0) 1.0))

(event `Reactivate`
  (params (Exclude :type Integer))
  ;[1 1 1] Reactivating a random switch. Done by removing, then readding, the last pressed switch
  (`|ExecutionSequence`
    (:`then_0`
      (`KismetArrayLibrary.Array_Remove` (`self.Plates`) Exclude)
      (`/Game/Dynamic/Blueprints/SummerLV/BP_HeatPlate.Activate` (`KismetArrayLibrary.Array_Random` (`self.Plates`))))
    (:`then_1`
      (`KismetArrayLibrary.Array_Clear` (`self.Plates`))
      (bind _outactors (`GameplayStatics.GetAllActorsOfClassWithTag` "/Game/Dynamic/Blueprints/SummerLV/BP_HeatPlate.BP_HeatPlate_C" (`self.RoomTag`)))
      (bind _output_get (set `self.Plates` _outactors))
      (for (_array_element _array_index) _output_get
        (set `/Game/Dynamic/Blueprints/SummerLV/BP_HeatPlate.PlateNum` _array_index _array_element)
        (set `/Game/Dynamic/Blueprints/SummerLV/BP_HeatPlate.Room` self _array_element))
      (`KismetSystemLibrary.PrintText` (`|FormatText` "Reset: {Num}" (`KismetArrayLibrary.Array_Length` _output_get))))))

(event `HeatActive`
  ;[1 1 1] Increases and checks the player's current heat when they are within the heat room
  (if (`self.PlayerInRoom?`)
    (if (`self.PlayerInWater?`)
      (`self.HeatActive`)
      (else
        (bind _output_get (set `self.PlayerHeat` (- (`self.PlayerHeat`) 1)))
        (`KismetSystemLibrary.PrintText` (`|FormatText` "{Seconds} Seconds Left" _output_get) true true (struct :`R` 1.0 :`G` 0.994057 :`A` 1.0) 2.0 "238")
        (if (== _output_get 0)
          (message `/Game/Dynamic/SaveSystem/BPI_SaveGame.LoadGameData` (`self.PlayerCharacter`) false)
          (`GameplayStatics.OpenLevel` "LV_SummerTesting")
          (else
            (`KismetSystemLibrary.Delay` 1.0)
            (`self.HeatActive`)))))))

(fn `UserConstructionScript`)