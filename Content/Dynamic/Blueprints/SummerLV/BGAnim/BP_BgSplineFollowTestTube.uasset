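; Background animation actor, apparently a test tube, that travels along a BP_BgSplinePath spline in the level.
; On BeginPlay it finds the path actor with a matching SplineNum and starts moving.
; MoveTimeline starts at the PlaceAlongSpline offset, with its play rate scaled by the inverse of TimeToComplete.
; Each update maps the timeline track to spline distance and sets the actor's world location and rotation there.
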(event `self.ReceiveBeginPlay`
  (bind _outactors (`GameplayStatics.GetAllActorsOfClass` "/Game/Dynamic/Blueprints/SummerLV/BGAnim/BP_BgSplinePath.BP_BgSplinePath_C"))
  (for _array_element _outactors
    (if (== (`self.SplineNum`) (`/Game/Dynamic/Blueprints/SummerLV/BGAnim/BP_BgSplinePath.SplineNum` _array_element))
      (set `self.SplineRef` _array_element)
      (break)))
  (`self.MoveObject`))

(event `MoveObject`
  (bind _spline (`/Game/Dynamic/Blueprints/SummerLV/BGAnim/BP_BgSplinePath.Spline` (`self.SplineRef`)))
  (`TimelineComponent.SetPlayRate` (`self.MoveTimeline`) (/ 1.0 (`self.TimeToComplete`)))
  (`|ExecutionSequence`
    (:`then_0`
      (bind (_direction _movetrack) (`Timeline|MoveTimeline` :`NewTime` (`self.PlaceAlongSpline`) :!via `SetNewTime` :!label _label)
        (:`Update`
          (bind _returnvalue (`KismetMathLibrary.Lerp` 0.0 (`SplineComponent.GetSplineLength` (`/Game/Dynamic/Blueprints/SummerLV/BGAnim/BP_BgSplinePath.Spline` (`self.SplineRef`))) _movetrack))
          (`self.K2_SetActorTransform` (`KismetMathLibrary.MakeTransform` (`SplineComponent.GetLocationAtDistanceAlongSpline` _spline _returnvalue "World") (`SplineComponent.GetRotationAtDistanceAlongSpline` _spline _returnvalue "World"))))))
    (:`then_1`
      (goto _label))))

(fn `UserConstructionScript`)