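; Background animation actor that loops a mesh through a press, where it transforms into a skeletal-mesh robot.
; The static mesh eases to the press position, swaps to the skeletal mesh on SwapModel, then on Leave moves out, resets to its start and repeats.
; A Master instance gathers others sharing its GroupNum at BeginPlay, triggers the Press, and relays swap and leave calls to the group.
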(event `self.ReceiveBeginPlay`
  (set `self.StartRelativeLocation` (`SceneComponent.RelativeLocation` (`self.StaticMesh`)))
  (if (`self.Master?`)
    (`KismetArrayLibrary.Array_Clear` (`self.Group`))
    (bind _outactors (`GameplayStatics.GetAllActorsOfClass` "BP_BgRobotTransform_C"))
    (for _array_element _outactors
      (if (== (`/Game/Dynamic/Blueprints/SummerLV/BGAnim/BP_BgRobotTransform.GroupNum` _array_element) (`self.GroupNum`))
        (if (not (== _array_element self))
          (`KismetArrayLibrary.Array_Add` (`self.Group`) _array_element)))))
  (`self.Move`))

(event `SwapModel (Robot)`
  (`SceneComponent.SetVisibility` (`self.StaticMesh`) false false)
  (`SceneComponent.SetVisibility` (`self.SkeletalMesh`) true false)
  (if (`self.Master?`)
    (for _array_element (`self.Group`)
      (`self.SwapModel (Robot)` _array_element))))

(event `Move`
  (`KismetSystemLibrary.MoveComponentTo` (`self.StaticMesh`) (`self.Relative Location (Press)`) (struct) true true (`self.MoveTime`))
  (`KismetSystemLibrary.Delay` 1.0)
  (if (`self.Master?`)
    (`/Game/Dynamic/Blueprints/SummerLV/BGAnim/BP_BgRobotPress.PressDown` (`self.Press`) self)))

(event `Leave`
  (if (`self.Master?`)
    (for _array_element (`self.Group`)
      (`self.Leave` _array_element)))
  (`KismetSystemLibrary.MoveComponentTo` (`self.StaticMesh`) (`self.Relative Location (Leaving)`) (struct) true true (`self.MoveTime`))
  (`self.MoveBack`))

(event `MoveBack`
  (`SceneComponent.SetVisibility` (`self.StaticMesh`) true false)
  (`SceneComponent.SetVisibility` (`self.SkeletalMesh`) false false)
  (`SceneComponent.K2_SetRelativeLocation` (`self.StaticMesh`) (`self.StartRelativeLocation`) false true)
  (`KismetSystemLibrary.Delay` (`self.MoveTime`))
  (`self.Move`))

(fn `UserConstructionScript`)