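; Background robot press prop that stamps down on a robot, swaps its model, then retracts and releases it.
; PressDown receives the robot, then chains delays and component moves between the start and drop positions cached on BeginPlay.
; PressUp returns the press and tells the robot to leave.
; Tick, switched on by PressDown and off by PressUp, stretches the cylinder's Z scale to follow the press head.
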(event `self.ReceiveTick`
  (params (DeltaSeconds :type "Float (single-precision)"))
  (bind (_relativelocation_x _relativelocation_y _relativelocation_z) (`KismetMathLibrary.BreakVector` (`SceneComponent.RelativeLocation` (`self.Press`))))
  (`SceneComponent.SetRelativeScale3D` (`self.PressCylinder`) (`KismetMathLibrary.MakeVector` 0.25 0.25 (/ (`KismetMathLibrary.Abs` _relativelocation_z) 5.0))))

(event `self.ReceiveBeginPlay`
  ;[1 1 1] Begins by setting the starting and end location of the end of the press, and checks if Auto Activate is true in order to begin the loop.
  (bind _output_get (set `self.OriginalLocation` (`SceneComponent.RelativeLocation` (`self.Press`))))
  (set `self.PressDropLocation` (- _output_get (`KismetMathLibrary.MakeVector` 0.0 0.0 (`self.PressMovement`)))))

(event `PressDown`
  (params (Robot :type "/Game/Dynamic/Blueprints/SummerLV/BGAnim/BP_BgRobotTransform Object Reference"))
  (bind _output_get (set `self.Robot` Robot))
  (`self.SetActorTickEnabled` true)
  (`KismetSystemLibrary.Delay` 0.5)
  (`KismetSystemLibrary.MoveComponentTo` (`self.Press`) (`self.PressDropLocation`) (struct) false false (`self.TravelTime`))
  (`KismetSystemLibrary.Delay` (`self.TimeBetween`))
  (`/Game/Dynamic/Blueprints/SummerLV/BGAnim/BP_BgRobotTransform.SwapModel (Robot)` Robot)
  (`/Game/Dynamic/Blueprints/SummerLV/BGAnim/BP_BgRobotTransform.SwapModel (Robot)` _output_get)
  (`KismetSystemLibrary.Delay` (`self.TimeBetween`))
  (`self.PressUp`))

(event `PressUp`
  (`KismetSystemLibrary.MoveComponentTo` (`self.Press`) (`self.OriginalLocation`) (struct) false false (`self.TravelTime`))
  (`self.SetActorTickEnabled` false)
  (`KismetSystemLibrary.Delay` (`self.TimeBetween`))
  (`/Game/Dynamic/Blueprints/SummerLV/BGAnim/BP_BgRobotTransform.Leave` (`self.Robot`)))

(fn `UserConstructionScript`)