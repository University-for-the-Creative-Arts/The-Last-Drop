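; BP_DoorCloser is a one-shot trigger actor that closes a door behind the player.
; On BeginPlay it finds and caches the BP_BodyChar player character.
; When that character overlaps the DoorCloser component, it calls ActivateDeactivate on the StartCloseDoor reference, if valid.
; It then turns off the component's overlap events so it does not fire again, even if the reference was invalid.
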(event `self.ReceiveBeginPlay`
  (bind _returnvalue (`GameplayStatics.GetActorOfClass` "/Game/Dynamic/Blueprints/Characters/BodyChar/BP_BodyChar.BP_BodyChar_C"))
  (set `self.PlayerCharacter` _returnvalue))

(event `self.DoorCloser.OnComponentBeginOverlap`
  (params (OverlappedComponent :type "PrimitiveComponent Object Reference") (OtherActor :type "Actor Object Reference") (OtherComp :type "PrimitiveComponent Object Reference") (OtherBodyIndex :type Integer) (bFromSweep :type Boolean) (SweepResult :type "HitResult Structure (by ref)"))
  ;[1 0.5718 0.7911] Closes door behind player
  (if (== OtherActor (`self.PlayerCharacter`))
    (`/Engine/EditorBlueprintResources/StandardMacros.IsValid` (`self.StartCloseDoor`)
      (:`Is Valid`
        (`/Game/Dynamic/Blueprints/Environment/Activatable/BP_ActivatableParent.Activate/Deactivate` (`self.StartCloseDoor`)))
      (:`Is Not Valid`
        _))
    (set `PrimitiveComponent.bGenerateOverlapEvents` false (`self.DoorCloser`))))

(fn `UserConstructionScript`)