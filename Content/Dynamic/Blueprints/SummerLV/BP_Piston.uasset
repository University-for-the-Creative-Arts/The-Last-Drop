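; A timed piston press hazard that can crush the player, starting its loop on BeginPlay or through Activate.
; PressDown and PressUp alternate via MoveComponentTo and delays, swapping the light material, while Tick scales the cylinder to follow the press.
; With Crush enabled, the overlap box is live during descent; an overlapping player who is not falling ragdolls, loses the bubble, then LV_SummerTesting opens after a delay.
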(event `self.ReceiveBeginPlay`
  ;[1 1 1] Begins by setting the starting and end location of the end of the press, and checks if Auto Activate is true in order to begin the loop.
  (bind _output_get (set `self.OriginalLocation` (`SceneComponent.RelativeLocation` (`self.Press`))))
  (set `self.PressDropLocation` (- _output_get (`KismetMathLibrary.MakeVector` 0.0 0.0 (`self.PressMovement`))))
  (if (`self.AutoActivate?`)
    (`self.Activate`)))

(event `PressDown`
  (`PrimitiveComponent.SetMaterial` (`self.Light`) 0 (`|GetArrayItem` (`self.LightMaterials`) 1))
  (`KismetSystemLibrary.Delay` 0.5)
  (if (`self.Crush?`)
    (set `PrimitiveComponent.bGenerateOverlapEvents` true (`self.Box`)))
  (`self.SetActorTickEnabled` true)
  (`KismetSystemLibrary.MoveComponentTo` (`self.Press`) (`self.PressDropLocation`) (struct) false false (`self.TravelTime`))
  (set `PrimitiveComponent.bGenerateOverlapEvents` false (`self.Box`))
  (set `self.TopCollision?` false)
  (`KismetSystemLibrary.Delay` (`self.TimeBetween`))
  (`self.PressUp`))

(event `PressUp`
  (`PrimitiveComponent.SetMaterial` (`self.Light`) 0 (`|GetArrayItem` (`self.LightMaterials`)))
  (set `PrimitiveComponent.bGenerateOverlapEvents` false (`self.Box`))
  (set `self.TopCollision?` false)
  (`KismetSystemLibrary.MoveComponentTo` (`self.Press`) (`self.OriginalLocation`) (struct) false false 1.0)
  (`self.SetActorTickEnabled` true)
  (`KismetSystemLibrary.Delay` (`self.PressDelay`))
  (`self.PressDown`))

(event `self.ReceiveTick`
  (params (DeltaSeconds :type "Float (single-precision)"))
  (bind _returnvalue (`GameplayStatics.GetPlayerCharacter` 0))
  (bind _returnvalue_2 (`GameplayStatics.GetPlayerController` 0))
  (bind (_relativelocation_x _relativelocation_y _relativelocation_z) (`KismetMathLibrary.BreakVector` (`SceneComponent.RelativeLocation` (`self.Press`))))
  (`SceneComponent.SetRelativeScale3D` (`self.PressCylinder`) (`KismetMathLibrary.MakeVector` 1.0 1.0 (`KismetMathLibrary.Abs` _relativelocation_z)))
  (if (and (`self.TopCollision?`) (not (`NavMovementComponent.IsFalling` (`Character.CharacterMovement` (`GameplayStatics.GetPlayerCharacter` 0)))))
    (bind _asbp_body_char (cast `/Game/Dynamic/Blueprints/Characters/BodyChar/BP_BodyChar` _returnvalue))
    (bind _aspc_bubble_bandit (cast `/Game/Dynamic/Blueprints/Interfaces/PC_BubbleBandit` _returnvalue_2))
    (`self.DisableInput` _aspc_bubble_bandit _aspc_bubble_bandit)
    (`self.DisableInput` _asbp_body_char _returnvalue_2)
    (bind _mesh (`Character.Mesh` _asbp_body_char))
    (`PrimitiveComponent.SetCollisionProfileName` _mesh "Ragdoll" true)
    (`PrimitiveComponent.SetSimulatePhysics` _mesh true)
    (`CharacterMovementComponent.DisableMovement` (`Character.CharacterMovement` _returnvalue))
    (bind _returnvalue_3 (`GameplayStatics.GetActorOfClass` "/Game/Dynamic/Blueprints/Characters/BubbleChar/BP_BubbleChar.BP_BubbleChar_C"))
    (`/Engine/EditorBlueprintResources/StandardMacros.IsValid` _returnvalue_3
      (:`Is Valid`
        (`/Game/Dynamic/Blueprints/Actor_Components/AC_BubbleControls.Pop` (`/Game/Dynamic/Blueprints/Characters/BubbleChar/BP_BubbleChar.AC_BubbleControls` _returnvalue_3) _returnvalue_3))
      (:`Is Not Valid`
        _))
    (`SceneComponent.SetHiddenInGame` (`/Game/Dynamic/Blueprints/Characters/BodyChar/BP_BodyChar.Sphere` _asbp_body_char) true false)
    (`KismetSystemLibrary.Delay` 3.0)
    (message `/Game/Dynamic/SaveSystem/BPI_SaveGame.LoadGameData` (`GameplayStatics.GetPlayerCharacter` 0) false)
    (`GameplayStatics.OpenLevel` "LV_SummerTesting")))

(event `self.Box.OnComponentBeginOverlap`
  (params (OverlappedComponent :type "PrimitiveComponent Object Reference") (OtherActor :type "Actor Object Reference") (OtherComp :type "PrimitiveComponent Object Reference") (OtherBodyIndex :type Integer) (bFromSweep :type Boolean) (SweepResult :type "HitResult Structure (by ref)"))
  (if (and (== OtherActor (`GameplayStatics.GetPlayerCharacter` 0)) (`GameplayStatics.ObjectIsA` OtherComp "/Script/Engine.CapsuleComponent"))
    (set `self.TopCollision?` true)
    (`KismetSystemLibrary.PrintString` "CollidingTop" true true (struct :`R` 0.017851 :`B` 1.0 :`A` 1.0) 2.0 "7878")))

(event `self.Box.OnComponentEndOverlap`
  (params (OverlappedComponent :type "PrimitiveComponent Object Reference") (OtherActor :type "Actor Object Reference") (OtherComp :type "PrimitiveComponent Object Reference") (OtherBodyIndex :type Integer))
  ;[1 1 1] Checks if the player is no longer touching the top of the piston
  (if (== OtherActor (`GameplayStatics.GetPlayerCharacter` 0))
    (set `self.TopCollision?` false)
    (`KismetSystemLibrary.PrintString` "NotCollidingTop" true true (struct :`R` 0.017851 :`B` 1.0 :`A` 1.0) 2.0 "7878")))

(event `Activate`
  ;[1 1 1] Activates the loop
  (`KismetSystemLibrary.Delay` (`self.PressDelay`))
  (`self.PressDown`))

(fn `UserConstructionScript`)