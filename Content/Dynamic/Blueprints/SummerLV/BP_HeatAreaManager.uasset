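; BP_HeatAreaManager is an actor that shows the player's heat level on the character mesh through a dynamic M_HeatRoomMat material.
; UpdateValues stores the heat, and Tick smoothly interpolates the inverted, normalized value into the Heat scalar parameter, with a debug printout.
; End plays the Cooldown timeline from a position derived from the current value, then restores MAT_BodyChar and destroys the actor.
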(event `self.ReceiveBeginPlay`
  (bind _returnvalue (`KismetMaterialLibrary.CreateDynamicMaterialInstance` "/Game/Static/Materials/M_HeatRoomMat.M_HeatRoomMat"))
  (bind _output_get (set `self.Mat Instance` _returnvalue))
  (`PrimitiveComponent.SetMaterial` (`Character.Mesh` (`GameplayStatics.GetPlayerCharacter` 0)) 0 _output_get)
  (bind _returnvalue_2 (`MaterialInstanceDynamic.K2_GetScalarParameterValue` (`self.Mat Instance`) "None"))
  (set `self.InterpValue` _returnvalue_2))

(event `UpdateValues`
  (params (Heat :type Integer))
  (set `self.PlayerHeat` Heat))

(event `self.ReceiveTick`
  (params (DeltaSeconds :type "Float (single-precision)"))
  (bind _returnvalue (`KismetMathLibrary.FInterpTo` (`self.InterpValue`) (- 1.0 (/ (`KismetMathLibrary.Conv_IntToDouble` (`self.PlayerHeat`)) 10.0)) (`GameplayStatics.GetWorldDeltaSeconds`) 5.0))
  (bind _output_get (set `self.InterpValue` _returnvalue))
  (`MaterialInstanceDynamic.SetScalarParameterValue` (`self.Mat Instance`) "Heat" _output_get)
  (`KismetSystemLibrary.PrintText` (`KismetTextLibrary.Conv_DoubleToText` _returnvalue "HalfToEven") true true (struct :`R` 1.0 :`G` 0.359132 :`B` 0.509859 :`A` 1.0) 2.0 "6767676"))

(event `End`
  (`|ExecutionSequence`
    (:`then_0`
      (bind (_direction _cooldown) (`Timeline|Cooldown` :`NewTime` (- 1.0 (`self.InterpValue`)) :!via `SetNewTime` :!label _label)
        (:`Update`
          (`MaterialInstanceDynamic.SetScalarParameterValue` (`self.Mat Instance`) "Heat" _cooldown))
        (:`Finished`
          (`PrimitiveComponent.SetMaterial` (`Character.Mesh` (`GameplayStatics.GetPlayerCharacter` 0)) 0 "/Game/Static/Characters/MAT_BodyChar.MAT_BodyChar")
          (`KismetSystemLibrary.PrintText` "Destroyed")
          (`self.K2_DestroyActor`))))
    (:`then_1`
      (goto _label))))

(fn `UserConstructionScript`)