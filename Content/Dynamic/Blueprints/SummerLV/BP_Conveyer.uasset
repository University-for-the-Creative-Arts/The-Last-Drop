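; BP_Conveyer is a conveyor belt actor that carries player characters along it.
; Each tick, it gathers BP_BodyChar actors overlapping its Box and offsets each along the Arrow component's forward vector, scaled by Speed and delta time.
; The movement is a direct world offset without sweep, so collisions are not checked while carrying them.
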(event `self.ReceiveTick`
  (params (DeltaSeconds :type "Float (single-precision)"))
  (bind _overlappingactors (`PrimitiveComponent.GetOverlappingActors` (`self.Box`) "/Game/Dynamic/Blueprints/Characters/BodyChar/BP_BodyChar.BP_BodyChar_C"))
  ;[1 1 1] Checks if the player is stood on the conveyer belt. If they are, it moves them in the direction of the arrow.
  (if (`KismetArrayLibrary.Array_IsNotEmpty` _overlappingactors)
    (for _array_element _overlappingactors
      (`self.K2_AddActorWorldOffset` _array_element (* (* DeltaSeconds (`self.Speed`)) (`KismetMathLibrary.GetForwardVector` (`SceneComponent.K2_GetComponentRotation` (`self.Arrow`)))) false false))))

(fn `UserConstructionScript`)