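; BP_Water is a water body in the summer level that cools the player down and pauses their in-water state in the room's heat mechanic.
; On overlap by BP_BodyChar, it flags the player as in water on RoomWithin, refills PlayerHeat to the maximum and also resets the BP_HeatAreaManager's heat to a fixed value.
; Leaving clears the flag and calls HeatActive on the room.
; The construction script sizes the underwater RectLight to the actor's scale.
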(event `self.ReceiveBeginPlay`
  ;[1 1 1] Find player character
  (bind _returnvalue (`GameplayStatics.GetActorOfClass` "/Game/Dynamic/Blueprints/Characters/BodyChar/BP_BodyChar.BP_BodyChar_C"))
  (set `self.PlayerCharacter` _returnvalue))

(event `self.Water.OnComponentBeginOverlap`
  (params (OverlappedComponent :type "PrimitiveComponent Object Reference") (OtherActor :type "Actor Object Reference") (OtherComp :type "PrimitiveComponent Object Reference") (OtherBodyIndex :type Integer) (bFromSweep :type Boolean) (SweepResult :type "HitResult Structure (by ref)"))
  (bind _roomwithin (`self.RoomWithin`))
  ;[0.3748 0.3416 1] Player overlaps with water
  (if (== OtherActor (`self.PlayerCharacter`))
    (set `/Game/Dynamic/Blueprints/SummerLV/BP_HeatArea.PlayerInWater?` true _roomwithin)
    (`KismetSystemLibrary.PrintString` "Cooled Down" true true (struct :`G` 0.66 :`B` 1.0 :`A` 1.0) 2.0 "238")
    (set `/Game/Dynamic/Blueprints/SummerLV/BP_HeatArea.PlayerHeat` (`/Game/Dynamic/Blueprints/SummerLV/BP_HeatArea.MaxHeat` _roomwithin) _roomwithin)
    (bind _returnvalue (`GameplayStatics.GetActorOfClass` "/Game/Dynamic/Blueprints/SummerLV/BP_HeatAreaManager.BP_HeatAreaManager_C"))
    (`/Engine/EditorBlueprintResources/StandardMacros.IsValid` _returnvalue
      (:`Is Valid`
        (set `/Game/Dynamic/Blueprints/SummerLV/BP_HeatAreaManager.PlayerHeat` 11 _returnvalue)))))

(event `self.Water.OnComponentEndOverlap`
  (params (OverlappedComponent :type "PrimitiveComponent Object Reference") (OtherActor :type "Actor Object Reference") (OtherComp :type "PrimitiveComponent Object Reference") (OtherBodyIndex :type Integer))
  (bind _roomwithin (`self.RoomWithin`))
  ;[1 0.336 0.2596] Player gets out of water
  (if (== OtherActor (`self.PlayerCharacter`))
    (if (`/Game/Dynamic/Blueprints/SummerLV/BP_HeatArea.PlayerInWater?` _roomwithin)
      (set `/Game/Dynamic/Blueprints/SummerLV/BP_HeatArea.PlayerInWater?` false _roomwithin)
      (`/Game/Dynamic/Blueprints/SummerLV/BP_HeatArea.HeatActive` _roomwithin))))

(fn `UserConstructionScript`
  (bind _rectlight (`self.RectLight`))
  (bind (_returnvalue_x _returnvalue_y) (`KismetMathLibrary.BreakVector` (`SceneComponent.K2_GetComponentScale` (`self.DefaultSceneRoot`))))
  ;[0.0287 0.04022 0.1858] Changes size of light below water
  (`RectLightComponent.SetSourceWidth` _rectlight (* _returnvalue_y 100.0))
  (`RectLightComponent.SetSourceHeight` _rectlight (* _returnvalue_x 100.0)))