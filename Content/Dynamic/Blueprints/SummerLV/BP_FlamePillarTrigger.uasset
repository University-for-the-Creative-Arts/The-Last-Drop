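; BP_FlamePillarTrigger is a trigger that starts and stops a group of flame pillars as the player moves through it.
; Separate Activate and Deactivate overlap components respond only to player 0's capsule component.
; An Active flag blocks repeat triggers, and each valid overlap calls ActivateCycle or DeactivateCycle on every entry in the FlamePillars array.
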(event `self.Activate.OnComponentBeginOverlap`
  (params (OverlappedComponent :type "PrimitiveComponent Object Reference") (OtherActor :type "Actor Object Reference") (OtherComp :type "PrimitiveComponent Object Reference") (OtherBodyIndex :type Integer) (bFromSweep :type Boolean) (SweepResult :type "HitResult Structure (by ref)"))
  (if (and (== OtherActor (`GameplayStatics.GetPlayerCharacter` 0)) (`GameplayStatics.ObjectIsA` OtherComp "/Script/Engine.CapsuleComponent") (not (`self.Active?`)))
    (set `self.Active?` true)
    (for _array_element (`self.FlamePillars`)
      (`/Game/Dynamic/Blueprints/SummerLV/BP_FlamePipe.ActivateCycle` _array_element))))

(event `self.Deactivate.OnComponentBeginOverlap`
  (params (OverlappedComponent :type "PrimitiveComponent Object Reference") (OtherActor :type "Actor Object Reference") (OtherComp :type "PrimitiveComponent Object Reference") (OtherBodyIndex :type Integer) (bFromSweep :type Boolean) (SweepResult :type "HitResult Structure (by ref)"))
  (if (and (== OtherActor (`GameplayStatics.GetPlayerCharacter` 0)) (`GameplayStatics.ObjectIsA` OtherComp "/Script/Engine.CapsuleComponent") (`self.Active?`))
    (set `self.Active?` false)
    (for _array_element (`self.FlamePillars`)
      (`/Game/Dynamic/Blueprints/SummerLV/BP_FlamePipe.DeactivateCycle` _array_element))))

(fn `UserConstructionScript`)