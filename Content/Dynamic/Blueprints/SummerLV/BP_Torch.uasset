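; BP_Torch is a torch that switches on its Niagara effect when the player's bubble character touches its base.
; On BeginPlay it caches the player character as BP_BodyChar.
; The Base overlap compares the other actor to the bubble character reached through that player's PCBubbleChar, then sets a one-way Active flag and activates Niagara.
; A note marks the trigger for editing based on bubble state, which is not checked.
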(event `self.ReceiveBeginPlay`
  (bind _asbp_body_char (cast `/Game/Dynamic/Blueprints/Characters/BodyChar/BP_BodyChar` (`GameplayStatics.GetPlayerCharacter` 0)))
  (set `self.Player` _asbp_body_char))

(event `self.Base.OnComponentBeginOverlap`
  (params (OverlappedComponent :type "PrimitiveComponent Object Reference") (OtherActor :type "Actor Object Reference") (OtherComp :type "PrimitiveComponent Object Reference") (OtherBodyIndex :type Integer) (bFromSweep :type Boolean) (SweepResult :type "HitResult Structure (by ref)"))
  (if (and (== OtherActor (`/Game/Dynamic/Blueprints/Interfaces/PC_BubbleBandit.BP Bubble Char` (`/Game/Dynamic/Blueprints/Characters/BodyChar/BP_BodyChar.PC_BubbleChar` (`self.Player`)))) (not (`self.Active?`)))
    (set `self.Active?` true)
    (`ActorComponent.Activate` (`self.Niagara`) false)))

(fn `UserConstructionScript`)