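; BP_BgSpawner is a timed spawner that continually creates actors of a configurable class at its own position.
; BeginPlay sets the actor tick interval to TickTime, so each Tick spawns one actor, ignoring collisions.
; The construction script caches the spawn location from the actor, and an optional RandomRot flag randomizes yaw before each spawn.
; It has no spawn limit or cleanup of its own.
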(event `self.ReceiveBeginPlay`
  (`self.SetActorTickInterval` (`self.TickTime`)))

(event `self.ReceiveTick`
  (params (DeltaSeconds :type "Float (single-precision)"))
  (bind (_returnvalue_roll _returnvalue_pitch _returnvalue_yaw) (`KismetMathLibrary.BreakRotator` (`KismetMathLibrary.RandomRotator` false)))
  (if (`self.RandomRot?`)
    (set `self.Spawn Transform Rotation` (`KismetMathLibrary.MakeRotator` 0.0 0.0 _returnvalue_yaw)))
  (`|SpawnActorFromClass` (`self.SpawnClass`) (`KismetMathLibrary.MakeTransform` (`self.Spawn Transform Location`) (`self.Spawn Transform Rotation`) (`self.Spawn Transform Scale`)) "AlwaysSpawn" "MultiplyWithRoot" null null))

(fn `UserConstructionScript`
  (set `self.Spawn Transform Location` (`self.K2_GetActorLocation`)))