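; BP_BgConveyorObject1 is a background conveyor object for the SummerLV level that moves along a supplied arrow's direction when told to fall.
; The Fall event stores the Arrow and plays a timeline from the start.
; Each timeline update offsets the actor, without sweep, along the arrow's forward vector by the timeline's Speed scaled by delta time.
; A debug print shows that offset every update.
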(event `Fall`
  (params (Arrow :type "ArrowComponent Object Reference"))
  (set `self.Arrow` Arrow)
  (bind (_direction _speed) (`Timeline|Timeline` :!via `PlayFromStart`)
    (:`Update`
      (`/Engine/EditorBlueprintResources/StandardMacros.IsValid` self
        (:`Is Valid`
          (bind _returnvalue (* (* _speed (`GameplayStatics.GetWorldDeltaSeconds`)) (`KismetMathLibrary.GetForwardVector` (`SceneComponent.K2_GetComponentRotation` (`self.Arrow`)))))
          (`KismetSystemLibrary.PrintString` (`KismetStringLibrary.Conv_VectorToString` _returnvalue) true true (struct :`R` 0.177314 :`B` 1.0 :`A` 1.0) 2.0 "22221")
          (`self.K2_AddActorWorldOffset` self _returnvalue false false))))))

(fn `UserConstructionScript`)