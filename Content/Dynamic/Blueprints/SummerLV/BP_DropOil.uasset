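; BP_DropOil is a short-lived oil drop that turns the player's bubble character into its oil variant on contact, then destroys itself.
; It caches the player BP_BodyChar on BeginPlay and self-destructs after a fixed delay.
; On the first capsule overlap with a bubble that is neither oil nor fire, it respawns that bubble as BP_BubbleChar_Child_Oil at the same transform and hands camera tracking to the new actor.
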(event `self.ReceiveBeginPlay`
  (bind _asbp_body_char (cast `/Game/Dynamic/Blueprints/Characters/BodyChar/BP_BodyChar` (`GameplayStatics.GetPlayerCharacter` 0)))
  (set `self.Player` _asbp_body_char)
  (`KismetSystemLibrary.Delay` 5.0)
  (`self.K2_DestroyActor`))

(event `self.Capsule.OnComponentBeginOverlap`
  (params (OverlappedComponent :type "PrimitiveComponent Object Reference") (OtherActor :type "Actor Object Reference") (OtherComp :type "PrimitiveComponent Object Reference") (OtherBodyIndex :type Integer) (bFromSweep :type Boolean) (SweepResult :type "HitResult Structure (by ref)"))
  (bind _player (`self.Player`))
  (bind _ac_cambehaviour (`/Game/Dynamic/Blueprints/Characters/BodyChar/BP_BodyChar.AC_CamBehaviour` _player))
  (bind _bp_bubble_char (`/Game/Dynamic/Blueprints/Interfaces/PC_BubbleBandit.BP Bubble Char` (`/Game/Dynamic/Blueprints/Characters/BodyChar/BP_BodyChar.PC_BubbleChar` _player)))
  (if (and (== OtherActor _bp_bubble_char) (not (or (`GameplayStatics.ObjectIsA` _bp_bubble_char "/Game/Dynamic/Blueprints/SummerLV/BP_BubbleChar_Child_Oil.BP_BubbleChar_Child_Oil_C") (`GameplayStatics.ObjectIsA` _bp_bubble_char "/Game/Dynamic/Blueprints/SummerLV/BP_BubbleChar_Child_Fire.BP_BubbleChar_Child_Fire_C"))) (== (`self.Touched?`) false))
    (set `self.Touched?` true)
    (`/Game/Dynamic/Blueprints/Actor_Components/AC_CamBehaviour.RemoveTrackingActor` _ac_cambehaviour OtherActor)
    (set `self.Transform` (`self.GetTransform` _bp_bubble_char))
    (`KismetSystemLibrary.PrintString` "Bubble in Oil" true true (struct :`R` 0.085375 :`G` 0.001344 :`B` 0.203125 :`A` 1.0) 2.0 "101010101010")
    (`self.K2_DestroyActor` _bp_bubble_char)
    (bind _returnvalue (`|SpawnActorFromClass` "/Game/Dynamic/Blueprints/SummerLV/BP_BubbleChar_Child_Oil.BP_BubbleChar_Child_Oil_C" (`self.Transform`) "AlwaysSpawn" "MultiplyWithRoot" null (`self.Player`) null))
    (`/Game/Dynamic/Blueprints/Actor_Components/AC_CamBehaviour.AddTrackingActor` _ac_cambehaviour _returnvalue)
    (`self.K2_DestroyActor`)))

(fn `UserConstructionScript`)