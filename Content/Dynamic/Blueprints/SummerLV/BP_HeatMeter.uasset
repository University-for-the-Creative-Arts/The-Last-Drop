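; BP_HeatMeter is a heat gauge actor for the summer level that displays the player's heat beside the character.
; Each Tick it moves to player character 0's location with a fixed Y offset and fills its WBP_Heat widget from the stored PlayerHeat.
; ChangeHeat receives the heat value from outside, while ChangeHeatColour switches the widget between Cool and Warm depending on whether the player is in water.
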(event `self.ReceiveBeginPlay`
  (bind _aswbp_heat (cast `/Game/Dynamic/Blueprints/SummerLV/WBP_Heat` (`WidgetComponent.GetWidget` (`self.Widget`))))
  (set `self.HeatWidget` _aswbp_heat))

(event `ChangeHeat`
  (params (PlayerHeat :type Integer))
  (set `self.Player Heat` PlayerHeat))

(event `self.ReceiveTick`
  (params (DeltaSeconds :type "Float (single-precision)"))
  (`self.Set Position`)
  (`/Game/Dynamic/Blueprints/SummerLV/WBP_Heat.FillMeter` (`self.HeatWidget`) (`self.Player Heat`)))

(event `ChangeHeatColour`
  (params (`InWater?` :type Boolean))
  (bind _heatwidget (`self.HeatWidget`))
  (if `InWater?`
    (`/Game/Dynamic/Blueprints/SummerLV/WBP_Heat.Cool` _heatwidget)
    (else
      (`/Game/Dynamic/Blueprints/SummerLV/WBP_Heat.Warm` _heatwidget))))

(fn `Set Position`
  (bind (_returnvalue_x _returnvalue_y _returnvalue_z) (`KismetMathLibrary.BreakVector` (`self.K2_GetActorLocation` (`GameplayStatics.GetPlayerCharacter` 0))))
  (`self.K2_SetActorLocation` (`KismetMathLibrary.MakeVector` _returnvalue_x (- _returnvalue_y 65.0) _returnvalue_z)))

(fn `UserConstructionScript`)