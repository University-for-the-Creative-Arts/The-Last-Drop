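; Falling lift platform hung on four cables that drops when the player's capsule enters its trigger box, then respawns.
; The trigger plays a timeline shake, then detaches the cables and enables physics on the lift.
; Tick watches for low velocity or a fall timeout, then hides the lift and, after a delay, spawns a fresh copy and destroys itself.
; The construction script applies CableLength to cable height and length.
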(event `self.ReceiveBeginPlay`
  (set `self.StartingLocation` (`SceneComponent.K2_GetComponentLocation` (`self.FallingLift`)))
  (set `self.Cables` (`|MakeArray` (`self.Cable`) (`self.Cable1`) (`self.Cable2`) (`self.Cable3`))))

(event `LiftShake`
  (bind (_startinglocation_x _startinglocation_y _startinglocation_z) (`KismetMathLibrary.BreakVector` (`self.StartingLocation`)))
  (bind (_direction _shakepos) (`Timeline|Timeline` :!via `PlayFromStart`)
    (:`Update`
      (`SceneComponent.K2_SetWorldLocation` (`self.FallingLift`) (`KismetMathLibrary.MakeVector` (+ _shakepos _startinglocation_x) _startinglocation_y _startinglocation_z) false true))))

(event `self.Box.OnComponentBeginOverlap`
  (params (OverlappedComponent :type "PrimitiveComponent Object Reference") (OtherActor :type "Actor Object Reference") (OtherComp :type "PrimitiveComponent Object Reference") (OtherBodyIndex :type Integer) (bFromSweep :type Boolean) (SweepResult :type "HitResult Structure (by ref)"))
  (if (and (== OtherActor (`GameplayStatics.GetPlayerCharacter` 0)) (`GameplayStatics.ObjectIsA` OtherComp "/Script/Engine.CapsuleComponent") (not (`self.Broken?`)))
    (set `self.Broken?` true)
    (`self.LiftShake`)
    (`KismetSystemLibrary.Delay` 1.05)
    (for _array_element (`self.Cables`)
      (set `CableComponent.bAttachEnd` false _array_element)
      (`CableComponent.SetAttachEndToComponent` _array_element null "None"))
    (`PrimitiveComponent.SetSimulatePhysics` (`self.FallingLift`) true)
    (set `self.FallTime` 0.0)
    (`KismetSystemLibrary.Delay` 0.1)
    (`self.SetActorTickEnabled` true)))

(event `self.ReceiveTick`
  (params (DeltaSeconds :type "Float (single-precision)"))
  (bind _fallinglift (`self.FallingLift`))
  (bind _returnvalue (`KismetMathLibrary.VSize` (`SceneComponent.GetComponentVelocity` (`self.FallingLift`))))
  (bind _output_get (set `self.FallTime` (+ (`self.FallTime`) DeltaSeconds)))
  (if (> _returnvalue 7.0)
    (`KismetSystemLibrary.PrintString` (`KismetStringLibrary.Conv_DoubleToString` _returnvalue) true true (struct :`R` 0.420045 :`G` 1.0 :`B` 0.807128 :`A` 1.0) 2.0 "12")
    (if (>= _output_get 3.0)
      (`PrimitiveComponent.SetSimulatePhysics` (`self.FallingLift`) false :!label _label)
      (`self.SetActorTickEnabled` false)
      (`KismetSystemLibrary.Delay` 0.1)
      (`PrimitiveComponent.SetCollisionEnabled` _fallinglift "NoCollision")
      (`SceneComponent.SetVisibility` _fallinglift false false)
      (`KismetSystemLibrary.Delay` 3.0)
      (`self.Fix`))
    (else
      (`KismetSystemLibrary.PrintString` "HitGround" true true (struct :`G` 0.66 :`B` 1.0 :`A` 1.0) 2.0 "12")
      (goto _label))))

(event `Fix`
  (`|SpawnActorFromClass` "BP_FallingPlatform_C" (`self.GetTransform`) "Undefined" "MultiplyWithRoot" null (`self.Cable Length`) null)
  (`self.K2_DestroyActor`))

(fn `UserConstructionScript`
  (bind _cable_length (`self.Cable Length`))
  (bind _output_get (set `self.Cables` (`|MakeArray` (`self.Cable`) (`self.Cable1`) (`self.Cable2`) (`self.Cable3`))))
  (for _array_element _output_get
    (bind (_relativelocation_x _relativelocation_y) (`KismetMathLibrary.BreakVector` (`SceneComponent.RelativeLocation` _array_element)))
    (`SceneComponent.K2_SetRelativeLocation` _array_element (`KismetMathLibrary.MakeVector` _relativelocation_x _relativelocation_y _cable_length) false false)
    (set `CableComponent.CableLength` _cable_length _array_element)))