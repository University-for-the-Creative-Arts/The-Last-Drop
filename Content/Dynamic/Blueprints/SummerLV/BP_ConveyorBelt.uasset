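; BP_ConveyorBelt is a conveyor belt actor that configures the look of its moving belt surface.
; The construction script calls SetMat to put a dynamic material instance on slot 1 of the Belt component.
; It then sets the material's Speed, signed by DirectionRight, and its Scale from the visual speed and scale variables.
; The event graph holds only disabled stub events, so the file contains no runtime transport logic.
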(fn `UserConstructionScript`
  (bind _matinstance (`self.SetMat`))
  (`MaterialInstanceDynamic.SetScalarParameterValue` _matinstance "Speed" (* (`self.BeltVisualSpeed`) (`KismetMathLibrary.SelectInt` 1 -1 (`self.DirectionRight?`))))
  (`MaterialInstanceDynamic.SetScalarParameterValue` _matinstance "Scale" (`self.BeltViusalScale`)))