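; Spinning hazard actor for the SummerLV content that carries two always-burning flamethrowers.
; RotatingMovement spins it at RotationSpeed, set in both the construction script and BeginPlay.
; On BeginPlay it spawns a BP_FlamePipe at each spawn point, aligned to a cylinder with one yaw-flipped 180 degrees, and attaches it to itself.
; Each pipe has its activation radius overlaps disabled and is ignited immediately.
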(event `self.ReceiveBeginPlay`
  (set `RotatingMovementComponent.RotationRate` (`KismetMathLibrary.MakeRotator` 0.0 0.0 (`self.RotationSpeed`)) (`self.RotatingMovement`))
  (`|ExecutionSequence`
    (:`then_0`
      (`self.SetupFlamethrowers` (`self.SpawnPoint`) (`self.Cylinder3`) true))
    (:`then_1`
      (`self.SetupFlamethrowers` (`self.SpawnPoint1`) (`self.Cylinder2`)))))

(fn `SetupFlamethrowers`
  (params (SpawnPointComponent :type "SceneComponent Object Reference") (SpawnRotationComponent :type "SceneComponent Object Reference") (`Flip?` :type Boolean))
  (returns (ReturnActor :type "/Game/Dynamic/Blueprints/SummerLV/BP_FlamePipe Object Reference"))
  (bind (_returnvalue_roll _returnvalue_pitch _returnvalue_yaw) (`KismetMathLibrary.BreakRotator` (`SceneComponent.K2_GetComponentRotation` SpawnRotationComponent)))
  (bind _returnvalue (`|SpawnActorFromClass` "/Game/Dynamic/Blueprints/SummerLV/BP_FlamePipe.BP_FlamePipe_C" (`KismetMathLibrary.MakeTransform` (`SceneComponent.K2_GetComponentLocation` SpawnPointComponent) (`KismetMathLibrary.MakeRotator` _returnvalue_roll _returnvalue_pitch (- _returnvalue_yaw (`KismetMathLibrary.SelectFloat` 180.0 0.0 `Flip?`)))) "AlwaysSpawn" "MultiplyWithRoot" self false null))
  (`self.K2_AttachToActor` _returnvalue self "None" "KeepWorld" "KeepWorld" "KeepWorld" true)
  (set `PrimitiveComponent.bGenerateOverlapEvents` false (`/Game/Dynamic/Blueprints/SummerLV/BP_FlamePipe.ActivationRadius` _returnvalue))
  (`/Game/Dynamic/Blueprints/SummerLV/BP_FlamePipe.ActivateFire` _returnvalue)
  (return _returnvalue))

(fn `UserConstructionScript`
  (set `RotatingMovementComponent.RotationRate` (`KismetMathLibrary.MakeRotator` 0.0 0.0 (`self.RotationSpeed`)) (`self.RotatingMovement`)))