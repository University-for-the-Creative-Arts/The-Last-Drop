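; BP_UpLiftEnd is a lift in the summer level that rises while the screen fades, apparently as an ending sequence.
; StartSequence calls Upward, which plays the Up timeline, rate-scaled by TimeToComplete, to drive the Lift component's relative Z by MovementAmount.
; A third of TimeToComplete later, it starts a player camera fade with configurable colour, duration, audio fade and hold.
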(event `Upward`
  (`TimelineComponent.SetPlayRate` (`self.Up`) (/ 1.0 (`self.TimeToComplete`)))
  (bind (_direction _movement) (`Timeline|Up` :!via `PlayFromStart`)
    (:`Update`
      (`SceneComponent.K2_SetRelativeLocation` (`self.Lift`) (`KismetMathLibrary.MakeVector` 0.0 0.0 (* _movement (`self.MovementAmount`))) false false))))

(event `StartSequence`
  (`self.Upward`)
  (`KismetSystemLibrary.Delay` (/ (`self.TimeToComplete`) 3.0))
  (`PlayerCameraManager.StartCameraFade` (`GameplayStatics.GetPlayerCameraManager` 0) 0.0 1.0 (`self.FadeOutDuration`) (`self.FadeColour`) (`self.Should Fade Audio`) (`self.Hold when Finished`)))

(fn `UserConstructionScript`)