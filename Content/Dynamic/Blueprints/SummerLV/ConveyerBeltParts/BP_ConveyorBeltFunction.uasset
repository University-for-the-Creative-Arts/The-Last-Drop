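; Conveyor belt Blueprint that carries any actors overlapping its box along the belt's direction.
; On construction and BeginPlay, a DirectionRight flag sets the arrow component's color and flips its rotation between two opposite sideways directions.
; Each Tick offsets every overlapping actor along the arrow's world forward vector, scaled by Speed and delta time, without sweeping.
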(event `self.ReceiveBeginPlay`
  (`self.ArrowDirection`))

(event `self.ReceiveTick`
  (params (DeltaSeconds :type "Float (single-precision)"))
  (bind _overlappingactors (`PrimitiveComponent.GetOverlappingActors` (`self.Box`) null))
  (if (`KismetArrayLibrary.Array_IsNotEmpty` _overlappingactors)
    (for _array_element _overlappingactors
      (`self.K2_AddActorWorldOffset` _array_element (* (* DeltaSeconds (`self.Speed`)) (`KismetMathLibrary.GetForwardVector` (`SceneComponent.K2_GetComponentRotation` (`self.Arrow`)))) false false))))

(fn `ArrowDirection`
  (bind _arrow (`self.Arrow`))
  (bind _arrow_2 (`self.Arrow`))
  (if (`self.DirectionRight?`)
    (`ArrowComponent.SetArrowColor` _arrow_2 (struct :`R` 1.0 :`A` 1.0))
    (`SceneComponent.K2_SetRelativeRotation` _arrow_2 (struct :`Yaw` 90.0) false false)
    (else
      (`ArrowComponent.SetArrowColor` _arrow (struct :`B` 1.0 :`A` 1.0))
      (`SceneComponent.K2_SetRelativeRotation` _arrow (struct :`Yaw` -90.0) false false))))

(fn `UserConstructionScript`
  (`self.ArrowDirection`))