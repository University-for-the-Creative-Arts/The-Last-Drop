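; BP_ConveyorBeltVisual is the visual part of a conveyor belt, animating the belt surface through its material.
; It creates a dynamic material instance for slot 1 of the Belt mesh if none is valid yet.
; Both construction and BeginPlay set that instance's Speed and Scale parameters from exposed-style variables, with DirectionRight flipping the sign of the speed.
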(event `self.ReceiveBeginPlay`
  (`self.ConveyorMaterialAndDirection`))

(fn `ConveyorMaterialAndDirection`
  (`/Engine/EditorBlueprintResources/StandardMacros.IsValid` (`self.MaterialInstance`)
    (:`Is Valid`
      _)
    (:`Is Not Valid`
      (bind _matinstance (`self.SetMat`))
      (bind _output_get (set `self.MaterialInstance` _matinstance))))
  (`MaterialInstanceDynamic.SetScalarParameterValue` _output_get "Speed" (* (`self.BeltVisualSpeed`) (`KismetMathLibrary.SelectInt` 1 -1 (`self.DirectionRight?`))))
  (`MaterialInstanceDynamic.SetScalarParameterValue` (`self.MaterialInstance`) "Scale" (`self.BeltViusalScale`)))

(fn `UserConstructionScript`
  (`self.ConveyorMaterialAndDirection`))