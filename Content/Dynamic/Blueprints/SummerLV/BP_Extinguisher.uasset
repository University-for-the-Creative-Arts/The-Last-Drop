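; Extinguisher hazard actor that turns the player's fire bubble character into an oil one.
; Player overlap with its activation radius toggles ticking, the Niagara spray and a debug message.
; While active, each tick sphere-traces along the actor's vertical axis.
; A hit on the player's fire bubble destroys it, spawns an oil bubble at the same transform and swaps the camera's tracked actor.
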(event `self.ReceiveBeginPlay`
  (bind _returnvalue (`GameplayStatics.GetActorOfClass` "/Game/Dynamic/Blueprints/Characters/BodyChar/BP_BodyChar.BP_BodyChar_C"))
  (set `self.Player` _returnvalue))

(event `self.ActivationRadius.OnComponentBeginOverlap`
  (params (OverlappedComponent :type "PrimitiveComponent Object Reference") (OtherActor :type "Actor Object Reference") (OtherComp :type "PrimitiveComponent Object Reference") (OtherBodyIndex :type Integer) (bFromSweep :type Boolean) (SweepResult :type "HitResult Structure (by ref)"))
  (if (and (not (`self.Active?`)) (== OtherActor (`GameplayStatics.GetPlayerCharacter` 0)))
    (set `self.Active?` true)
    (`self.SetActorTickEnabled` true)
    (`ActorComponent.Activate` (`self.NS_Extinguish`) false)
    (`KismetSystemLibrary.PrintText` (`|FormatText` "{ObjectName} is active" (`KismetTextLibrary.Conv_StringToText` (`KismetSystemLibrary.GetDisplayName` self))) true true (struct :`R` 0.409181 :`G` 1.0 :`B` 0.910095 :`A` 1.0) 1.0)))

(event `self.ActivationRadius.OnComponentEndOverlap`
  (params (OverlappedComponent :type "PrimitiveComponent Object Reference") (OtherActor :type "Actor Object Reference") (OtherComp :type "PrimitiveComponent Object Reference") (OtherBodyIndex :type Integer))
  (if (and (`self.Active?`) (== OtherActor (`GameplayStatics.GetPlayerCharacter` 0)))
    (set `self.Active?` false)
    (`self.SetActorTickEnabled` false)
    (`ActorComponent.Deactivate` (`self.NS_Extinguish`))
    (`KismetSystemLibrary.PrintText` (`|FormatText` "{ObjectName} is inactive" (`KismetTextLibrary.Conv_StringToText` (`KismetSystemLibrary.GetDisplayName` self))) true true (struct :`R` 1.0 :`G` 0.526528 :`B` 0.839368 :`A` 1.0) 1.0)))

(event `self.ReceiveTick`
  (params (DeltaSeconds :type "Float (single-precision)"))
  (bind (_outhit _returnvalue) (`self.Traces`))
  (if _returnvalue
    (`self.ExtinguishHit` _outhit)))

(event `ExtinguishHit`
  (params (`Hit Result` :type "HitResult Structure"))
  (bind (_bblockinghit _binitialoverlap _time _distance _location _impactpoint _normal _impactnormal _physmat _hitactor) (`GameplayStatics.BreakHitResult` `Hit Result`))
  (bind _player (`self.Player`))
  (bind _ac_cambehaviour (`/Game/Dynamic/Blueprints/Characters/BodyChar/BP_BodyChar.AC_CamBehaviour` _player))
  (if (and (== _hitactor (`/Game/Dynamic/Blueprints/Interfaces/PC_BubbleBandit.BP Bubble Char` (`/Game/Dynamic/Blueprints/Characters/BodyChar/BP_BodyChar.PC_BubbleChar` _player))) (`GameplayStatics.ObjectIsA` _hitactor "/Game/Dynamic/Blueprints/SummerLV/BP_BubbleChar_Child_Fire.BP_BubbleChar_Child_Fire_C"))
    (`/Game/Dynamic/Blueprints/Actor_Components/AC_CamBehaviour.RemoveTrackingActor` _ac_cambehaviour _hitactor)
    (bind _output_get (set `self.Transform` (`self.GetTransform` _hitactor)))
    (`self.K2_DestroyActor` _hitactor)
    (bind _returnvalue (`|SpawnActorFromClass` "/Game/Dynamic/Blueprints/SummerLV/BP_BubbleChar_Child_Oil.BP_BubbleChar_Child_Oil_C" _output_get "AlwaysSpawn" "MultiplyWithRoot" null (`self.Player`) null))
    (`/Game/Dynamic/Blueprints/Actor_Components/AC_CamBehaviour.AddTrackingActor` _ac_cambehaviour _returnvalue)))

(fn `Traces`
  (returns (OutHit :type "HitResult Structure") (ReturnValue :type Boolean))
  (bind (_returnvalue_x _returnvalue_y _returnvalue_z) (`KismetMathLibrary.BreakVector` (`self.K2_GetActorLocation`)))
  (bind (_returnvalue_x_2 _returnvalue_y_2 _returnvalue_z_2) (`KismetMathLibrary.BreakVector` (`self.K2_GetActorLocation`)))
  (bind (_returnvalue_x_3 _returnvalue_y_3 _returnvalue_z_3) (`KismetMathLibrary.BreakVector` (* (`KismetMathLibrary.GetUpVector` (`self.K2_GetActorRotation`)) -300.0)))
  (bind (_returnvalue_x_4 _returnvalue_y_4 _returnvalue_z_4) (`KismetMathLibrary.BreakVector` (* (`KismetMathLibrary.GetUpVector` (`self.K2_GetActorRotation`)) 130.0)))
  (bind (_outhit _returnvalue) (`KismetSystemLibrary.SphereTraceSingle` :`Start` (`KismetMathLibrary.MakeVector` (+ _returnvalue_x_2 _returnvalue_x_4) (+ _returnvalue_y_2 _returnvalue_y_4) (+ _returnvalue_z_2 _returnvalue_z_4)) :`End` (`KismetMathLibrary.MakeVector` (+ _returnvalue_x _returnvalue_x_3) (+ _returnvalue_y _returnvalue_y_3) (+ _returnvalue_z _returnvalue_z_3)) :`Radius` 40.0 :`TraceChannel` "TraceTypeQuery2" :`DrawTime` 0.0))
  (return _outhit _returnvalue))

(fn `UserConstructionScript`)