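; Oil variant child of the bubble character that can turn into a fire bubble.
; On BeginPlay it plays an oil bubble sound, runs the parent logic and registers itself with the body character's bubble controller and its PCBubbleBandit.
; SwapToFire spawns a fire bubble child at the same transform, passes on the body character, moves camera tracking to the new bubble and destroys itself.
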(event `self.ReceiveBeginPlay`
  (bind _ac_bubblecontroller (`/Game/Dynamic/Blueprints/Characters/BodyChar/BP_BodyChar.AC_BubbleController` (`self.BP_BodyChar`)))
  (`GameplayStatics.PlaySound2D` "/Game/Static/Audio/BubbleStates/Oil_Bubble.Oil_Bubble" 1.0 1.0 0.0 null null)
  (`parent.ReceiveBeginPlay`)
  (set `/Game/Dynamic/Blueprints/Characters/BodyChar/AC_BubbleController.BP_BubbleChar` self _ac_bubblecontroller)
  (set `/Game/Dynamic/Blueprints/Interfaces/PC_BubbleBandit.BP Bubble Char` self (`/Game/Dynamic/Blueprints/Characters/BodyChar/AC_BubbleController.PC Bubble Bandit` _ac_bubblecontroller)))

(event `SwapToFire`
  (bind _ac_cambehaviour (`/Game/Dynamic/Blueprints/Characters/BodyChar/BP_BodyChar.AC_CamBehaviour` (`self.BP_BodyChar`)))
  (`/Game/Dynamic/Blueprints/Actor_Components/AC_CamBehaviour.RemoveTrackingActor` _ac_cambehaviour self)
  (bind _output_get (set `self.Transform` (`self.GetTransform` self)))
  (`KismetSystemLibrary.PrintString` "Bubble on fire" true true (struct :`R` 1.0 :`G` 0.323394 :`A` 1.0) 2.0 "101010101010")
  (bind _returnvalue (`|SpawnActorFromClass` "/Game/Dynamic/Blueprints/SummerLV/BP_BubbleChar_Child_Fire.BP_BubbleChar_Child_Fire_C" _output_get "AlwaysSpawn" "MultiplyWithRoot" null (`self.BP_BodyChar`) null))
  (`/Game/Dynamic/Blueprints/Actor_Components/AC_CamBehaviour.AddTrackingActor` _ac_cambehaviour _returnvalue)
  (`self.K2_DestroyActor`))

(fn `UserConstructionScript`
  (`parent.UserConstructionScript`))