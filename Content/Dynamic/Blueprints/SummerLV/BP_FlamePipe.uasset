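; BP_FlamePipe is a hazard pipe that cycles flames on and off on a timer.
; The cycle starts and stops through custom events or, when RadiusBased is set, as the player crosses ActivationRadius.
; While burning, Tick runs a sphere trace along the up axis.
; Hitting the player's capsule spawns BP_DeadPlayer with a flame death animation, while hitting an oil bubble swaps it to fire.
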(event `self.ReceiveBeginPlay`
  (bind _returnvalue (`GameplayStatics.GetActorOfClass` "/Game/Dynamic/Blueprints/Characters/BodyChar/BP_BodyChar.BP_BodyChar_C"))
  (set `self.Player` _returnvalue))

(event `ActivateCycle`
  ;[1 1 1] Checks if the player is within a certain radius before activating the fire - Only activates if the RadiusBased? variable is set to True
  (set `self.Active?` true :!label _label)
  (`self.FlameCycle`)
  (`KismetSystemLibrary.PrintText` (`|FormatText` "{ObjectName} is active" (`KismetTextLibrary.Conv_StringToText` (`KismetSystemLibrary.GetDisplayName` self))) true true (struct :`R` 0.365334 :`G` 0.561537 :`B` 1.0 :`A` 1.0) 1.0))

(event `self.ActivationRadius.OnComponentBeginOverlap`
  (params (OverlappedComponent :type "PrimitiveComponent Object Reference") (OtherActor :type "Actor Object Reference") (OtherComp :type "PrimitiveComponent Object Reference") (OtherBodyIndex :type Integer) (bFromSweep :type Boolean) (SweepResult :type "HitResult Structure (by ref)"))
  ;[1 1 1] Checks if the player is within a certain radius before activating the fire - Only activates if the RadiusBased? variable is set to True
  (if (== OtherActor (`GameplayStatics.GetPlayerCharacter` 0))
    (if (`self.RadiusBased?`)
      (if (not (`self.Active?`))
        (goto _label)))))

(event `DeactivateCycle`
  ;[1 1 1] Checks if the player has left the activation radius
  (set `self.Active?` false :!label _label_2)
  (`self.DeactivateFire`)
  (`KismetSystemLibrary.PrintText` (`|FormatText` "{ObjectName} is inactive" (`KismetTextLibrary.Conv_StringToText` (`KismetSystemLibrary.GetDisplayName` self))) true true (struct :`R` 1.0 :`G` 0.622676 :`B` 0.716576 :`A` 1.0) 1.0))

(event `self.ActivationRadius.OnComponentEndOverlap`
  (params (OverlappedComponent :type "PrimitiveComponent Object Reference") (OtherActor :type "Actor Object Reference") (OtherComp :type "PrimitiveComponent Object Reference") (OtherBodyIndex :type Integer))
  ;[1 1 1] Checks if the player has left the activation radius
  (if (== OtherActor (`GameplayStatics.GetPlayerCharacter` 0))
    (if (`self.RadiusBased?`)
      (if (`self.Active?`)
        (goto _label_2)))))

(event `ActivateFire`
  ;[1 1 1] Activating and deactivating the flames
  (`ActorComponent.Activate` (`self.Fire`) false)
  (`KismetSystemLibrary.Delay` 0.3)
  (`self.SetActorTickEnabled` true))

(event `DeactivateFire`
  ;[1 1 1] Activating and deactivating the flames
  (`ActorComponent.Deactivate` (`self.Fire`))
  (`self.SetActorTickEnabled` false))

(event `FlameCycle`
  ;[1 1 1] The loop that activates and deactivates the flames
  (`KismetSystemLibrary.Delay` 3.0)
  (if (`self.Active?`)
    (`self.ActivateFire`)
    (`KismetSystemLibrary.Delay` 3.0)
    (if (`self.Active?`)
      (`self.DeactivateFire`)
      (`self.FlameCycle`))))

(event `self.ReceiveTick`
  (params (DeltaSeconds :type "Float (single-precision)"))
  ;[1 1 1] When the tick is enabled, creates traces that check for actors. If there's a hit, it activates a custom event to see if the hit was from the player.
  (bind (_outhit _hit_) (`self.Traces`))
  (if _hit_
    (`self.FlameHit` _outhit)))

(event `FlameHit`
  (params (`Out Hit` :type "HitResult Structure"))
  (bind (_bblockinghit _binitialoverlap _time _distance _location _impactpoint _normal _impactnormal _physmat _hitactor _hitcomponent) (`GameplayStatics.BreakHitResult` `Out Hit`))
  (bind _player (`self.Player`))
  ;[1 1 1] Checks if the trace hit was the player. If so, it kills the player and reloads the level.
  (if (and (== _hitactor (`self.Player`)) (`GameplayStatics.ObjectIsA` _hitcomponent "/Script/Engine.CapsuleComponent") (not (`self.BurningPlayer?`)))
    (set `self.BurningPlayer?` true)
    (bind _returnvalue (`|SpawnActorFromClass` "/Game/Dynamic/Blueprints/SummerLV/BP_DeadPlayer.BP_DeadPlayer_C" (`KismetMathLibrary.MakeTransform` (`self.K2_GetActorLocation` _player) (`self.K2_GetActorRotation` _player)) "Undefined" "MultiplyWithRoot" _player null))
    (`KismetSystemLibrary.Delay` 0.01)
    (`/Game/Dynamic/Blueprints/SummerLV/BP_DeadPlayer.FlameDeathAnim` _returnvalue (struct :`R` 20.0 :`G` 2.343563 :`A` 1.0) 11.0 "/Engine/Functions/Engine_MaterialFunctions02/ExampleContent/Textures/OffsetNoiseDistanceFields_ForNormals.OffsetNoiseDistanceFields_ForNormals")
    (elif (`GameplayStatics.ObjectIsA` _hitactor "/Game/Dynamic/Blueprints/SummerLV/BP_BubbleChar_Child_Oil.BP_BubbleChar_Child_Oil_C")
      (`KismetSystemLibrary.PrintString` "OilBubble" true true (struct :`G` 0.66 :`B` 1.0 :`A` 1.0) 2.0 "88888888")
      (bind _asbp_bubble_char_child_oil (cast `/Game/Dynamic/Blueprints/SummerLV/BP_BubbleChar_Child_Oil` _hitactor))
      (`/Game/Dynamic/Blueprints/SummerLV/BP_BubbleChar_Child_Oil.SwapToFire` _asbp_bubble_char_child_oil))))

(fn `Traces`
  (returns (OutHit :type "HitResult Structure") (`Hit?` :type Boolean))
  (bind (_returnvalue_x _returnvalue_y _returnvalue_z) (`KismetMathLibrary.BreakVector` (`self.K2_GetActorLocation`)))
  (bind (_returnvalue_x_2 _returnvalue_y_2 _returnvalue_z_2) (`KismetMathLibrary.BreakVector` (`self.K2_GetActorLocation`)))
  (bind (_returnvalue_x_3 _returnvalue_y_3 _returnvalue_z_3) (`KismetMathLibrary.BreakVector` (* (`KismetMathLibrary.GetUpVector` (`self.K2_GetActorRotation`)) -70.0)))
  (bind (_returnvalue_x_4 _returnvalue_y_4 _returnvalue_z_4) (`KismetMathLibrary.BreakVector` (* (`KismetMathLibrary.GetUpVector` (`self.K2_GetActorRotation`)) 130.0)))
  (bind (_outhit _returnvalue) (`KismetSystemLibrary.SphereTraceSingle` :`Start` (`KismetMathLibrary.MakeVector` (+ _returnvalue_x_2 _returnvalue_x_4) (+ _returnvalue_y_2 _returnvalue_y_4) (+ _returnvalue_z_2 _returnvalue_z_4)) :`End` (`KismetMathLibrary.MakeVector` (+ _returnvalue_x _returnvalue_x_3) (+ _returnvalue_y _returnvalue_y_3) (+ _returnvalue_z _returnvalue_z_3)) :`Radius` 20.0 :`TraceChannel` "TraceTypeQuery2" :`DrawTime` 0.0))
  (return _outhit _returnvalue))

(fn `UserConstructionScript`)