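; Room torch puzzle manager that triggers a door once every torch in its room is active.
; On BeginPlay it gathers all BP_Torch actors with a matching room number and registers itself as their manager.
; CheckTorches tests whether all of them are active, then latches completion, prints a message and calls ActivateDeactivate on the door.
; DisableTorches switches off every torch in the room.
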(event `self.ReceiveBeginPlay`
  (bind _outactors (`GameplayStatics.GetAllActorsOfClass` "/Game/Dynamic/Blueprints/SummerLV/BP_Torch.BP_Torch_C"))
  (for _array_element _outactors
    (if (== (`/Game/Dynamic/Blueprints/SummerLV/BP_Torch.RoomNum` _array_element) (`self.RoomNumber`))
      (`KismetArrayLibrary.Array_Add` (`self.Torches`) _array_element)
      (`/Game/Dynamic/Blueprints/SummerLV/BP_Torch.ManagerSet` _array_element self))))

(event `CheckTorches`
  (if (== (`self.Complete?`) false)
    (set `self.CorrectTorches` 0)
    (for _array_element (`self.Torches`)
      (if (`/Game/Dynamic/Blueprints/SummerLV/BP_Torch.Active?` _array_element)
        (`/Engine/EditorBlueprintResources/StandardMacros.IncrementInt` (`self.CorrectTorches`))
        (else
          (break))))
    (if (== (`self.CorrectTorches`) (`KismetArrayLibrary.Array_Length` (`self.Torches`)))
      (`KismetSystemLibrary.PrintString` "Completed Room")
      (set `self.Complete?` true)
      (`/Game/Dynamic/Blueprints/Environment/Activatable/BP_ActivatableParent.Activate/Deactivate` (`self.OpenDoor`)))))

(event `DisableTorches`
  (for _array_element (`self.Torches`)
    (`/Game/Dynamic/Blueprints/SummerLV/BP_Torch.Disable` _array_element)))

(fn `UserConstructionScript`)