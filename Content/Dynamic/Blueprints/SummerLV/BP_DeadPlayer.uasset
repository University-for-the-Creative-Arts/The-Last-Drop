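; Ragdoll stand-in for the dead player that plays a flame, crush or heat-room death, then reloads the level.
; On spawn it caches its BP_BodyChar owner's velocity, hides and disables the real player, and pops any bubble.
; Flame death adds that velocity as impulse and drives a dissolve material and Niagara from a timeline; heat death swaps material.
; Each death ends with a camera fade, load-game-data message and level reopen.
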(event `self.ReceiveBeginPlay`
  (bind _asbp_body_char (cast `/Game/Dynamic/Blueprints/Characters/BodyChar/BP_BodyChar` (`self.GetOwner`)))
  (bind _output_get (set `self.Player` _asbp_body_char))
  (set `self.PlayerVelocity` (`self.GetVelocity` _output_get))
  (`KismetSystemLibrary.PrintText` "Spawned Dead Player" true true (struct :`R` 0.185861 :`B` 0.276042 :`A` 1.0) 2.0 "6789")
  (`self.SetUp`))

(event `SetUp`
  (bind _returnvalue (`GameplayStatics.GetPlayerCharacter` 0))
  (bind _returnvalue_2 (`GameplayStatics.GetPlayerController` 0))
  (`self.SetActorHiddenInGame` _returnvalue true)
  (`self.SetActorEnableCollision` _returnvalue false)
  (bind _aspc_bubble_bandit (cast `/Game/Dynamic/Blueprints/Interfaces/PC_BubbleBandit` _returnvalue_2))
  (`self.DisableInput` _aspc_bubble_bandit _aspc_bubble_bandit)
  (`self.DisableInput` _returnvalue _returnvalue_2)
  (`CharacterMovementComponent.DisableMovement` (`Character.CharacterMovement` _returnvalue))
  (bind _returnvalue_3 (`GameplayStatics.GetActorOfClass` "/Game/Dynamic/Blueprints/Characters/BubbleChar/BP_BubbleChar.BP_BubbleChar_C"))
  (`/Engine/EditorBlueprintResources/StandardMacros.IsValid` _returnvalue_3
    (:`Is Valid`
      (`/Game/Dynamic/Blueprints/Actor_Components/AC_BubbleControls.Pop` (`/Game/Dynamic/Blueprints/Characters/BubbleChar/BP_BubbleChar.AC_BubbleControls` _returnvalue_3) _returnvalue_3))))

(event `FlameDeathAnim`
  (params (EdgeColour :type "LinearColor Structure") (ColourBoost :type "Float (single-precision)") (Texture :type "Texture Object Reference"))
  (bind _skeletalmesh (`self.SkeletalMesh`))
  ;[1 1 1] Death Animation when touching fire
  (set `self.EdgeColour` EdgeColour)
  (set `self.ColourBoost` ColourBoost)
  (set `self.Texture` Texture)
  (bind _returnvalue (`KismetMaterialLibrary.CreateDynamicMaterialInstance` "/Game/Static/Materials/M_Dissolve_FlamePipe.M_Dissolve_FlamePipe"))
  (`PrimitiveComponent.SetMaterial` (`self.SkeletalMesh`) 0 _returnvalue)
  (`MeshComponent.SetVectorParameterValueOnMaterials` (`self.SkeletalMesh`) "EdgeColour" (* (`KismetMathLibrary.Conv_LinearColorToVector` (`self.EdgeColour`)) (`self.ColourBoost`)))
  (`NiagaraComponent.SetVariableLinearColor` (`self.SK_Niagara`) "EdgeColour" (`self.EdgeColour`))
  (`NiagaraFunctionLibrary.SetTextureObject` null "DissolveTexture" (`self.Texture`))
  (`PrimitiveComponent.SetCollisionProfileName` _skeletalmesh "Ragdoll" true)
  (`PrimitiveComponent.SetSimulatePhysics` _skeletalmesh true)
  (`ActorComponent.Activate` (`self.SK_Niagara`) false)
  (`PrimitiveComponent.AddImpulse` _skeletalmesh (`self.PlayerVelocity`) "None" false)
  (bind (_direction _newtrack_0) (`Timeline|Timeline` :!via `PlayFromStart`)
    (:`Update`
      (`MaterialInstanceDynamic.SetScalarParameterValue` _returnvalue "Alpha" _newtrack_0)
      (`NiagaraComponent.SetVariableFloat` (`self.SK_Niagara`) "Alpha" _newtrack_0))
    (:`Finished`
      (`PlayerCameraManager.StartCameraFade` :`self` (`GameplayStatics.GetPlayerCameraManager` 0) :`ToAlpha` 1.0 :`Duration` 1.0 :`bHoldWhenFinished` true)
      (`KismetSystemLibrary.Delay` 2.0)
      (message `/Game/Dynamic/SaveSystem/BPI_SaveGame.LoadGameData` (`GameplayStatics.GetPlayerCharacter` 0) false)
      (bind _returnvalue_2 (`GameplayStatics.GetCurrentLevelName` true))
      (`GameplayStatics.OpenLevel` (`KismetStringLibrary.Conv_StringToName` _returnvalue_2)))))

(event `CrushDeathAnim`
  (bind _skeletalmesh (`self.SkeletalMesh`))
  ;[1 1 1] Death Animation when being crushed
  (`PrimitiveComponent.SetCollisionProfileName` _skeletalmesh "Ragdoll" true)
  (`PrimitiveComponent.SetSimulatePhysics` _skeletalmesh true)
  (`KismetSystemLibrary.Delay` 2.0)
  (`PlayerCameraManager.StartCameraFade` :`self` (`GameplayStatics.GetPlayerCameraManager` 0) :`ToAlpha` 1.0 :`Duration` 1.0 :`bHoldWhenFinished` true)
  (`KismetSystemLibrary.Delay` 2.0)
  (message `/Game/Dynamic/SaveSystem/BPI_SaveGame.LoadGameData` (`GameplayStatics.GetPlayerCharacter` 0) false)
  (bind _returnvalue (`GameplayStatics.GetCurrentLevelName` true))
  (`GameplayStatics.OpenLevel` (`KismetStringLibrary.Conv_StringToName` _returnvalue)))

(event `HeatRoomDeathAnim`
  (bind _skeletalmesh (`self.SkeletalMesh`))
  ;[1 1 1] Death Animation when heating up
  (`PrimitiveComponent.SetCollisionProfileName` _skeletalmesh "Ragdoll" true)
  (`PrimitiveComponent.SetSimulatePhysics` _skeletalmesh true)
  (`PrimitiveComponent.SetMaterial` (`self.SkeletalMesh`) 0 "/Game/Static/Materials/M_PlayerMaxHeatRoom.M_PlayerMaxHeatRoom")
  (`KismetSystemLibrary.Delay` 2.0)
  (`PlayerCameraManager.StartCameraFade` :`self` (`GameplayStatics.GetPlayerCameraManager` 0) :`ToAlpha` 1.0 :`Duration` 1.0 :`bHoldWhenFinished` true)
  (`KismetSystemLibrary.Delay` 2.0)
  (message `/Game/Dynamic/SaveSystem/BPI_SaveGame.LoadGameData` (`GameplayStatics.GetPlayerCharacter` 0) false)
  (bind _returnvalue (`GameplayStatics.GetCurrentLevelName` true))
  (`GameplayStatics.OpenLevel` (`KismetStringLibrary.Conv_StringToName` _returnvalue)))

(fn `UserConstructionScript`)