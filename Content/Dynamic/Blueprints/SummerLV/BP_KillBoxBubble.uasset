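; BP_KillBoxBubble is a kill volume that fails the player's BP_BubbleChar when its capsule enters the Killbox.
; On that overlap, PlayerLoseInput disables controller and character input and pops the bubble through ACBubbleControls.
; The camera then fades to black, and after a delay it sends LoadGameDataMessage to the player character and reopens the current level.
; Any other overlap just prints the actor's name.
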(event `self.Killbox.OnComponentBeginOverlap`
  (params (OverlappedComponent :type "PrimitiveComponent Object Reference") (OtherActor :type "Actor Object Reference") (OtherComp :type "PrimitiveComponent Object Reference") (OtherBodyIndex :type Integer) (bFromSweep :type Boolean) (SweepResult :type "HitResult Structure (by ref)"))
  (bind _returnvalue (`GameplayStatics.GetActorOfClass` "/Game/Dynamic/Blueprints/Characters/BubbleChar/BP_BubbleChar.BP_BubbleChar_C"))
  (if (and (== OtherActor _returnvalue) (`GameplayStatics.ObjectIsA` OtherComp "/Script/Engine.CapsuleComponent"))
    (`self.PlayerLoseInput`)
    (`PlayerCameraManager.StartCameraFade` :`self` (`GameplayStatics.GetPlayerCameraManager` 0) :`ToAlpha` 1.0 :`Duration` 1.0 :`bHoldWhenFinished` true)
    (`KismetSystemLibrary.Delay` 3.0)
    (message `/Game/Dynamic/SaveSystem/BPI_SaveGame.LoadGameData` (`GameplayStatics.GetPlayerCharacter` 0) false)
    (bind _returnvalue_2 (`GameplayStatics.GetCurrentLevelName` true))
    (`GameplayStatics.OpenLevel` (`KismetStringLibrary.Conv_StringToName` _returnvalue_2))
    (else
      (`KismetSystemLibrary.PrintString` (`KismetSystemLibrary.GetDisplayName` OtherActor)))))

(fn `PlayerLoseInput`
  (bind _returnvalue (`GameplayStatics.GetPlayerController` 0))
  (bind _aspc_bubble_bandit (cast `/Game/Dynamic/Blueprints/Interfaces/PC_BubbleBandit` _returnvalue))
  (`self.DisableInput` _aspc_bubble_bandit _aspc_bubble_bandit)
  (`self.DisableInput` (`GameplayStatics.GetPlayerCharacter` 0) _returnvalue)
  (bind _returnvalue_2 (`GameplayStatics.GetActorOfClass` "/Game/Dynamic/Blueprints/Characters/BubbleChar/BP_BubbleChar.BP_BubbleChar_C"))
  (`/Engine/EditorBlueprintResources/StandardMacros.IsValid` _returnvalue_2
    (:`Is Valid`
      (`/Game/Dynamic/Blueprints/Actor_Components/AC_BubbleControls.Pop` (`/Game/Dynamic/Blueprints/Characters/BubbleChar/BP_BubbleChar.AC_BubbleControls` _returnvalue_2) _returnvalue_2))))

(fn `UserConstructionScript`)