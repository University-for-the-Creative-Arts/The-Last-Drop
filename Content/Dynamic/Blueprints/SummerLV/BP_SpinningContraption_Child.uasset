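; A child variant of the spinning contraption in the SummerLV content that fits it with two flamethrowers.
; On BeginPlay it runs the parent logic, then calls SetupFlamethrowers for two spawn point and cylinder pairs, taking rotation from the cylinders.
; It adds each result to the Flames array, then calls ActivateFlames.
; The construction script only calls the parent.
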(event `self.ReceiveBeginPlay`
  (`parent.ReceiveBeginPlay`)
  (`|ExecutionSequence`
    (:`then_0`
      (bind _returnactor (`self.SetupFlamethrowers` (`self.SpawnPoint3`) (`self.Cylinder5`)))
      (`KismetArrayLibrary.Array_Add` (`self.Flames`) _returnactor))
    (:`then_1`
      (bind _returnactor_2 (`self.SetupFlamethrowers` (`self.SpawnPoint2`) (`self.Cylinder4_0`)))
      (`KismetArrayLibrary.Array_Add` (`self.Flames`) _returnactor_2))
    (:`then_2`
      (`self.ActivateFlames`))))

(fn `UserConstructionScript`
  (`parent.UserConstructionScript`))