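; BP_MoltenMetal is a molten metal hazard volume that triggers a burning death effect when the player touches it.
; The construction script scales its Cube from Width, Depth and Height variables to size the hazard.
; When the player character's capsule overlaps the Cube, it spawns a BP_DeadPlayer at the player's transform.
; After a brief delay, it plays that actor's FlameDeathAnim with a bright orange edge and noise texture.
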(event `self.Cube.OnComponentBeginOverlap`
  (params (OverlappedComponent :type "PrimitiveComponent Object Reference") (OtherActor :type "Actor Object Reference") (OtherComp :type "PrimitiveComponent Object Reference") (OtherBodyIndex :type Integer) (bFromSweep :type Boolean) (SweepResult :type "HitResult Structure (by ref)"))
  (bind _returnvalue (`GameplayStatics.GetPlayerCharacter` 0))
  (if (and (== OtherActor _returnvalue) (`GameplayStatics.ObjectIsA` OtherComp "/Script/Engine.CapsuleComponent"))
    (bind _returnvalue_2 (`|SpawnActorFromClass` "/Game/Dynamic/Blueprints/SummerLV/BP_DeadPlayer.BP_DeadPlayer_C" (`KismetMathLibrary.MakeTransform` (`self.K2_GetActorLocation` _returnvalue) (`self.K2_GetActorRotation` _returnvalue)) "Undefined" "MultiplyWithRoot" _returnvalue null))
    (`KismetSystemLibrary.Delay` 0.01)
    (`/Game/Dynamic/Blueprints/SummerLV/BP_DeadPlayer.FlameDeathAnim` _returnvalue_2 (struct :`R` 20.0 :`G` 3.833086 :`A` 1.0) 11.0 "/Engine/Functions/Engine_MaterialFunctions02/ExampleContent/Textures/OffsetNoiseDistanceFields_ForNormals.OffsetNoiseDistanceFields_ForNormals")))

(fn `UserConstructionScript`
  (`SceneComponent.SetRelativeScale3D` (`self.Cube`) (`KismetMathLibrary.MakeVector` (`self.Width`) (`self.Depth`) (`self.Height`))))