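; BP_Arrow is a guide arrow that follows the player and points toward the active BP_HeatPlate.
; NewActive, run at BeginPlay, searches all heat plates and stores the first active one as the target.
; Each tick snaps the actor to the player's location and rotates Arm to face the target.
; It also prints the player's distance to the plate and hides Arrow when that plate is near.
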(event `self.ReceiveBeginPlay`
  (`self.NewActive`))

(event `NewActive`
  (bind _outactors (`GameplayStatics.GetAllActorsOfClass` "/Game/Dynamic/Blueprints/SummerLV/BP_HeatPlate.BP_HeatPlate_C"))
  (for _array_element _outactors
    (if (`/Game/Dynamic/Blueprints/SummerLV/BP_HeatPlate.Active?` _array_element)
      (set `self.CurrentActivePlate` _array_element)
      (break))))

(event `self.ReceiveTick`
  (params (DeltaSeconds :type "Float (single-precision)"))
  (`self.SetPosition`)
  (`self.SetRotation`)
  (`self.CheckDistance`))

(fn `CheckDistance`
  (bind _arrow (`self.Arrow`))
  (bind _returnvalue (`self.GetDistanceTo` (`GameplayStatics.GetPlayerCharacter` 0) (`self.CurrentActivePlate`)))
  (`KismetSystemLibrary.PrintText` (`KismetTextLibrary.Conv_DoubleToText` _returnvalue "HalfToEven") true true (struct :`R` 0.903279 :`G` 1.0 :`B` 0.733361 :`A` 1.0) 1.0 "958563859678463785967")
  (if (<= _returnvalue 500.0)
    (`SceneComponent.SetHiddenInGame` _arrow true false)
    (else
      (`SceneComponent.SetHiddenInGame` _arrow false false))))

(fn `SetPosition`
  (bind (_returnvalue_x _returnvalue_y _returnvalue_z) (`KismetMathLibrary.BreakVector` (`self.K2_GetActorLocation` (`GameplayStatics.GetPlayerCharacter` 0))))
  (`self.K2_SetActorLocation` (`KismetMathLibrary.MakeVector` _returnvalue_x _returnvalue_y _returnvalue_z)))

(fn `SetRotation`
  (`SceneComponent.K2_SetWorldRotation` (`self.Arm`) (`KismetMathLibrary.FindLookAtRotation` (`self.K2_GetActorLocation`) (`self.K2_GetActorLocation` (`self.CurrentActivePlate`))) false false))

(fn `UserConstructionScript`)