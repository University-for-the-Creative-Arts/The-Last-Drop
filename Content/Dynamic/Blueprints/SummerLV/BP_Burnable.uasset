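; BP_Burnable is a destructible object, apparently a wall, that burns away when the player's bubble touches it.
; At BeginPlay it calls UpdateDataStatic and caches the player's BP_BodyChar.
; On box overlap with that player's bubble character, it removes the box, runs StaticTimeline, disables collision and destroys itself after a short delay.
; The overlap does not check bubble state, despite comments describing a burning bubble.
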(event `self.ReceiveBeginPlay`
  (`self.UpdateDataStatic`)
  (bind _asbp_body_char (cast `/Game/Dynamic/Blueprints/Characters/BodyChar/BP_BodyChar` (`GameplayStatics.GetPlayerCharacter` 0)))
  (set `self.Player` _asbp_body_char))

(event `self.Box.OnComponentBeginOverlap`
  (params (OverlappedComponent :type "PrimitiveComponent Object Reference") (OtherActor :type "Actor Object Reference") (OtherComp :type "PrimitiveComponent Object Reference") (OtherBodyIndex :type Integer) (bFromSweep :type Boolean) (SweepResult :type "HitResult Structure (by ref)"))
  (if (== OtherActor (`/Game/Dynamic/Blueprints/Interfaces/PC_BubbleBandit.BP Bubble Char` (`/Game/Dynamic/Blueprints/Characters/BodyChar/BP_BodyChar.PC_BubbleChar` (`self.Player`))))
    ;[1 1 1] Once the burning bubble touches the object, burns it and destroys it.
    (`ActorComponent.K2_DestroyComponent` (`self.Box`))
    (`self.StaticTimeline`)
    (`self.SetActorEnableCollision` false)
    (`KismetSystemLibrary.Delay` 2.0)
    (`KismetSystemLibrary.PrintString` "DestroyedWall" true true (struct :`R` 1.0 :`G` 0.298067 :`B` 0.288119 :`A` 1.0))
    (`self.K2_DestroyActor`)))

(fn `UserConstructionScript`
  (`parent.UserConstructionScript`))