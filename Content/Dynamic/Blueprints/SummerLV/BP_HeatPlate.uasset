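; BP_HeatPlate is a pressure plate for a heat area (Room) that responds only to the player character.
; Activate and Deactivate toggle its Active flag, plate material and arrow visibility.
; Stepping on an active plate enables the Room's tick, starts its fans and hides the arrow.
; Stepping off deactivates the plate, stops the tick and fans, and passes PlateNum to Room.Reactivate.
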(event `Deactivate`
  ;[1 1 1] Quickly activates and deactivates this pressure plate
  (set `self.Active?` false)
  (`PrimitiveComponent.SetMaterial` (`self.Plate`) 0 "/Engine/EngineMaterials/WorldGridMaterial_Low.WorldGridMaterial_Low")
  (`SceneComponent.SetVisibility` (`self.Arrow`) false false))

(event `Activate`
  ;[1 1 1] Quickly activates and deactivates this pressure plate
  (set `self.Active?` true)
  (`PrimitiveComponent.SetMaterial` (`self.Plate`) 0 "/Game/Static/Materials/M_Plate_On.M_Plate_On")
  (`SceneComponent.SetVisibility` (`self.Arrow`) true false))

(event `self.Plate.OnComponentBeginOverlap`
  (params (OverlappedComponent :type "PrimitiveComponent Object Reference") (OtherActor :type "Actor Object Reference") (OtherComp :type "PrimitiveComponent Object Reference") (OtherBodyIndex :type Integer) (bFromSweep :type Boolean) (SweepResult :type "HitResult Structure (by ref)"))
  ;[1 0.5712 0.548] Checks if the player is stood on the plate. If so, the tick of the assigned heat area is activated
  (if (`self.Active?`)
    (if (== OtherActor (`GameplayStatics.GetPlayerCharacter` 0))
      (`self.SetActorTickEnabled` (`self.Room`) true)
      (`SceneComponent.SetVisibility` (`self.Arrow`) false false)
      (`PrimitiveComponent.SetMaterial` (`self.Plate`) 0 "/Game/Static/Materials/M_Plate_Off.M_Plate_Off")
      (for _array_element (`/Game/Dynamic/Blueprints/SummerLV/BP_HeatArea.Fans` (`self.Room`))
        (`/Game/Dynamic/Blueprints/SummerLV/BP_HeatAreaFan.Start` _array_element)))))

(event `self.Plate.OnComponentEndOverlap`
  (params (OverlappedComponent :type "PrimitiveComponent Object Reference") (OtherActor :type "Actor Object Reference") (OtherComp :type "PrimitiveComponent Object Reference") (OtherBodyIndex :type Integer))
  (bind _room (`self.Room`))
  ;[0.6433 0.7114 1] Checks once the player has left the plate, if it's the current active one, the plate is disabled
  (if (== OtherActor (`GameplayStatics.GetPlayerCharacter` 0))
    (if (`self.Active?`)
      (set `self.Active?` false)
      (`self.Deactivate`)
      (`self.SetActorTickEnabled` _room false)
      (`/Game/Dynamic/Blueprints/SummerLV/BP_HeatArea.Reactivate` _room (`self.PlateNum`))
      (for _array_element (`/Game/Dynamic/Blueprints/SummerLV/BP_HeatArea.Fans` (`self.Room`))
        (`/Game/Dynamic/Blueprints/SummerLV/BP_HeatAreaFan.Stop` _array_element)))))

(fn `UserConstructionScript`)