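; BP_HitButtonPlat is a hit-activated button that moves a bridge into position.
; When a BP_BodyChar with a valid Mesh hits the Button, a Sequence fires two DoOnce-gated moves, so each runs only once.
; The Button shifts 20 units along relative Z, while the Bridge eases over four seconds to the relative location of the Billboard component, which serves as the destination marker.
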(event `self.Button.OnComponentHit`
  (params (HitComponent :type "PrimitiveComponent Object Reference") (OtherActor :type "Actor Object Reference") (OtherComp :type "PrimitiveComponent Object Reference") (NormalImpulse :type "Vector Structure") (Hit :type "HitResult Structure (by ref)"))
  (bind _button (`self.Button`))
  (bind (_relativelocation_x _relativelocation_y _relativelocation_z) (`KismetMathLibrary.BreakVector` (`SceneComponent.RelativeLocation` _button)))
  (bind _asbp_body_char (cast `/Game/Dynamic/Blueprints/Characters/BodyChar/BP_BodyChar` OtherActor))
  (`/Engine/EditorBlueprintResources/StandardMacros.IsValid` (`Character.Mesh` _asbp_body_char)
    (:`Is Valid`
      (`|ExecutionSequence`
        (:`then_0`
          (`/Engine/EditorBlueprintResources/StandardMacros.DoOnce` false
            (:`Completed`
              (`KismetSystemLibrary.MoveComponentTo` _button (`KismetMathLibrary.MakeVector` _relativelocation_x _relativelocation_y (+ _relativelocation_z 20.0)) (struct) true true))))
        (:`then_1`
          (`/Engine/EditorBlueprintResources/StandardMacros.DoOnce` false
            (:`Completed`
              (`KismetSystemLibrary.MoveComponentTo` (`self.Bridge`) (`SceneComponent.RelativeLocation` (`self.Billboard`)) (struct) true true 4.0))))))))

(fn `UserConstructionScript`)