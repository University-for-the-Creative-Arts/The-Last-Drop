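; BP_HitMovingPlatform is a platform that moves when a BP_BodyChar enters or leaves its trigger Box.
; Begin overlap eases the Platform component to the Billboard's relative location, and end overlap eases it to Billboard1's, keeping its current rotation.
; Both moves use MoveComponentTo over a fixed duration, with the two billboards serving as placeable endpoint markers.
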(event `self.Box.OnComponentBeginOverlap`
  (params (OverlappedComponent :type "PrimitiveComponent Object Reference") (OtherActor :type "Actor Object Reference") (OtherComp :type "PrimitiveComponent Object Reference") (OtherBodyIndex :type Integer) (bFromSweep :type Boolean) (SweepResult :type "HitResult Structure (by ref)"))
  (cast `/Game/Dynamic/Blueprints/Characters/BodyChar/BP_BodyChar` OtherActor)
  (`KismetSystemLibrary.MoveComponentTo` (`self.Platform`) (`SceneComponent.RelativeLocation` (`self.Billboard`)) (`SceneComponent.RelativeRotation` (`self.Platform`)) true true 4.0))

(event `self.Box.OnComponentEndOverlap`
  (params (OverlappedComponent :type "PrimitiveComponent Object Reference") (OtherActor :type "Actor Object Reference") (OtherComp :type "PrimitiveComponent Object Reference") (OtherBodyIndex :type Integer))
  (cast `/Game/Dynamic/Blueprints/Characters/BodyChar/BP_BodyChar` OtherActor)
  (`KismetSystemLibrary.MoveComponentTo` (`self.Platform`) (`SceneComponent.RelativeLocation` (`self.Billboard1`)) (`SceneComponent.RelativeRotation` (`self.Platform`)) true true 4.0))

(fn `UserConstructionScript`)