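; Button-and-platform sequence puzzle where BP_BodyChar overlaps four trigger boxes to move four platforms in order.
; Each overlap bobs its button behind a resetting DoOnce and eases its platform to an end marker with MoveComponentTo.
; Pressed flags chain the order: platforms 2 to 4 move to hard-coded positions after a delay if the preceding flag is unset.
; The Plat1 hit event has no effect.
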(event `self.Box1.OnComponentBeginOverlap`
  (params (OverlappedComponent :type "PrimitiveComponent Object Reference") (OtherActor :type "Actor Object Reference") (OtherComp :type "PrimitiveComponent Object Reference") (OtherBodyIndex :type Integer) (bFromSweep :type Boolean) (SweepResult :type "HitResult Structure (by ref)"))
  (bind _plat1end (`self.Plat1End`))
  (bind _button1 (`self.Button1`))
  (bind _button1_2 (`self.Button1`))
  (bind (_relativelocation_x _relativelocation_y _relativelocation_z) (`KismetMathLibrary.BreakVector` (`SceneComponent.RelativeLocation` _button1_2)))
  (bind (_relativelocation_x_2 _relativelocation_y_2 _relativelocation_z_2) (`KismetMathLibrary.BreakVector` (`SceneComponent.RelativeLocation` _button1)))
  (bind _asbp_body_char (cast `/Game/Dynamic/Blueprints/Characters/BodyChar/BP_BodyChar` OtherActor))
  (`/Engine/EditorBlueprintResources/StandardMacros.IsValid` (`Character.Mesh` _asbp_body_char)
    (:`Is Valid`
      (`|ExecutionSequence`
        (:`then_0`
          (`KismetSystemLibrary.Delay` 0.1)
          (`/Engine/EditorBlueprintResources/StandardMacros.DoOnce` false :!label _label
            (:`Completed`
              (`KismetSystemLibrary.MoveComponentTo` _button1_2 (`KismetMathLibrary.MakeVector` _relativelocation_x _relativelocation_y (+ _relativelocation_z 20.0)) (struct) true true)
              (`KismetSystemLibrary.Delay` 0.2)
              (`KismetSystemLibrary.MoveComponentTo` _button1 (`KismetMathLibrary.MakeVector` _relativelocation_x_2 _relativelocation_y_2 (+ _relativelocation_z_2 -20.0)) (struct) true true)
              (goto _label))))
        (:`then_1`
          (`KismetSystemLibrary.MoveComponentTo` (`self.Plat1`) (`SceneComponent.RelativeLocation` _plat1end) (`SceneComponent.RelativeRotation` _plat1end) true true 2.0)
          (set `self.1pressed?` true))))))

(event `self.Plat1.OnComponentHit`
  (params (HitComponent :type "PrimitiveComponent Object Reference") (OtherActor :type "Actor Object Reference") (OtherComp :type "PrimitiveComponent Object Reference") (NormalImpulse :type "Vector Structure") (Hit :type "HitResult Structure (by ref)"))
  (bind _asbp_body_char (cast `/Game/Dynamic/Blueprints/Characters/BodyChar/BP_BodyChar` OtherActor))
  (`/Engine/EditorBlueprintResources/StandardMacros.IsValid` (`Character.Mesh` _asbp_body_char)))

(event `self.Box2.OnComponentBeginOverlap`
  (params (OverlappedComponent :type "PrimitiveComponent Object Reference") (OtherActor :type "Actor Object Reference") (OtherComp :type "PrimitiveComponent Object Reference") (OtherBodyIndex :type Integer) (bFromSweep :type Boolean) (SweepResult :type "HitResult Structure (by ref)"))
  (bind _plat2end (`self.Plat2End`))
  (bind _button2 (`self.Button2`))
  (bind _button2_2 (`self.Button2`))
  (bind (_relativelocation_x _relativelocation_y _relativelocation_z) (`KismetMathLibrary.BreakVector` (`SceneComponent.RelativeLocation` _button2)))
  (bind (_relativelocation_x_2 _relativelocation_y_2 _relativelocation_z_2) (`KismetMathLibrary.BreakVector` (`SceneComponent.RelativeLocation` _button2_2)))
  (bind _relativerotation (`SceneComponent.RelativeRotation` _plat2end))
  (bind _asbp_body_char (cast `/Game/Dynamic/Blueprints/Characters/BodyChar/BP_BodyChar` OtherActor))
  (`|ExecutionSequence`
    (:`then_0`
      (`KismetSystemLibrary.Delay` 0.1)
      (`/Engine/EditorBlueprintResources/StandardMacros.DoOnce` false :!label _label_2
        (:`Completed`
          (`KismetSystemLibrary.MoveComponentTo` _button2 (`KismetMathLibrary.MakeVector` _relativelocation_x _relativelocation_y (+ _relativelocation_z 20.0)) (struct) true true)
          (`KismetSystemLibrary.Delay` 0.2)
          (`KismetSystemLibrary.MoveComponentTo` _button2_2 (`KismetMathLibrary.MakeVector` _relativelocation_x_2 _relativelocation_y_2 (+ _relativelocation_z_2 -20.0)) (struct) true true)
          (goto _label_2 :!via `Reset`))))
    (:`then_1`
      (`/Engine/EditorBlueprintResources/StandardMacros.IsValid` (`Character.Mesh` _asbp_body_char)
        (:`Is Valid`
          (`KismetSystemLibrary.MoveComponentTo` (`self.Plat2`) (`SceneComponent.RelativeLocation` _plat2end) _relativerotation true true 2.0)
          (if (`self.1pressed?`)
            (set `self.2pressed?` true)
            (else
              (`KismetSystemLibrary.Delay` 1.5)
              (`KismetSystemLibrary.MoveComponentTo` (`self.Plat2`) (-10.0 980.0 -600.0) _relativerotation true true 2.0))))))))

(event `self.Box3.OnComponentBeginOverlap`
  (params (OverlappedComponent :type "PrimitiveComponent Object Reference") (OtherActor :type "Actor Object Reference") (OtherComp :type "PrimitiveComponent Object Reference") (OtherBodyIndex :type Integer) (bFromSweep :type Boolean) (SweepResult :type "HitResult Structure (by ref)"))
  (bind _plat3end (`self.Plat3End`))
  (bind _button3 (`self.Button3`))
  (bind _button3_2 (`self.Button3`))
  (bind (_relativelocation_x _relativelocation_y _relativelocation_z) (`KismetMathLibrary.BreakVector` (`SceneComponent.RelativeLocation` _button3)))
  (bind (_relativelocation_x_2 _relativelocation_y_2 _relativelocation_z_2) (`KismetMathLibrary.BreakVector` (`SceneComponent.RelativeLocation` _button3_2)))
  (bind _relativerotation (`SceneComponent.RelativeRotation` _plat3end))
  (bind _asbp_body_char (cast `/Game/Dynamic/Blueprints/Characters/BodyChar/BP_BodyChar` OtherActor))
  (`|ExecutionSequence`
    (:`then_0`
      (`KismetSystemLibrary.Delay` 0.1)
      (`/Engine/EditorBlueprintResources/StandardMacros.DoOnce` false :!label _label_3
        (:`Completed`
          (`KismetSystemLibrary.MoveComponentTo` _button3 (`KismetMathLibrary.MakeVector` _relativelocation_x _relativelocation_y (+ _relativelocation_z 20.0)) (struct) true true)
          (`KismetSystemLibrary.Delay` 0.2)
          (`KismetSystemLibrary.MoveComponentTo` _button3_2 (`KismetMathLibrary.MakeVector` _relativelocation_x_2 _relativelocation_y_2 (+ _relativelocation_z_2 -20.0)) (struct) true true)
          (goto _label_3 :!via `Reset`))))
    (:`then_1`
      (`/Engine/EditorBlueprintResources/StandardMacros.IsValid` (`Character.Mesh` _asbp_body_char)
        (:`Is Valid`
          (`KismetSystemLibrary.MoveComponentTo` (`self.Plat3`) (`SceneComponent.RelativeLocation` _plat3end) _relativerotation true true 2.0)
          (if (`self.2pressed?`)
            (set `self.3pressed?` true)
            (else
              (`KismetSystemLibrary.Delay` 1.5)
              (`KismetSystemLibrary.MoveComponentTo` (`self.Plat3`) (-10.0 1530.0 -600.0) _relativerotation true true 2.0))))))))

(event `self.Box4.OnComponentBeginOverlap`
  (params (OverlappedComponent :type "PrimitiveComponent Object Reference") (OtherActor :type "Actor Object Reference") (OtherComp :type "PrimitiveComponent Object Reference") (OtherBodyIndex :type Integer) (bFromSweep :type Boolean) (SweepResult :type "HitResult Structure (by ref)"))
  (bind _plat4end (`self.Plat4End`))
  (bind _button4 (`self.Button4`))
  (bind _button4_2 (`self.Button4`))
  (bind (_relativelocation_x _relativelocation_y _relativelocation_z) (`KismetMathLibrary.BreakVector` (`SceneComponent.RelativeLocation` _button4_2)))
  (bind (_relativelocation_x_2 _relativelocation_y_2 _relativelocation_z_2) (`KismetMathLibrary.BreakVector` (`SceneComponent.RelativeLocation` _button4)))
  (bind _relativerotation (`SceneComponent.RelativeRotation` _plat4end))
  (bind _asbp_body_char (cast `/Game/Dynamic/Blueprints/Characters/BodyChar/BP_BodyChar` OtherActor))
  (`|ExecutionSequence`
    (:`then_0`
      (`KismetSystemLibrary.Delay` 0.1)
      (`/Engine/EditorBlueprintResources/StandardMacros.DoOnce` false :!label _label_4
        (:`Completed`
          (`KismetSystemLibrary.MoveComponentTo` _button4_2 (`KismetMathLibrary.MakeVector` _relativelocation_x _relativelocation_y (+ _relativelocation_z 20.0)) (struct) true true)
          (`KismetSystemLibrary.Delay` 0.2)
          (`KismetSystemLibrary.MoveComponentTo` _button4 (`KismetMathLibrary.MakeVector` _relativelocation_x_2 _relativelocation_y_2 (+ _relativelocation_z_2 -20.0)) (struct) true true)
          (goto _label_4 :!via `Reset`))))
    (:`then_1`
      (`/Engine/EditorBlueprintResources/StandardMacros.IsValid` (`Character.Mesh` _asbp_body_char)
        (:`Is Valid`
          (`KismetSystemLibrary.MoveComponentTo` (`self.Plat4`) (`SceneComponent.RelativeLocation` _plat4end) _relativerotation true true 2.0)
          (if (not (`self.3pressed?`))
            (`KismetSystemLibrary.Delay` 1.5)
            (`KismetSystemLibrary.MoveComponentTo` (`self.Plat4`) (-10.0 2080.0 -600.0) _relativerotation true true 2.0)))))))

(fn `UserConstructionScript`)