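; Spring level Blueprint of four jumping platforms that shuttle endlessly between their own start and end marker components.
; BeginPlay uses a Sequence to launch four parallel latent loops, each easing a platform via MoveComponentTo over a shared Overtime duration while keeping its rotation.
; Staggered initial delays and differing pauses at each start point offset the platforms' timing, with no pause at the end points.
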(event `self.ReceiveBeginPlay`
  (bind _platform2 (`self.Platform2`))
  (bind _platform1 (`self.Platform1`))
  (bind _platform3 (`self.Platform3`))
  (bind _overtime (`self.Overtime`))
  (bind _overtime_2 (`self.Overtime`))
  (bind _overtime_3 (`self.Overtime`))
  (bind _overtime_4 (`self.Overtime`))
  (bind _platform4 (`self.Platform4`))
  (bind _relativerotation (`SceneComponent.RelativeRotation` _platform1))
  (bind _relativerotation_2 (`SceneComponent.RelativeRotation` _platform2))
  (bind _relativerotation_3 (`SceneComponent.RelativeRotation` _platform3))
  (bind _relativerotation_4 (`SceneComponent.RelativeRotation` _platform4))
  (`|ExecutionSequence`
    (:`then_0`
      (`KismetSystemLibrary.MoveComponentTo` _platform1 (`SceneComponent.RelativeLocation` (`self.Start`)) _relativerotation true true _overtime_2 :!label _label)
      (`KismetSystemLibrary.Delay` 1.0)
      (`KismetSystemLibrary.MoveComponentTo` (`self.Platform1`) (`SceneComponent.RelativeLocation` (`self.End`)) _relativerotation true true _overtime_2)
      (goto _label))
    (:`then_1`
      (`KismetSystemLibrary.Delay` 1.0)
      (`KismetSystemLibrary.MoveComponentTo` _platform2 (`SceneComponent.RelativeLocation` (`self.Start2`)) _relativerotation_2 true true _overtime_3 :!label _label_2)
      (`KismetSystemLibrary.Delay` 1.0)
      (`KismetSystemLibrary.MoveComponentTo` (`self.Platform2`) (`SceneComponent.RelativeLocation` (`self.End2`)) _relativerotation_2 true true _overtime_3)
      (goto _label_2))
    (:`then_2`
      (`KismetSystemLibrary.Delay` 1.0)
      (`KismetSystemLibrary.MoveComponentTo` _platform3 (`SceneComponent.RelativeLocation` (`self.Start3`)) _relativerotation_3 true true _overtime_4 :!label _label_3)
      (`KismetSystemLibrary.Delay` 1.7)
      (`KismetSystemLibrary.MoveComponentTo` (`self.Platform3`) (`SceneComponent.RelativeLocation` (`self.End3`)) _relativerotation_3 true true _overtime_4)
      (goto _label_3))
    (:`then_3`
      (`KismetSystemLibrary.Delay` 1.5)
      (`KismetSystemLibrary.MoveComponentTo` _platform4 (`SceneComponent.RelativeLocation` (`self.Start4`)) _relativerotation_4 true true _overtime :!label _label_4)
      (`KismetSystemLibrary.Delay` 2.3)
      (`KismetSystemLibrary.MoveComponentTo` (`self.Platform4`) (`SceneComponent.RelativeLocation` (`self.End4`)) _relativerotation_4 true true _overtime)
      (goto _label_4))))

(fn `UserConstructionScript`)