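; ElectricWater is a level actor that turns the player's bubble into an electric bubble when the bubble touches its mesh.
; On BeginPlay it caches the player's BP_BodyChar; on overlap it checks that the other actor is that player's current bubble and not already electric.
; It then destroys the bubble, spawns BP_BubbleElectric at the same transform, and moves the camera behaviour's tracking to the new one.
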(event `self.ReceiveBeginPlay`
  ;[1 1 1] Set player
  (bind _asbp_body_char (cast `/Game/Dynamic/Blueprints/Characters/BodyChar/BP_BodyChar` (`GameplayStatics.GetPlayerCharacter` 0)))
  (set `self.Player` _asbp_body_char))

(event `self.StaticMesh.OnComponentBeginOverlap`
  (params (OverlappedComponent :type "PrimitiveComponent Object Reference") (OtherActor :type "Actor Object Reference") (OtherComp :type "PrimitiveComponent Object Reference") (OtherBodyIndex :type Integer) (bFromSweep :type Boolean) (SweepResult :type "HitResult Structure (by ref)"))
  (bind _player (`self.Player`))
  (bind _ac_cambehaviour (`/Game/Dynamic/Blueprints/Characters/BodyChar/BP_BodyChar.AC_CamBehaviour` _player))
  (bind _bp_bubble_char (`/Game/Dynamic/Blueprints/Interfaces/PC_BubbleBandit.BP Bubble Char` (`/Game/Dynamic/Blueprints/Characters/BodyChar/BP_BodyChar.PC_BubbleChar` _player)))
  ;[1 1 1] Remove currently tracked bubble and destroys it
  (if (and (== OtherActor _bp_bubble_char) (not (`GameplayStatics.ObjectIsA` _bp_bubble_char "/Game/Dynamic/Blueprints/Characters/BubbleChar/BP_BubbleElectric.BP_BubbleElectric_C")))
    (`/Game/Dynamic/Blueprints/Actor_Components/AC_CamBehaviour.RemoveTrackingActor` _ac_cambehaviour OtherActor)
    (set `self.Transform` (`self.GetTransform` _bp_bubble_char))
    (`self.K2_DestroyActor` _bp_bubble_char)
    ;[1 1 1] Spawns a new one to make the current tracking actor
    (bind _returnvalue (`|SpawnActorFromClass` "/Game/Dynamic/Blueprints/Characters/BubbleChar/BP_BubbleElectric.BP_BubbleElectric_C" (`self.Transform`) "AlwaysSpawn" "MultiplyWithRoot" null (`self.Player`) null))
    (`/Game/Dynamic/Blueprints/Actor_Components/AC_CamBehaviour.AddTrackingActor` _ac_cambehaviour _returnvalue)))

(fn `UserConstructionScript`)